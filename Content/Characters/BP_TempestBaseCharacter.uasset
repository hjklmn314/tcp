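; BP_TempestBaseCharacter is a base character Blueprint that routes incoming damage into the Tempest combat and state systems.
; On AnyDamage, unless the controller's state manager reports an active Death state, OnAttackReceived has the combat component's defense property process the attack.
; It then attempts the Death state with a condition check, resolving the state class by gameplay tag.
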(event `self.ReceiveAnyDamage`
  (params (Damage :type "Float (single-precision)") (DamageType :type "DamageType Object Reference") (InstigatedBy :type "Controller Object Reference") (DamageCauser :type "Actor Object Reference"))
  (bind _returnvalue (`self.GetComponentByClass` (`self.GetController`) "/Script/TempestCombatFramework.TempestBaseStateManagerComponent"))
  (bind _returnvalue_2 (`self.GetComponentByClass` (`self.GetController`) "/Script/TempestCombatFramework.TempestBaseStateManagerComponent"))
  (bind _returnvalue_3 (`TempestBaseStateManagerComponent.GetCurrentActiveState` _returnvalue))
  (`/Engine/EditorBlueprintResources/StandardMacros.IsValid` _returnvalue
    (:`Is Valid`
      (`/Engine/EditorBlueprintResources/StandardMacros.IsValid` _returnvalue_3
        (:`Is Valid`
          (if (!= (`TempestBaseStateObject.StateGameplayTag` _returnvalue_3) (struct :`TagName` "State.Death"))
            (`self.On Attack Received`)
            (`/Engine/EditorBlueprintResources/StandardMacros.IsValid` _returnvalue_2
              (:`Is Valid`
                (`TempestBaseStateManagerComponent.TryPerformStateOfClass` _returnvalue_2 (`GameplayStatics.GetObjectClass` (`TempestBaseStateManagerComponent.GetStateOfGameplayTag` _returnvalue_2 (struct :`TagName` "State.Death"))) true)))))))))

(fn `On Attack Received`
  (locals (`Local Combat Component` :type "TempestCombatComponent Object Reference"))
  (bind _ownerdefenseproperty (`TempestCombatComponent.OwnerDefenseProperty` (`local.Local Combat Component`)))
  (bind _output_get (set `local.Local Combat Component` (`self.GetComponentByClass` "/Script/TempestCombatFramework.TempestCombatComponent")))
  (`/Engine/EditorBlueprintResources/StandardMacros.IsValid` _output_get
    (:`Is Valid`
      (`/Engine/EditorBlueprintResources/StandardMacros.IsValid` _ownerdefenseproperty
        (:`Is Valid`
          (`TempestDefensePropertiesObject.ProcessReceivedAttack` _ownerdefenseproperty))))))

(fn `UserConstructionScript`)