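; Master enemy character for the Tempest combat system, configured by an enemy data asset and warning the developer when none is assigned.
; BeginPlay ensures the asset's AI controller class possesses it, then initializes the controller, combat component, attributes, defense property and hit/block statistics.
; Spawner assignment records spawn info and activates the controller's spawn state.
; As a lock-on target, it creates or destroys a screen-space widget, with a timeline for offsetting it.
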(event `self.ReceiveBeginPlay`
  (bind _returnvalue (`self.GetComponentByClass` "/Script/TempestCombatFramework.TempestCombatComponent"))
  (bind _enemy_controller (`/TempestCombatFramework/DataAssets/DA_Enemyinfo.Get Enemy Controller Class` (`self.Enemy Info Ref`)))
  (`parent.ReceiveBeginPlay`)
  (`/Engine/EditorBlueprintResources/StandardMacros.IsValid` (`self.Enemy Info Ref`)
    (:`Is Valid`
      (`/Game/TempestCombatFramework/AI/Enemy/FL_DeveloperWarnings.Warn Developer To Adjust /Create Nav Mesh` self)
      (if (not (== _enemy_controller (`self.AIControllerClass`)))
        (bind _output_get (set `self.AIControllerClass` _enemy_controller))
        (bind _returnvalue_2 (`|SpawnActorFromClass` _output_get (`KismetMathLibrary.MakeTransform` (0.0 0.0 0.0)) "Undefined" "OverrideRootScale" null null))
        (bind _asaicontroller (cast `AIController` _returnvalue_2))
        (`Controller.Possess` _asaicontroller self))
      (bind _astcf_master_enemy_aic_bp (cast `/TempestCombatFramework/Controllers/TCF_MasterEnemy_AIC_BP` (`AIBlueprintHelperLibrary.GetAIController` self)))
      (bind _output_get_2 (set `self.Master Enemy AIC` _astcf_master_enemy_aic_bp))
      (`/TempestCombatFramework/Controllers/TCF_MasterEnemy_AIC_BP.Initialize Enemy Controller` _output_get_2)
      (`/TempestCombatFramework/Components/AI/AICombatComponent.Init AI Combat Component` (`self.BP_TempestEnemyCombatComponent`))
      (`TempestAttributesComponents.AssignAttributes` (`self.BP_TempestAttributesComponents`) (`TempestGeneral_PDA.AttributesToCreate` (`self.Get Enemy Data Asset`)))
      (bind _constructedproperty (`TempestCombatComponent.ConstructDefensePropertyOfClass` _returnvalue "/TempestCombatFramework/DefenseProperties/BP_EnemyDefenseProperty.BP_EnemyDefenseProperty_C"))
      (`TempestCombatComponent.SetDefenseProperty` _returnvalue _constructedproperty)
      (`TempestStatisticsComponent.ConstructStatisticOfClass` (`self.BP_TempestStatisticsComponent`) "/TempestCombatFramework/Statistics/BP_HitCountStatistic.BP_HitCountStatistic_C")
      (`TempestStatisticsComponent.ConstructStatisticOfClass` (`self.BP_TempestStatisticsComponent`) "/TempestCombatFramework/Statistics/BP_BlockCountStatistic.BP_BlockCountStatistic_C"))
    (:`Is Not Valid`
      (`/Game/TempestCombatFramework/AI/Enemy/FL_DeveloperWarnings.Warn Developer Of Unassigned Enemy Data Asset Variable` self))))

(event `/TempestCombatFramework/Interfaces/BPI_EnemySpawner.Assign Enemy Spawner`
  (params (`Enemy Spawner` :type "/TempestCombatFramework/Actors/Spawner/BP_EnemySpawner Object Reference"))
  (setmembers `/TempestCombatFramework/StructuresEnums/S_Enemy_SpawnInfo` :`StructRef` (`self.Enemy Spawn Info`) :`Spawner` `Enemy Spawner` :`Spawn Location` (`self.K2_GetActorLocation`))
  (`/Engine/EditorBlueprintResources/StandardMacros.IsValid` (`.Spawner_29_F09BD5E34E47067EBE18C39743D73637` (break `/TempestCombatFramework/StructuresEnums/S_Enemy_SpawnInfo` (`self.Enemy Spawn Info`)))
    (:`Is Valid`
      (`/Engine/EditorBlueprintResources/StandardMacros.IsValid` (`self.Master Enemy AIC`)
        (:`Is Valid`
          (`/TempestCombatFramework/Controllers/TCF_MasterEnemy_AIC_BP.Activate Spawn State` (`self.Master Enemy AIC`)))))))

(event `/TempestCombatFramework/Interfaces/BPI_TargetingSystem.Toggle Targeting Point`
  (params (Toggle :type Boolean))
  (bind _created_widget_component (`self.Created Widget Component`))
  (bind _created_widget_component_2 (`self.Created Widget Component`))
  (if Toggle
    (`/Engine/EditorBlueprintResources/StandardMacros.IsValid` (`self.Created Widget Component`)
      (:`Is Not Valid`
        (bind _returnvalue (`AddComponent|NODE_AddWidgetComponent-0`))
        (bind _output_get (set `self.Created Widget Component` _returnvalue))
        (`WidgetComponent.SetWidgetSpace` _output_get "Screen")
        (`WidgetComponent.SetDrawSize` (`self.Created Widget Component`) (30.0 30.0))
        (bind _returnvalue_2 (`|CreateWidget` "/Game/TempestCombatFramework/AI/WB_LockOnPoint.WB_LockOnPoint_C"))
        (`WidgetComponent.SetWidget` _created_widget_component _returnvalue_2)
        (`SceneComponent.K2_AttachToComponent` _created_widget_component (`self.CapsuleComponent`) "None" "SnapToTarget" "SnapToTarget" "SnapToTarget" true)))
    (else
      (`/Engine/EditorBlueprintResources/StandardMacros.IsValid` _created_widget_component_2
        (:`Is Valid`
          (`ActorComponent.K2_DestroyComponent` _created_widget_component_2))))))

(event `/TempestCombatFramework/Interfaces/BPI_TargetingSystem.Offset Widget Location`
  (params (`New Offset Value` :type "Vector Structure"))
  (bind _created_widget_component (`self.Created Widget Component`))
  (`/Engine/EditorBlueprintResources/StandardMacros.IsValid` (`self.Created Widget Component`)
    (:`Is Valid`
      (if (== `New Offset Value` (0.0 0.0 0.0))
        (bind (_direction _alpha) (`Timeline|Move Widget Component` :!via `Reverse` :!label _label)
          (:`Update`
            (`SceneComponent.K2_SetRelativeLocation` _created_widget_component (`KismetMathLibrary.VLerp` (0.0 0.0 0.0) (+ (`SceneComponent.RelativeLocation` _created_widget_component) `New Offset Value`) _alpha) false true)))
        (else
          (goto _label :!via `PlayFromStart`))))))

(fn `Get Enemy Data Asset`
  (returns (`Enemy Info` :type "/TempestCombatFramework/DataAssets/DA_Enemyinfo Object Reference"))
  (return (`self.Enemy Info Ref`)))

(fn `Get Enemy Spawn Info`
  (returns (`Enemy Spawn Info` :type "/TempestCombatFramework/StructuresEnums/S_Enemy_SpawnInfo Structure"))
  (return (`self.Enemy Spawn Info`)))

(fn `Get Lock On Location`
  (returns (Location :type "Vector Structure"))
  (return (`self.K2_GetActorLocation`)))

(fn `UserConstructionScript`)