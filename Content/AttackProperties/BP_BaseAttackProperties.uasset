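; Base attack property Blueprint that resolves how a hit lands and scales the damage it applies.
; On processing, it takes the impact result from the hit actor's TempestCombatComponent defense property and selects that result's damage applications.
; Each amount is multiplied by the owner's attributes matching its modifier gameplay tags, via TempestAttributesComponents.
; Scaled amounts overwrite that result's entry in the damage map.
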(event `self.ConstructAttackPropertry`)

(event `self.ProcessAttackPropertry`
  (bind _hit_target_defense_property (`self.Get Hit Target Defense Property`))
  (`/Engine/EditorBlueprintResources/StandardMacros.IsValid` (`self.GetAttackPropertyOwner`)
    (:`Is Valid`
      (`/Engine/EditorBlueprintResources/StandardMacros.IsValid` _hit_target_defense_property
        (:`Is Valid`
          (`self.SetImpactResult` (`TempestDefensePropertiesObject.ImpactResult` _hit_target_defense_property))
          (`self.Set Attack Impact Values`))))))

(fn `Get Hit Target Defense Property`
  (returns (`Hit Target Defense Property` :type "TempestDefensePropertiesObject Object Reference"))
  (bind _returnvalue (`Actor.GetComponentByClass` (`.HitActor` (`GameplayStatics.BreakHitResult` (`self.GetHitResult`))) "/Script/TempestCombatFramework.TempestCombatComponent"))
  (`/Engine/EditorBlueprintResources/StandardMacros.IsValid` _returnvalue
    (:`Is Valid`
      (return (`TempestCombatComponent.OwnerDefenseProperty` _returnvalue)))
    (:`Is Not Valid`
      (return null))))

(fn `Influence Attribute Value To Apply`
  (params (GameplayTags :type "Array of GameplayTag Structure") (`Amount To Apply` :type "Float (double-precision)"))
  (returns (`Return Value` :type "Float (double-precision)"))
  (locals (`Local Attributes Component` :type "TempestAttributesComponents Object Reference") (`Local Amount To Apply` :type "Float (double-precision)"))
  (if (> (`KismetArrayLibrary.Array_Length` GameplayTags) 0)
    (bind _output_get (set `local.Local Attributes Component` (`Actor.GetComponentByClass` (`self.GetAttackPropertyOwner`) "/Script/TempestCombatFramework.TempestAttributesComponents")))
    (`/Engine/EditorBlueprintResources/StandardMacros.IsValid` _output_get
      (:`Is Valid`
        (set `local.Local Amount To Apply` `Amount To Apply`)
        (for _array_element GameplayTags
          (bind _returnvalue (`TempestAttributesComponents.GetAttributeOfGameplayTag` (`local.Local Attributes Component`) _array_element))
          (`/Engine/EditorBlueprintResources/StandardMacros.IsValid` _returnvalue
            (:`Is Valid`
              (set `local.Local Amount To Apply` (* (`local.Local Amount To Apply`) (`.AttributeValue` (break `AttributeProperties` (`TempestBaseAttributeObject.AttributeValues` _returnvalue))))))))
        (return (`local.Local Amount To Apply`))))
    (else
      (return `Amount To Apply`))))

(fn `Set Attack Impact Values`
  (locals (`Local Damage To Apply` :type "Array of /TempestCombatFramework/StructuresEnums/S_DamageToApply Structure"))
  (bind _returnvalue (`self.GetImpactResult`))
  (bind _damage_applications_per_impact_result (`self.Damage Applications Per Impact Result`))
  (bind (_value _returnvalue_2) (`BlueprintMapLibrary.Map_Find` (`self.Damage Applications Per Impact Result`) (`self.GetImpactResult`)))
  (if _returnvalue_2
    (set `local.Local Damage To Apply` (`.DamageToApply_31_E5B87B0B4F2CC52CCF2141B256ECEE4A` (break `/TempestCombatFramework/StructuresEnums/S_DamageApplications` _value)))
    (for (_array_element _array_index) (`local.Local Damage To Apply`)
      (bind (_targetattributetoeffect _targetattributeamounttoapply _modifiedbyownerattributes) (break `/TempestCombatFramework/StructuresEnums/S_DamageToApply` _array_element))
      (bind _return_value (`self.Influence Attribute Value To Apply` (`BlueprintGameplayTagLibrary.BreakGameplayTagContainer` _modifiedbyownerattributes) _targetattributeamounttoapply))
      (setmembers `/TempestCombatFramework/StructuresEnums/S_DamageToApply` :`StructRef` (`|GetArrayItem` (`local.Local Damage To Apply`) _array_index) :`Target Attribute Amount To Apply` _return_value))
    (`BlueprintMapLibrary.Map_Remove` _damage_applications_per_impact_result _returnvalue)
    (`BlueprintMapLibrary.Map_Add` _damage_applications_per_impact_result _returnvalue (make `/TempestCombatFramework/StructuresEnums/S_DamageApplications` (`local.Local Damage To Apply`)))))