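; Player death state for the Tempest combat framework, eligible when a death ability can run and Health is at or below its minimum.
; On start it performs the selected death ability, tags the character State.Death and makes its mesh ignore the Pawn channel.
; It raises camera boom lag speed while preparing state values, lowers it when clearing them, and resets the selected ability on end.
; A delayed main-menu level load is present but unconnected.
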(event `self.StartState`
  (bind _selected_ability_to_trigger (`self.Get Selected Ability`))
  (`parent.StartState`)
  (if (`KismetSystemLibrary.IsValidClass` _selected_ability_to_trigger)
    (`TempestBaseAbilityManagerComponent.PerformAbilityOfClass` (`self.Tempest Ability System Component`) _selected_ability_to_trigger))
  (bind _astempest_base_character (cast `TempestBaseCharacter` (`self.Owner Character`)))
  (`BlueprintGameplayTagLibrary.AddGameplayTag` (`TempestBaseCharacter.ActorGameplayTags` _astempest_base_character) (struct :`TagName` "State.Death"))
  (`PrimitiveComponent.SetCollisionResponseToChannel` (`Character.Mesh` _astempest_base_character) "ECC_Pawn" "ECR_Ignore"))

(event `self.PrepareStateValues`
  (`parent.PrepareStateValues`)
  (bind _asbp_tcf_default_third_person_character (cast `/TempestCombatFramework/Characters/BP_TCF_DefaultThirdPersonCharacter` (`self.Owner Character`)))
  (set `SpringArmComponent.CameraLagSpeed` 15.0 (`/TempestCombatFramework/Characters/BP_TCF_DefaultThirdPersonCharacter.CameraBoom` _asbp_tcf_default_third_person_character)))

(event `self.ClearStateValues`
  (`parent.ClearStateValues`)
  (bind _asbp_tcf_default_third_person_character (cast `/TempestCombatFramework/Characters/BP_TCF_DefaultThirdPersonCharacter` (`self.Owner Character`)))
  (set `SpringArmComponent.CameraLagSpeed` 5.0 (`/TempestCombatFramework/Characters/BP_TCF_DefaultThirdPersonCharacter.CameraBoom` _asbp_tcf_default_third_person_character)))

(event `self.EndState`
  (`self.Set Selected Ability` null))

(fn `CanPerformState`
  (returns (ReturnValue :type Boolean))
  (bind (_attributevalue _minattributevalue) (break `AttributeProperties` (`TempestBaseAttributeObject.AttributeValues` (`TempestAttributesComponents.GetAttributeOfGameplayTag` (`Actor.GetComponentByClass` (`self.Owner Character`) "/Script/TempestCombatFramework.TempestAttributesComponents") (struct :`TagName` "Attribute.Health")))))
  (bind _return_value (`self.Check Abilities To Run` (`self.Death Abilities`)))
  (return (and _return_value (<= _attributevalue _minattributevalue))))