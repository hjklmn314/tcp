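; Player jumping state for the Tempest state manager, driving the owning character's jump.
; Starting the state calls Jump on the character.
; Each tick it looks up the state tagged State.Falling and tries to switch to it with a condition check.
; Ending the state stops the jump and runs the parent logic only if the state is currently active.
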(event `self.StartState`
  (`parent.StartState`)
  (`Character.Jump` (`self.Owner Character`)))

(event `self.TickState`
  (params (TickTime :type "Float (single-precision)"))
  (bind _tempest_state_manager_component (`self.Get Tempest State Manager Component`))
  (`TempestBaseStateManagerComponent.TryPerformStateOfClass` _tempest_state_manager_component (`GameplayStatics.GetObjectClass` (`TempestBaseStateManagerComponent.GetStateOfGameplayTag` _tempest_state_manager_component (struct :`TagName` "State.Falling"))) true))

(event `self.EndState`
  (if (`self.Get Is State Currentely Active`)
    (`Character.StopJumping` (`self.Owner Character`))
    (`parent.EndState`)))