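; Player state for deflecting, run through the Tempest state manager and ability system.
; It can start only when a check of its deflect abilities passes, then performs the selected ability and sets up allowed inputs with the movement axes.
; On ending it attempts a condition-checked switch to the Idle state and assigns a moveset message to the character's anim instance.
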(event `self.StartState`
  (`parent.StartState`)
  (`TempestBaseAbilityManagerComponent.PerformAbilityOfClass` (`self.Tempest Ability System Component`) (`self.Get Selected Ability`))
  (`self.Construct Default Allowed Inputs` (`|MakeArray` "/TempestCombatFramework/Input/MoveForwardBackward_Input.MoveForwardBackward_Input" "/TempestCombatFramework/Input/MoveRightLeft_Input.MoveRightLeft_Input" :!type "InputAction Object Reference")))

(event `self.EndState`
  (bind _tempest_state_manager_component (`self.Get Tempest State Manager Component`))
  (`parent.EndState`)
  (`TempestBaseStateManagerComponent.TryPerformStateOfClass` _tempest_state_manager_component (`GameplayStatics.GetObjectClass` (`TempestBaseStateManagerComponent.GetStateOfGameplayTag` _tempest_state_manager_component (struct :`TagName` "State.Idle"))) true)
  (message `/TempestCombatFramework/Interfaces/BPI_GeneralInterface.Assign Moveset` (`SkeletalMeshComponent.GetAnimInstance` (`Character.Mesh` (`self.Owner Character`))) "NewEnumerator1"))

(fn `CanPerformState`
  (returns (ReturnValue :type Boolean))
  (bind _return_value (`self.Check Abilities To Run` (`self.Deflect Abilities`)))
  (return _return_value))