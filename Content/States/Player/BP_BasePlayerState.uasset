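; Base player state that caches the owning Character with its Tempest ability and targeting components, and manages input allowance and buffering.
; A default NoBuffer object defines allowed inputs, though the permission check returns after the first buffering object.
; Other buffering objects can save input, and are removed when buffered input fires or state values clear.
; A helper yaw-lerps the character toward its targeted actor.
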(event `self.ConstructState`
  (`parent.ConstructState`)
  (bind _ascharacter (cast `Character` (`self.GetPerformingActor`)))
  (bind _output_get (set `self.Owner Character` _ascharacter))
  (set `self.Tempest Ability System Component` (`Actor.GetComponentByClass` _output_get "/Script/TempestCombatFramework.TempestBaseAbilityManagerComponent"))
  (set `self.Tempest Targeting Systen Component` (`Actor.GetComponentByClass` (`self.Owner Character`) "/Script/TempestCombatFramework.TempestTargetingComponent")))

(event `self.StartState`
  (`parent.StartState`))

(event `self.ClearStateValues`
  (`parent.ClearStateValues`)
  (`self.Set Buffered Input` null)
  (`self.Remove All None Buffering Objects`))

(event `Fire Buffered Input`
  (`self.Remove All None Buffering Objects`))

(fn `Add Buffering Object`
  (params (`New Buffer Object` :type "/TempestCombatFramework/Input/BP_BaseBufferingObject Object Reference"))
  (`KismetArrayLibrary.Array_AddUnique` (`self.Buffering Objects`) `New Buffer Object`)
  (`/TempestCombatFramework/Input/BP_BaseBufferingObject.Set Base State To Effect` `New Buffer Object` self))

(fn `Construct Default Allowed Inputs`
  (params (`Allowed Input Actions` :type "Array of InputAction Object Reference"))
  (`/Engine/EditorBlueprintResources/StandardMacros.IsValid` (`self.Default Buffer Object`)
    (:`Is Not Valid`
      (bind _returnvalue (`|GenericCreateObject` :`self` (`self.Owner Character`) :`Class` "/TempestCombatFramework/Input/BP_BaseBufferingObject.BP_BaseBufferingObject_C" :`Allowed Input Actions` `Allowed Input Actions`))
      (bind _output_get (set `self.Default Buffer Object` _returnvalue))
      (`self.Add Buffering Object` _output_get)
      (`/TempestCombatFramework/Input/BP_BaseBufferingObject.Set Buffering State` (`self.Default Buffer Object`) "NoBuffer"))))

(fn `Get Buffered Input`
  (returns (`Buffered Input` :type "InputAction Object Reference"))
  (return (`self.Buffered Input`)))

(fn `Get Buffering Objects`
  (returns (`Buffering Objects` :type "Array of /TempestCombatFramework/Input/BP_BaseBufferingObject Object Reference"))
  (return (`self.Buffering Objects`)))

(fn `Get Can Allow State With Input`
  (params (`Input Action` :type "InputAction Object Reference (by ref)"))
  (returns (`Return Value` :type Boolean))
  (for _array_element (`self.Buffering Objects`)
    (if (and (`|EnumEquality` (`/TempestCombatFramework/Input/BP_BaseBufferingObject.Buffering State` _array_element) "NoBuffer") (`KismetArrayLibrary.Array_Contains` (`/TempestCombatFramework/Input/BP_BaseBufferingObject.Allowed Input Actions` _array_element) `Input Action`))
      (return true)
      (else
        (return false))))
  (return false))

(fn `Get Default Buffer Object`
  (returns (`Default Buffer Object` :type "/TempestCombatFramework/Input/BP_BaseBufferingObject Object Reference"))
  (return (`self.Default Buffer Object`)))

(fn `Modify Default Allowed Inputs`
  (params (`Allowed Input Actions` :type "Array of InputAction Object Reference"))
  (bind _default_buffer_object (`self.Default Buffer Object`))
  (`/Engine/EditorBlueprintResources/StandardMacros.IsValid` _default_buffer_object
    (:`Is Valid`
      (set `/TempestCombatFramework/Input/BP_BaseBufferingObject.Allowed Input Actions` `Allowed Input Actions` _default_buffer_object))))

(fn `Remove All None Buffering Objects`
  (locals (`Local Set To Remove` :type "Set of /TempestCombatFramework/Input/BP_BaseBufferingObject Object Reference"))
  (bind (_arrayindex _arrayelement) (`/Engine/EditorBlueprintResources/StandardMacros.ReverseForEachLoop` (`self.Buffering Objects`))
    (:`LoopBody`
      (if (`|EnumInequality` (`/TempestCombatFramework/Input/BP_BaseBufferingObject.Buffering State` _arrayelement) "NoBuffer")
        (`self.Remove Buffering Object` _arrayelement)))
    (:`Completed`
      (return))))

(fn `Remove Buffering Object`
  (params (`Buffer Object To Remove` :type "/TempestCombatFramework/Input/BP_BaseBufferingObject Object Reference"))
  (`KismetArrayLibrary.Array_RemoveItem` (`self.Buffering Objects`) `Buffer Object To Remove`))

(fn `Rotate To Targeted Actor`
  (params (Alpha :type "Float (single-precision)" :default 0.1))
  (bind _tempest_targeting_systen_component (`self.Tempest Targeting Systen Component`))
  (bind _owner_character (`self.Owner Character`))
  (bind _returnvalue (`Actor.K2_GetActorRotation` _owner_character))
  (bind (_returnvalue_roll _returnvalue_pitch _returnvalue_yaw) (`KismetMathLibrary.BreakRotator` (`KismetMathLibrary.RLerp` _returnvalue (`KismetMathLibrary.FindLookAtRotation` (`Actor.K2_GetActorLocation` _owner_character) (`Actor.K2_GetActorLocation` (`TempestTargetingComponent.GetTargetedActor` (`self.Tempest Targeting Systen Component`)))) Alpha true)))
  (`/Engine/EditorBlueprintResources/StandardMacros.IsValid` _tempest_targeting_systen_component
    (:`Is Valid`
      (`/Engine/EditorBlueprintResources/StandardMacros.IsValid` (`TempestTargetingComponent.GetTargetedActor` _tempest_targeting_systen_component)
        (:`Is Valid`
          (`Actor.K2_SetActorRotation` (`self.Owner Character`) (`KismetMathLibrary.MakeRotator` (.roll _returnvalue) (.pitch _returnvalue) _returnvalue_yaw) true))))))

(fn `Set Buffered Input`
  (params (`Buffered Input` :type "InputAction Object Reference"))
  (set `self.Buffered Input` `Buffered Input`))

(fn `Try Save As Buffered Input`
  (params (`Input Action To Save` :type "InputAction Object Reference (by ref)"))
  (for _array_element (`self.Buffering Objects`)
    (`/TempestCombatFramework/Input/BP_BaseBufferingObject.Try Save As Input Buffer` _array_element `Input Action To Save`)))