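; Player walking state for the Tempest state manager, allowed while the owning character has velocity and is not falling.
; On start it builds the allowed input list for movement, combat and utility actions and sets the walk speed.
; Each tick it rotates toward the targeted actor, then attempts a condition-checked switch to Falling, falling back to Idle.
; A Sprint transition node exists but is never executed.
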(event `self.StartState`
  (`parent.StartState`)
  (`self.Construct Default Allowed Inputs` (`|MakeArray` "/TempestCombatFramework/Input/Attack_Input.Attack_Input" "/TempestCombatFramework/Input/RightMouse_Input.RightMouse_Input" "/TempestCombatFramework/Input/Jump_Input.Jump_Input" "/TempestCombatFramework/Input/Sprint_Input.Sprint_Input" "/TempestCombatFramework/Input/MoveForwardBackward_Input.MoveForwardBackward_Input" "/TempestCombatFramework/Input/MoveRightLeft_Input.MoveRightLeft_Input" "/TempestCombatFramework/Input/Dodge_Input.Dodge_Input" "/TempestCombatFramework/Input/SpecialAttack_Input.SpecialAttack_Input" "/TempestCombatFramework/Input/EquipUnequip_Input.EquipUnequip_Input" "/TempestCombatFramework/Input/Heal_Input.Heal_Input" :!type "InputAction Object Reference"))
  (set `CharacterMovementComponent.MaxWalkSpeed` 600.0 (`Character.CharacterMovement` (`self.Owner Character`))))

(event `self.TickState`
  (params (TickTime :type "Float (single-precision)"))
  (bind _tempest_state_manager_component (`self.Get Tempest State Manager Component`))
  (bind _tempest_state_manager_component_2 (`self.Get Tempest State Manager Component`))
  (`parent.TickState` TickTime)
  (`self.Rotate To Targeted Actor` 0.1)
  (bind _returnvalue (`TempestBaseStateManagerComponent.TryPerformStateOfClass` _tempest_state_manager_component_2 (`GameplayStatics.GetObjectClass` (`TempestBaseStateManagerComponent.GetStateOfGameplayTag` _tempest_state_manager_component_2 (struct :`TagName` "State.Falling"))) true))
  (if (not _returnvalue)
    (bind _returnvalue_2 (`TempestBaseStateManagerComponent.TryPerformStateOfClass` _tempest_state_manager_component (`GameplayStatics.GetObjectClass` (`TempestBaseStateManagerComponent.GetStateOfGameplayTag` _tempest_state_manager_component (struct :`TagName` "State.Idle"))) true))
    (if (not _returnvalue_2)
      _)))

(fn `CanPerformState`
  (returns (ReturnValue :type Boolean))
  (return (and (> (`KismetMathLibrary.VSize` (`Actor.GetVelocity` (`self.Owner Character`))) 0.0) (not (`NavMovementComponent.IsFalling` (`Character.CharacterMovement` (`self.Owner Character`)))))))