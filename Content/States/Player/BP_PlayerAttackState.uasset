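; Player attack state for the Tempest state and ability framework, gated by its attack ability list.
; It runs the selected ability on start and requests Idle on end.
; Buffered inputs resolve to tags through the equipped weapon's data asset, then branch on the active ability.
; Attack re-triggers abilities, hold attack cancels light attack and restarts the state, and block, dodge or movement interrupt light attacks.
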(event `self.ConstructState`
  (`parent.ConstructState`)
  (set `self.Tempest Ability Component` (`Actor.GetComponentByClass` (`self.GetPerformingActor`) "/Script/TempestCombatFramework.TempestBaseAbilityManagerComponent")))

(event `self.StartState`
  (`parent.StartState`)
  (`TempestBaseAbilityManagerComponent.PerformAbilityOfClass` (`self.Tempest Ability Component`) (`self.Get Selected Ability`)))

(event `self.EndState`
  (bind _tempest_state_manager_component (`self.Get Tempest State Manager Component`))
  (`parent.EndState`)
  (`TempestBaseStateManagerComponent.TryPerformStateOfClass` _tempest_state_manager_component (`GameplayStatics.GetObjectClass` (`TempestBaseStateManagerComponent.GetStateOfGameplayTag` _tempest_state_manager_component (struct :`TagName` "State.Idle"))) true))

(event `self.Fire Buffered Input`
  (bind _buffered_input (`self.Get Buffered Input`))
  (bind _tempest_state_manager_component (`self.Get Tempest State Manager Component`))
  (bind _tempest_state_manager_component_2 (`self.Get Tempest State Manager Component`))
  (bind _tempest_ability_component (`self.Tempest Ability Component`))
  (bind _owner_character (`self.Owner Character`))
  (bind _returnvalue (`TempestBaseAbilityManagerComponent.GetCurrentActiveAbility` _tempest_ability_component))
  (bind _returnvalue_2 (`TempestBaseAbilityManagerComponent.GetCurrentActiveAbility` (`self.Tempest Ability Component`)))
  (bind _returnvalue_3 (`TempestBaseAbilityManagerComponent.GetCurrentActiveAbility` (`self.Tempest Ability Component`)))
  (bind _returnvalue_4 (`TempestBaseAbilityManagerComponent.GetCurrentActiveAbility` (`self.Tempest Ability Component`)))
  (bind _asbp_base_player_weapon (cast `/TempestCombatFramework/Actors/Weapons/Player/BP_BasePlayerWeapon` (`/TempestCombatFramework/Components/BP_TempestPlayerCombatComponent.Get Equipped Weapon` (`Actor.GetComponentByClass` _owner_character "/TempestCombatFramework/Components/BP_TempestPlayerCombatComponent.BP_TempestPlayerCombatComponent_C"))))
  (`/Engine/EditorBlueprintResources/StandardMacros.IsValid` _buffered_input
    (:`Is Valid`
      (bind _player_inputs (`/TempestCombatFramework/DataAssets/BasePlayer_PDA.Player Inputs` (`/TempestCombatFramework/Actors/Weapons/Player/BP_BasePlayerWeapon.Associated Data Asset` _asbp_base_player_weapon)))
      (bind _associated_tag (`/TempestCombatFramework/Libraries/BFL_TempestInputs.Get Input Tag Of Input Map` _player_inputs _buffered_input))
      (bind (_value _returnvalue_5) (`BlueprintMapLibrary.Map_Find` _player_inputs _associated_tag))
      (if _returnvalue_5
        (message `/TempestCombatFramework/Interfaces/BPI_PlayerInputs.Set Last Fired Input` (`Pawn.GetController` _owner_character) _value))
      (`|SwitchGameplayTag` _associated_tag
        (:`Input.Attack`
          (`|SwitchGameplayTag` (`TempestBaseAbilityObject.AbilityGameplayTag` _returnvalue)
            (:`Default`
              (`self.RestartState` true :!label _label))
            (:`Ability.Attack.LightAttack`
              (`TempestBaseAbilityObject.StartAbility` _returnvalue))))
        (:`Input.Block`
          (`|SwitchGameplayTag` (`TempestBaseAbilityObject.AbilityGameplayTag` _returnvalue_4)
            (:`Ability.Attack.LightAttack`
              (`TempestBaseAbilityObject.CancelAbility` _returnvalue_4)
              (`TempestBaseStateManagerComponent.TryPerformStateOfClass` _tempest_state_manager_component (`GameplayStatics.GetObjectClass` (`TempestBaseStateManagerComponent.GetStateOfGameplayTag` _tempest_state_manager_component (struct :`TagName` "State.Normal Block"))) true))))
        (:`Input.MoveForwardBackward`
          (`|SwitchGameplayTag` (`TempestBaseAbilityObject.AbilityGameplayTag` _returnvalue_3) :!label _label_2
            (:`Ability.Attack.LightAttack`
              (`Character.StopAnimMontage` (`self.Owner Character`) null)
              (`TempestBaseAbilityObject.EndAbility` _returnvalue_3))))
        (:`Input.MoveRightLeft`
          (goto _label_2))
        (:`Input.HoldAttack`
          (`TempestBaseAbilityObject.CancelAbility` (`TempestBaseAbilityManagerComponent.GetAbilityOfGameplayTag` _tempest_ability_component (struct :`TagName` "Ability.Attack.LightAttack")))
          (goto _label))
        (:`Input.Dodge`
          (`|SwitchGameplayTag` (`TempestBaseAbilityObject.AbilityGameplayTag` _returnvalue_2)
            (:`Ability.Attack.LightAttack`
              (`TempestBaseAbilityObject.CancelAbility` _returnvalue_2)
              (`TempestBaseStateManagerComponent.TryPerformStateOfClass` _tempest_state_manager_component_2 (`GameplayStatics.GetObjectClass` (`TempestBaseStateManagerComponent.GetStateOfGameplayTag` _tempest_state_manager_component_2 (struct :`TagName` "State.Dodge"))) true)))))
      (`self.Set Buffered Input` null)
      (`self.Remove All None Buffering Objects`))))

(fn `CanPerformState`
  (returns (ReturnValue :type Boolean))
  (bind _return_value (`self.Check Abilities To Run` (`self.Attack Abilities`)))
  (return _return_value))