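; Player falling state for a state-manager-driven character, representing the descending part of airborne movement.
; It can be performed only while the owner's movement component reports falling and vertical velocity is negative.
; Each tick it runs the parent logic, then asks the Tempest state manager to switch to Idle, Walk or Sprint, in that priority, stopping at the first whose condition check passes.
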(event `self.TickState`
  (params (TickTime :type "Float (single-precision)"))
  (bind _tempest_state_manager_component (`self.Get Tempest State Manager Component`))
  (bind _tempest_state_manager_component_2 (`self.Get Tempest State Manager Component`))
  (bind _tempest_state_manager_component_3 (`self.Get Tempest State Manager Component`))
  (`parent.TickState` TickTime)
  (bind _returnvalue (`TempestBaseStateManagerComponent.TryPerformStateOfClass` _tempest_state_manager_component_3 (`GameplayStatics.GetObjectClass` (`TempestBaseStateManagerComponent.GetStateOfGameplayTag` _tempest_state_manager_component_3 (struct :`TagName` "State.Idle"))) true))
  (if (not _returnvalue)
    (bind _returnvalue_2 (`TempestBaseStateManagerComponent.TryPerformStateOfClass` _tempest_state_manager_component_2 (`GameplayStatics.GetObjectClass` (`TempestBaseStateManagerComponent.GetStateOfGameplayTag` _tempest_state_manager_component_2 (struct :`TagName` "State.Walk"))) true))
    (if (not _returnvalue_2)
      (`TempestBaseStateManagerComponent.TryPerformStateOfClass` _tempest_state_manager_component (`GameplayStatics.GetObjectClass` (`TempestBaseStateManagerComponent.GetStateOfGameplayTag` _tempest_state_manager_component (struct :`TagName` "State.Sprint"))) true))))

(fn `CanPerformState`
  (returns (ReturnValue :type Boolean))
  (bind _owner_character (`self.Owner Character`))
  (return (and (`NavMovementComponent.IsFalling` (`Character.CharacterMovement` _owner_character)) (< (.z (`Actor.GetVelocity` _owner_character)) 0.0))))