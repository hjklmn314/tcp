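; Player "Convert" state built on the Tempest state manager and ability system, which runs the selected ability while active.
; Entry is gated by an ability check on EquipAbility, while StartState performs whatever GetSelectedAbility returns.
; It sets the default allowed inputs to the two movement axes.
; On end, it tries a condition-checked switch to the state tagged State.Idle.
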(event `self.StartState`
  (`parent.StartState`)
  (`TempestBaseAbilityManagerComponent.PerformAbilityOfClass` (`self.Tempest Ability System Component`) (`self.Get Selected Ability`))
  (`self.Construct Default Allowed Inputs` (`|MakeArray` "/TempestCombatFramework/Input/MoveForwardBackward_Input.MoveForwardBackward_Input" "/TempestCombatFramework/Input/MoveRightLeft_Input.MoveRightLeft_Input" :!type "InputAction Object Reference")))

(event `self.EndState`
  (bind _tempest_state_manager_component (`self.Get Tempest State Manager Component`))
  (`parent.EndState`)
  (`TempestBaseStateManagerComponent.TryPerformStateOfClass` _tempest_state_manager_component (`GameplayStatics.GetObjectClass` (`TempestBaseStateManagerComponent.GetStateOfGameplayTag` _tempest_state_manager_component (struct :`TagName` "State.Idle"))) true))

(fn `CanPerformState`
  (returns (ReturnValue :type Boolean))
  (bind _return_value (`self.Check Abilities To Run` (`|MakeArray` (`self.Equip Ability`))))
  (return _return_value))