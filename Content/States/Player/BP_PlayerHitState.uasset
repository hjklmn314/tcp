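; Player hit-reaction state in the Tempest state and ability system, blocked while the player is in the Death state.
; On start it cancels attack abilities, runs the selected hit ability and, if out of combat, attaches weapons and enters combat.
; Buffered dodge input can switch from hit react to the Dodge state, while movement input ends the reaction early.
; On end it attempts to return to Idle.
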(event `self.StartState`
  (bind _owner_character (`self.Owner Character`))
  (bind _returnvalue (`Actor.GetComponentByClass` _owner_character "/TempestCombatFramework/Components/BP_TempestBaseCombatComponent.BP_TempestBaseCombatComponent_C"))
  (`parent.StartState`)
  (`self.Cancel Attack Abilities`)
  (`TempestBaseAbilityManagerComponent.PerformAbilityOfClass` (`self.Tempest Ability System Component`) (`self.Get Selected Ability`))
  (if (not (`BlueprintGameplayTagLibrary.HasTag` (`TempestCombatComponent.GetCombatStatus` _returnvalue) (struct :`TagName` "Status.Combat.InCombat")))
    (`/TempestCombatFramework/Actors/Weapons/BP_BaseWeapon.Attach All Weapon` (`/TempestCombatFramework/Components/BP_TempestBaseCombatComponent.Get Equipped Weapon` _returnvalue) true)
    (`TempestCombatComponent.ModifyCombatStatus` _returnvalue (struct :`TagName` "Status.Combat.InCombat") "Add")
    (message `/TempestCombatFramework/Interfaces/BPI_GeneralInterface.Assign Moveset` (`SkeletalMeshComponent.GetAnimInstance` (`Character.Mesh` _owner_character)) "NewEnumerator1")))

(event `self.EndState`
  (bind _tempest_state_manager_component (`self.Get Tempest State Manager Component`))
  (`parent.EndState`)
  (`TempestBaseStateManagerComponent.TryPerformStateOfClass` _tempest_state_manager_component (`GameplayStatics.GetObjectClass` (`TempestBaseStateManagerComponent.GetStateOfGameplayTag` _tempest_state_manager_component (struct :`TagName` "State.Idle"))) true))

(event `self.Fire Buffered Input`
  (bind _buffered_input (`self.Get Buffered Input`))
  (bind _tempest_state_manager_component (`self.Get Tempest State Manager Component`))
  (bind _owner_character (`self.Owner Character`))
  (bind _asbp_base_player_weapon (cast `/TempestCombatFramework/Actors/Weapons/Player/BP_BasePlayerWeapon` (`/TempestCombatFramework/Components/BP_TempestPlayerCombatComponent.Get Equipped Weapon` (`Actor.GetComponentByClass` _owner_character "/TempestCombatFramework/Components/BP_TempestPlayerCombatComponent.BP_TempestPlayerCombatComponent_C"))))
  (`/Engine/EditorBlueprintResources/StandardMacros.IsValid` _buffered_input
    (:`Is Valid`
      (bind _player_inputs (`/TempestCombatFramework/DataAssets/BasePlayer_PDA.Player Inputs` (`/TempestCombatFramework/Actors/Weapons/Player/BP_BasePlayerWeapon.Associated Data Asset` _asbp_base_player_weapon)))
      (bind _associated_tag (`/TempestCombatFramework/Libraries/BFL_TempestInputs.Get Input Tag Of Input Map` _player_inputs _buffered_input))
      (bind (_value _returnvalue) (`BlueprintMapLibrary.Map_Find` _player_inputs _associated_tag))
      (if _returnvalue
        (message `/TempestCombatFramework/Interfaces/BPI_PlayerInputs.Set Last Fired Input` (`Pawn.GetController` _owner_character) _value))
      (`|SwitchGameplayTag` _associated_tag
        (:`Input.Dodge`
          (`|SwitchGameplayTag` (`TempestBaseAbilityObject.AbilityGameplayTag` (`TempestBaseAbilityManagerComponent.GetCurrentActiveAbility` (`self.Tempest Ability System Component`)))
            (:`Ability.Hit React`
              (`TempestBaseStateManagerComponent.TryPerformStateOfClass` _tempest_state_manager_component (`GameplayStatics.GetObjectClass` (`TempestBaseStateManagerComponent.GetStateOfGameplayTag` _tempest_state_manager_component (struct :`TagName` "State.Dodge"))) true))))
        (:`Input.MoveForwardBackward`
          (`Character.StopAnimMontage` (`self.Owner Character`) null :!label _label)
          (`TempestBaseAbilityObject.EndAbility` (`TempestBaseAbilityManagerComponent.GetCurrentActiveAbility` (`self.Tempest Ability System Component`))))
        (:`Input.MoveRightLeft`
          (goto _label)))
      (`self.Set Buffered Input` null)
      (`self.Remove All None Buffering Objects`))))

(fn `Cancel Attack Abilities`
  (bind _tempest_ability_system_component (`self.Tempest Ability System Component`))
  (bind _returnvalue (`TempestBaseAbilityManagerComponent.GetAbilityOfGameplayTag` _tempest_ability_system_component (struct :`TagName` "Ability.Attack.HeavyAttack")))
  (bind _returnvalue_2 (`TempestBaseAbilityManagerComponent.GetAbilityOfGameplayTag` _tempest_ability_system_component (struct :`TagName` "Ability.Attack.LightAttack")))
  (bind _returnvalue_3 (`TempestBaseAbilityManagerComponent.GetAbilityOfGameplayTag` _tempest_ability_system_component (struct :`TagName` "Ability.Attack.SpecialAttack")))
  (`|ExecutionSequence`
    (:`then_0`
      (`/Engine/EditorBlueprintResources/StandardMacros.IsValid` _returnvalue
        (:`Is Valid`
          (`TempestBaseAbilityObject.CancelAbility` _returnvalue))))
    (:`then_1`
      (`/Engine/EditorBlueprintResources/StandardMacros.IsValid` _returnvalue_2
        (:`Is Valid`
          (`TempestBaseAbilityObject.CancelAbility` _returnvalue_2))))
    (:`then_2`
      (`/Engine/EditorBlueprintResources/StandardMacros.IsValid` _returnvalue_3
        (:`Is Valid`
          (`TempestBaseAbilityObject.CancelAbility` _returnvalue_3))))))

(fn `CanPerformState`
  (returns (ReturnValue :type Boolean))
  (bind _tempest_ability_system_component (`self.Tempest Ability System Component`))
  (`/Engine/EditorBlueprintResources/StandardMacros.IsValid` (`TempestBaseStateManagerComponent.GetCurrentActiveState` (`self.Get Tempest State Manager Component`))
    (:`Is Valid`
      (if (!= (`TempestBaseStateObject.StateGameplayTag` (`TempestBaseStateManagerComponent.GetCurrentActiveState` (`self.Get Tempest State Manager Component`))) (struct :`TagName` "State.Death"))
        (`/Engine/EditorBlueprintResources/StandardMacros.IsValid` (`TempestBaseAbilityManagerComponent.GetAbilityOfGameplayTag` _tempest_ability_system_component (struct :`TagName` "Ability.Hit React.IK"))
          (:`Is Valid`
            _)
          (:`Is Not Valid`
            (`TempestBaseAbilityManagerComponent.ConstructAbilityOfClass` _tempest_ability_system_component (`self.IK Hit React`))))
        (bind _return_value (`self.Check Abilities To Run` (`self.Hit Abilities`)))
        (return _return_value)
        (else
          (return false))))
    (:`Is Not Valid`
      (return false))))