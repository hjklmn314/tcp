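; Player idle state in a Tempest state manager, valid only while the owning character's velocity is zero.
; On start it registers the default set of allowed player inputs, covering movement, combat, dodge, equip and heal.
; Each tick it condition-checks a switch to the Falling state and, if that fails, tries the Walk state, both looked up by gameplay tag.
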(event `self.StartState`
  (`parent.StartState`)
  (`self.Construct Default Allowed Inputs` (`|MakeArray` "/TempestCombatFramework/Input/Attack_Input.Attack_Input" "/TempestCombatFramework/Input/RightMouse_Input.RightMouse_Input" "/TempestCombatFramework/Input/Jump_Input.Jump_Input" "/TempestCombatFramework/Input/Sprint_Input.Sprint_Input" "/TempestCombatFramework/Input/MoveForwardBackward_Input.MoveForwardBackward_Input" "/TempestCombatFramework/Input/MoveRightLeft_Input.MoveRightLeft_Input" "/TempestCombatFramework/Input/Dodge_Input.Dodge_Input" "/TempestCombatFramework/Input/SpecialAttack_Input.SpecialAttack_Input" "/TempestCombatFramework/Input/EquipUnequip_Input.EquipUnequip_Input" "/TempestCombatFramework/Input/Heal_Input.Heal_Input" :!type "InputAction Object Reference")))

(event `self.TickState`
  (params (TickTime :type "Float (single-precision)"))
  (bind _tempest_state_manager_component (`self.Get Tempest State Manager Component`))
  (bind _tempest_state_manager_component_2 (`self.Get Tempest State Manager Component`))
  (`parent.TickState` TickTime)
  (bind _returnvalue (`TempestBaseStateManagerComponent.TryPerformStateOfClass` _tempest_state_manager_component_2 (`GameplayStatics.GetObjectClass` (`TempestBaseStateManagerComponent.GetStateOfGameplayTag` _tempest_state_manager_component_2 (struct :`TagName` "State.Falling"))) true))
  (if (not _returnvalue)
    (`TempestBaseStateManagerComponent.TryPerformStateOfClass` _tempest_state_manager_component (`GameplayStatics.GetObjectClass` (`TempestBaseStateManagerComponent.GetStateOfGameplayTag` _tempest_state_manager_component (struct :`TagName` "State.Walk"))) true)))

(fn `CanPerformState`
  (returns (ReturnValue :type Boolean))
  (return (== (`KismetMathLibrary.VSize` (`Actor.GetVelocity` (`self.Owner Character`))) 0.0)))