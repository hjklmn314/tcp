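; Player dodge state that runs a selected dodge ability and attempts to return to Idle when it ends.
; Entry is gated by a check on the dodge abilities.
; Buffered input is resolved to a tag through the equipped weapon's input map, and its message is recorded on the controller.
; Buffered movement input during an active dodge cancels the montage and ability, then clears the buffer.
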(event `self.StartState`
  (`parent.StartState`)
  (`TempestBaseAbilityManagerComponent.PerformAbilityOfClass` (`self.Tempest Ability System Component`) (`self.Get Selected Ability`)))

(event `self.EndState`
  (bind _tempest_state_manager_component (`self.Get Tempest State Manager Component`))
  (`parent.EndState`)
  (`TempestBaseStateManagerComponent.TryPerformStateOfClass` _tempest_state_manager_component (`GameplayStatics.GetObjectClass` (`TempestBaseStateManagerComponent.GetStateOfGameplayTag` _tempest_state_manager_component (struct :`TagName` "State.Idle"))) true))

(event `self.Fire Buffered Input`
  (bind _buffered_input (`self.Get Buffered Input`))
  (bind _owner_character (`self.Owner Character`))
  (bind _returnvalue (`TempestBaseAbilityManagerComponent.GetCurrentActiveAbility` (`self.Tempest Ability System Component`)))
  (bind _asbp_base_player_weapon (cast `/TempestCombatFramework/Actors/Weapons/Player/BP_BasePlayerWeapon` (`/TempestCombatFramework/Components/BP_TempestPlayerCombatComponent.Get Equipped Weapon` (`Actor.GetComponentByClass` _owner_character "/TempestCombatFramework/Components/BP_TempestPlayerCombatComponent.BP_TempestPlayerCombatComponent_C"))))
  (`/Engine/EditorBlueprintResources/StandardMacros.IsValid` _buffered_input
    (:`Is Valid`
      (bind _player_inputs (`/TempestCombatFramework/DataAssets/BasePlayer_PDA.Player Inputs` (`/TempestCombatFramework/Actors/Weapons/Player/BP_BasePlayerWeapon.Associated Data Asset` _asbp_base_player_weapon)))
      (bind _associated_tag (`/TempestCombatFramework/Libraries/BFL_TempestInputs.Get Input Tag Of Input Map` _player_inputs _buffered_input))
      (bind (_value _returnvalue_2) (`BlueprintMapLibrary.Map_Find` _player_inputs _associated_tag))
      (if _returnvalue_2
        (message `/TempestCombatFramework/Interfaces/BPI_PlayerInputs.Set Last Fired Input` (`Pawn.GetController` _owner_character) _value))
      (`|SwitchGameplayTag` _associated_tag
        (:`Input.MoveForwardBackward`
          _)
        (:`Input.MoveRightLeft`
          _))
      (`|SwitchGameplayTag` (`TempestBaseAbilityObject.AbilityGameplayTag` _returnvalue)
        (:`Ability.Dodge`
          (`Character.StopAnimMontage` (`self.Owner Character`) null)
          (`TempestBaseAbilityObject.EndAbility` _returnvalue)
          (`self.Set Buffered Input` null)
          (`parent.Fire Buffered Input`))))))

(fn `CanPerformState`
  (returns (ReturnValue :type Boolean))
  (bind _return_value (`self.Check Abilities To Run` (`self.Dodge Abilities`)))
  (return _return_value))