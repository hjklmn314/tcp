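; Player block state for the Tempest state machine: runs block abilities while right mouse is held, with reduced walk speed and a block moveset.
; While moving, it rotates toward the targeted actor.
; Releasing during Block Start returns to Idle; during Block Loop it plays Block End, falling back to Idle.
; A looping timer, started at construction, tracks time without block input during Deflect or Block Hit states, otherwise resetting it.
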(event `self.ConstructState`
  (bind _tempest_ability_system_component (`self.Tempest Ability System Component`))
  (`parent.ConstructState`)
  (bind _asplayer_controller (cast `PlayerController` (`Pawn.GetController` (`self.Owner Character`))))
  (set `self.Owner Player Controller` _asplayer_controller)
  (for _array_element (`self.Block Abilities`)
    (`/Engine/EditorBlueprintResources/StandardMacros.IsValid` (`TempestBaseAbilityManagerComponent.GetAbilityOfClass` _tempest_ability_system_component _array_element)
      (:`Is Not Valid`
        (`TempestBaseAbilityManagerComponent.ConstructAbilityOfClass` _tempest_ability_system_component _array_element))))
  (`self.Construct Default Allowed Inputs` (`|MakeArray` "/TempestCombatFramework/Input/MoveForwardBackward_Input.MoveForwardBackward_Input" "/TempestCombatFramework/Input/MoveRightLeft_Input.MoveRightLeft_Input" "/TempestCombatFramework/Input/RightMouse_Input.RightMouse_Input" :!type "InputAction Object Reference"))
  (`KismetSystemLibrary.K2_SetTimer` null "Calculate Block Time" 0.0167 true))

(event `self.StartState`
  (`parent.StartState`)
  (bind _mapping_context (message `/TempestCombatFramework/Interfaces/BPI_PlayerInputs.Get Mapping Context` (`self.Owner Player Controller`)))
  (set `self.Input Actions Keys` (`/TempestCombatFramework/Libraries/BFL_TempestInputs.Get Keys Of Input Action` _mapping_context "/TempestCombatFramework/Input/RightMouse_Input.RightMouse_Input"))
  (`TempestBaseAbilityManagerComponent.PerformAbilityOfClass` (`self.Tempest Ability System Component`) (`self.Get Selected Ability`))
  (message `/TempestCombatFramework/Interfaces/BPI_GeneralInterface.Assign Moveset` (`SkeletalMeshComponent.GetAnimInstance` (`Character.Mesh` (`self.Owner Character`))) "NewEnumerator3"))

(event `self.PrepareStateValues`
  (`parent.PrepareStateValues`)
  (set `CharacterMovementComponent.MaxWalkSpeed` 200.0 (`Character.CharacterMovement` (`self.Owner Character`))))

(event `self.TickState`
  (params (TickTime :type "Float (single-precision)"))
  (bind _tempest_ability_system_component (`self.Tempest Ability System Component`))
  (bind _abilitygameplaytag (`TempestBaseAbilityObject.AbilityGameplayTag` (`TempestBaseAbilityManagerComponent.GetCurrentActiveAbility` (`self.Tempest Ability System Component`))))
  (bind _returnvalue (== _abilitygameplaytag (struct :`TagName` "Ability.Block.Start")))
  (if (> (`KismetMathLibrary.VSize` (`Actor.GetVelocity` (`self.Owner Character`))) 0.0)
    (`self.Rotate To Targeted Actor` 0.1))
  (if (or (== _abilitygameplaytag (struct :`TagName` "Ability.Block.Loop")) _returnvalue)
    (if (not (`self.Input Still Clicked`))
      (if _returnvalue
        (`self.EndState` :!label _label)
        (else
          (bind _returnvalue_2 (`TempestBaseAbilityManagerComponent.TryPerformAbilityOfClass` _tempest_ability_system_component (`GameplayStatics.GetObjectClass` (`TempestBaseAbilityManagerComponent.GetAbilityOfGameplayTag` _tempest_ability_system_component (struct :`TagName` "Ability.Block.End"))) true))
          (if (not _returnvalue_2)
            (goto _label)))))))

(event `self.ClearStateValues`
  (`parent.ClearStateValues`)
  (message `/TempestCombatFramework/Interfaces/BPI_GeneralInterface.Assign Moveset` (`SkeletalMeshComponent.GetAnimInstance` (`Character.Mesh` (`self.Owner Character`))) "NewEnumerator1"))

(event `self.EndState`
  (bind _tempest_state_manager_component (`self.Get Tempest State Manager Component`))
  (`parent.EndState`)
  (`TempestBaseStateManagerComponent.TryPerformStateOfClass` _tempest_state_manager_component (`GameplayStatics.GetObjectClass` (`TempestBaseStateManagerComponent.GetStateOfGameplayTag` _tempest_state_manager_component (struct :`TagName` "State.Idle"))) true))

(fn `Calculate Block Time`
  (bind _returnvalue (`TempestBaseStateManagerComponent.GetCurrentActiveState` (`self.Get Tempest State Manager Component`)))
  (`/Engine/EditorBlueprintResources/StandardMacros.IsValid` _returnvalue
    (:`Is Valid`
      (bind _mapping_context (message `/TempestCombatFramework/Interfaces/BPI_PlayerInputs.Get Mapping Context` (`self.Owner Player Controller`)))
      (`|SwitchGameplayTag` (`TempestBaseStateObject.StateGameplayTag` _returnvalue)
        (:`Default`
          (set `self.Block Time` -1.0))
        (:`State.Deflect`
          (bind _return_value (`/TempestCombatFramework/Libraries/BFL_TempestInputs.Get Is Input Clicked` _mapping_context "/TempestCombatFramework/Input/RightMouse_Input.RightMouse_Input" (`self.Owner Player Controller`)))
          (if _return_value
            (set `self.Block Time` -1.0 :!label _label)
            (else
              (if (== (`self.Block Time`) -1.0) :!label _label_2
                (set `self.Block Time` 0.0))
              (set `self.Block Time` (+ (`GameplayStatics.GetWorldDeltaSeconds`) (`self.Block Time`))))))
        (:`State.BlockHit`
          (if _return_value
            (goto _label)
            (else
              (goto _label_2))))))))

(fn `CanPerformState`
  (returns (ReturnValue :type Boolean))
  (bind _return_value (`self.Check Abilities To Run` (`|MakeArray` (`|GetArrayItem` (`self.Block Abilities`)))))
  (return _return_value))

(fn `Get Block Time Since Last Clicked`
  (returns (`Return Value` :type "Float (double-precision)"))
  (return (`self.Block Time`)))

(fn `Get Montage Counter For Ability`
  (returns (`Counter Montage` :type "AnimMontage Object Reference"))
  (return null))

(fn `Input Still Clicked`
  (returns (ReturnValue :type Boolean))
  (for _array_element (`self.Input Actions Keys`)
    (if (`PlayerController.IsInputKeyDown` (`self.Owner Player Controller`) _array_element)
      (return true)))
  (return false))