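; Player state for sprinting in the Tempest state manager, enterable only from the Walk state while the character is not falling.
; On start it sets the allowed inputs and raises or sets max walk speed to the sprinting speed.
; Each tick it rotates toward the targeted actor, then attempts transitions to Falling, then Idle, and falls back to trying Walk when Sprint input is not among the pressed actions.
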(event `self.ConstructState`
  (`parent.ConstructState`)
  (bind _asplayer_controller (cast `PlayerController` (`Pawn.GetController` (`self.Owner Character`))))
  (set `self.Owner Player Controller` _asplayer_controller))

(event `self.StartState`
  (`parent.StartState`)
  (`self.Construct Default Allowed Inputs` (`|MakeArray` "/TempestCombatFramework/Input/Attack_Input.Attack_Input" "/TempestCombatFramework/Input/RightMouse_Input.RightMouse_Input" "/TempestCombatFramework/Input/Jump_Input.Jump_Input" "/TempestCombatFramework/Input/Sprint_Input.Sprint_Input" "/TempestCombatFramework/Input/MoveForwardBackward_Input.MoveForwardBackward_Input" "/TempestCombatFramework/Input/MoveRightLeft_Input.MoveRightLeft_Input" "/TempestCombatFramework/Input/Dodge_Input.Dodge_Input" "/TempestCombatFramework/Input/SpecialAttack_Input.SpecialAttack_Input" "/TempestCombatFramework/Input/EquipUnequip_Input.EquipUnequip_Input" "/TempestCombatFramework/Input/Heal_Input.Heal_Input" :!type "InputAction Object Reference"))
  (set `CharacterMovementComponent.MaxWalkSpeed` (`self.Sprinting Speed`) (`Character.CharacterMovement` (`self.Owner Character`))))

(event `self.TickState`
  (params (TickTime :type "Float (single-precision)"))
  (bind _tempest_state_manager_component (`self.Get Tempest State Manager Component`))
  (bind _tempest_state_manager_component_2 (`self.Get Tempest State Manager Component`))
  (bind _tempest_state_manager_component_3 (`self.Get Tempest State Manager Component`))
  (bind _owner_player_controller (`self.Owner Player Controller`))
  (`parent.TickState` TickTime)
  (`self.Rotate To Targeted Actor` 0.1)
  (bind _returnvalue (`TempestBaseStateManagerComponent.TryPerformStateOfClass` _tempest_state_manager_component_3 (`GameplayStatics.GetObjectClass` (`TempestBaseStateManagerComponent.GetStateOfGameplayTag` _tempest_state_manager_component_3 (struct :`TagName` "State.Falling"))) true))
  (if (not _returnvalue)
    (bind _returnvalue_2 (`TempestBaseStateManagerComponent.TryPerformStateOfClass` _tempest_state_manager_component_2 (`GameplayStatics.GetObjectClass` (`TempestBaseStateManagerComponent.GetStateOfGameplayTag` _tempest_state_manager_component_2 (struct :`TagName` "State.Idle"))) true))
    (if (not _returnvalue_2)
      (bind _mapping_context (message `/TempestCombatFramework/Interfaces/BPI_PlayerInputs.Get Mapping Context` _owner_player_controller))
      (if (not (`KismetArrayLibrary.Array_Contains` (`/TempestCombatFramework/Libraries/BFL_TempestInputs.Get Pressed Input Actions` _mapping_context _owner_player_controller) "/TempestCombatFramework/Input/Sprint_Input.Sprint_Input"))
        (`TempestBaseStateManagerComponent.TryPerformStateOfClass` _tempest_state_manager_component (`GameplayStatics.GetObjectClass` (`TempestBaseStateManagerComponent.GetStateOfGameplayTag` _tempest_state_manager_component (struct :`TagName` "State.Walk"))) true)))))

(fn `CanPerformState`
  (returns (ReturnValue :type Boolean))
  (return (and (== (`TempestBaseStateObject.StateGameplayTag` (`TempestBaseStateManagerComponent.GetCurrentActiveState` (`self.Get Tempest State Manager Component`))) (struct :`TagName` "State.Walk")) (not (`NavMovementComponent.IsFalling` (`Character.CharacterMovement` (`self.Owner Character`)))))))