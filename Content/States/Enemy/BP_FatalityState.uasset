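; BP_FatalityState is an enemy AI state that performs a fatality ability through the enemy's Tempest ability system component.
; It can run only when an ability from FatalityAbilities qualifies, the active state matches a required gameplay tag, and the enemy owns a required tag.
; On start it begins the state timer and performs the selected ability by class.
; Next-state selection defers to the parent state.
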(event `self.StartState`
  (`self.StartStateTimer`)
  (`TempestBaseAbilityManagerComponent.PerformAbilityOfClass` (`/TempestCombatFramework/Characters/TCF_MasterEnemy_BP.BP_TempestAbilitySystemComponent` (`/TempestCombatFramework/Controllers/TCF_MasterEnemy_AIC_BP.Master Enemy` (`self.Master Enemy AIC`))) (`self.Get Selected Ability`)))

(fn `CanPerformState`
  (returns (ReturnValue :type Boolean))
  (bind _master_enemy_aic (`self.Master Enemy AIC`))
  (bind _return_value (`self.Check Abilities To Run` (`self.Fatality Abilities`)))
  (bind _tagcontainer (message `GameplayTagAssetInterface.GetOwnedGameplayTags` (`/TempestCombatFramework/Controllers/TCF_MasterEnemy_AIC_BP.Master Enemy` _master_enemy_aic)))
  (return (and _return_value (== (`TempestBaseStateObject.StateGameplayTag` (`TempestBaseStateManagerComponent.GetCurrentActiveState` (`/TempestCombatFramework/Controllers/TCF_MasterEnemy_AIC_BP.EnemyStateManagerComponent` _master_enemy_aic))) (struct)) (`BlueprintGameplayTagLibrary.HasTag` _tagcontainer (struct) true))))

(fn `Decide Next State`
  (`parent.Decide Next State`))