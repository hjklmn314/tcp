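; Base state for enemy states, giving child states shared references and spatial queries against the enemy's combat target.
; On construction it casts the performing actor to TCF_MasterEnemy_BP and caches the enemy and its AI controller.
; Helper functions read the combat component's target to return its distance from the controlled pawn, plus the pitch and yaw deltas between the pawn's rotation and the look-at rotation toward it.
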(event `self.ConstructState`
  (`parent.ConstructState`)
  (bind _astcf_master_enemy_bp (cast `/TempestCombatFramework/Characters/TCF_MasterEnemy_BP` (`self.GetPerformingActor`)))
  (set `self.Master Enemy` _astcf_master_enemy_bp)
  (set `self.Master Enemy AIC` (`/TempestCombatFramework/Characters/TCF_MasterEnemy_BP.Master Enemy AIC` _astcf_master_enemy_bp)))

(fn `Calculate Distance Difference`
  (returns (ReturnValue :type "Float (double-precision)"))
  (bind _master_enemy_aic (`self.Master Enemy AIC`))
  (bind _return_value (`/TempestCombatFramework/Components/AI/AICombatComponent.Get Combat Target` (`/TempestCombatFramework/Characters/TCF_MasterEnemy_BP.BP_TempestEnemyCombatComponent` (`/TempestCombatFramework/Controllers/TCF_MasterEnemy_AIC_BP.Master Enemy` _master_enemy_aic))))
  (`/Engine/EditorBlueprintResources/StandardMacros.IsValid` _return_value
    (:`Is Valid`
      (return (`KismetMathLibrary.VSize` (- (`Actor.K2_GetActorLocation` _return_value) (`Actor.K2_GetActorLocation` (`Controller.K2_GetPawn` _master_enemy_aic))))))))

(fn `Calculate Yaw & Pitch Difference`
  (returns (`Return Value Y (Pitch)` :type "Float (double-precision)") (`Return Value Z (Yaw)` :type "Float (double-precision)"))
  (bind _returnvalue (`Controller.K2_GetPawn` (`self.Master Enemy AIC`)))
  (bind _return_value (`/TempestCombatFramework/Components/AI/AICombatComponent.Get Combat Target` (`/TempestCombatFramework/Characters/TCF_MasterEnemy_BP.BP_TempestEnemyCombatComponent` (`/TempestCombatFramework/Controllers/TCF_MasterEnemy_AIC_BP.Master Enemy` (`self.Master Enemy AIC`)))))
  (bind (_returnvalue_roll _returnvalue_pitch _returnvalue_yaw) (`KismetMathLibrary.BreakRotator` (`KismetMathLibrary.NormalizedDeltaRotator` (`Actor.K2_GetActorRotation` _returnvalue) (`KismetMathLibrary.FindLookAtRotation` (`Actor.K2_GetActorLocation` _returnvalue) (`Actor.K2_GetActorLocation` _return_value)))))
  (`/Engine/EditorBlueprintResources/StandardMacros.IsValid` _return_value
    (:`Is Valid`
      (return _returnvalue_pitch _returnvalue_yaw))))