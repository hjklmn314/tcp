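; Base enemy AI state for a Tempest state manager, providing optional time limits on how long a state runs.
; When time-controlled, starting the state runs a looping timer that accumulates passed time while it is the manager's active state.
; Reaching the limit calls DecideNextState, which ends the state by default; a timer tick finding another state active also ends it.
; ProcessCalculations is an empty stub.
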(event `self.StartState`
  (`self.StartStateTimer`))

(event `self.EndState`
  (`self.ClearStateValues`))

(event `self.ClearStateValues`
  (`KismetSystemLibrary.K2_PauseTimer` null "IncrementPassedTime")
  (`KismetSystemLibrary.K2_ClearTimer` null "IncrementPassedTime")
  (`self.ClearPassedTime`))

(event `self.PrepareStateValues`
  (`self.ClearPassedTime`))

(event `self.StartStateTimer`
  (if (`self.bTimeControlledState`)
    (`KismetSystemLibrary.K2_SetTimer` null "IncrementPassedTime" (`self.TimerUpdateRate`) true)))

(event `self.ClearPassedTime`
  (set `self.TimePassed` 0.0))

(event `self.StopStateTimer`
  (`KismetSystemLibrary.K2_PauseTimer` null "IncrementPassedTime")
  (`KismetSystemLibrary.K2_ClearTimer` null "IncrementPassedTime")
  (`self.ClearPassedTime`))

(event `self.IncrementPassedTime`
  (bind _returnvalue (`TempestBaseStateManagerComponent.GetCurrentActiveState` (`self.Get Tempest State Manager Component`)))
  (`/Engine/EditorBlueprintResources/StandardMacros.IsValid` _returnvalue
    (:`Is Valid`
      (if (== _returnvalue self)
        (bind _returnvalue_2 (`self.IncrementTimeByUpdateRate`))
        (if (>= _returnvalue_2 (`self.StateTimeLimit`))
          (`self.ClearPassedTime`)
          (`self.Decide Next State`))
        (else
          (`self.EndState`))))))

(fn `Decide Next State`
  (`self.EndState`))

(fn `Process Calculations`)