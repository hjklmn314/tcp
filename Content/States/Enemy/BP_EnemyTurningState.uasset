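; Enemy AI state that turns the enemy toward its combat target by running a turning ability.
; It can run only when a valid target sits more than 45 degrees off in yaw and one of the turning abilities passes its check.
; Starting the state performs the selected ability through the enemy's Tempest ability system component.
; When deciding the next state, it tries the FollowTarget state, found by gameplay tag, with condition checks.
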(event `self.StartState`
  (`TempestBaseAbilityManagerComponent.PerformAbilityOfClass` (`/TempestCombatFramework/Characters/TCF_MasterEnemy_BP.BP_TempestAbilitySystemComponent` (`/TempestCombatFramework/Controllers/TCF_MasterEnemy_AIC_BP.Master Enemy` (`self.Master Enemy AIC`))) (`self.Get Selected Ability`)))

(fn `CanPerformState`
  (returns (ReturnValue :type Boolean))
  (`/Engine/EditorBlueprintResources/StandardMacros.IsValid` (`/TempestCombatFramework/Components/AI/AICombatComponent.Get Combat Target` (`/TempestCombatFramework/Characters/TCF_MasterEnemy_BP.BP_TempestEnemyCombatComponent` (`/TempestCombatFramework/Controllers/TCF_MasterEnemy_AIC_BP.Master Enemy` (`self.Master Enemy AIC`))))
    (:`Is Valid`
      (bind (_return_value_y__pitch_ _return_value_z__yaw_) (`self.Calculate Yaw & Pitch Difference`))
      (if (> (`KismetMathLibrary.Abs` _return_value_z__yaw_) 45.0)
        (bind _return_value (`self.Check Abilities To Run` (`self.Turning Abilities`)))
        (return _return_value)
        (else
          (return false))))
    (:`Is Not Valid`
      (return false))))

(fn `Decide Next State`
  (bind _tempest_state_manager_component (`self.Get Tempest State Manager Component`))
  (`parent.Decide Next State`)
  (`TempestBaseStateManagerComponent.TryPerformStateOfClass` _tempest_state_manager_component (`GameplayStatics.GetObjectClass` (`TempestBaseStateManagerComponent.GetStateOfGameplayTag` _tempest_state_manager_component (struct :`TagName` "State.FollowTarget"))) true))