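; Enemy AI state that sends an enemy patrolling between its spawner's patrol points, and can only run when that spawner is valid.
; Preparing the state updates the enemy's AI move set; starting it caches point locations, adding the enemy's own position if only one point exists.
; Each start writes the next point to the Blackboard destination, stepping back and forth along the path, and sets a fixed walk speed.
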(event `self.PrepareStateValues`
  (`/TempestCombatFramework/Characters/TCF_MasterEnemy_BP.OnUpdated_AI_MoveSet` (`/TempestCombatFramework/Controllers/TCF_MasterEnemy_AIC_BP.Master Enemy` (`self.Master Enemy AIC`)) "NewEnumerator0"))

(event `self.StartState`
  (bind _master_enemy_aic (`self.Master Enemy AIC`))
  (bind _spawner (break `/TempestCombatFramework/StructuresEnums/S_Enemy_SpawnInfo` (`/TempestCombatFramework/Characters/TCF_MasterEnemy_BP.Get Enemy Spawn Info` (`/TempestCombatFramework/Controllers/TCF_MasterEnemy_AIC_BP.Master Enemy` (`self.Master Enemy AIC`)))))
  (bind _patrolling_points (`/TempestCombatFramework/Actors/Spawner/BP_EnemySpawner.Patrolling Points` _spawner))
  (`/Engine/EditorBlueprintResources/StandardMacros.IsValid` _spawner
    (:`Is Valid`
      (for _array_element _patrolling_points
        (`KismetArrayLibrary.Array_AddUnique` (`self.Patrolling Points Locations`) (`Actor.K2_GetActorLocation` _array_element)))
      (if (== (`KismetArrayLibrary.Array_Length` _patrolling_points) 1)
        (`KismetArrayLibrary.Array_AddUnique` (`self.Patrolling Points Locations`) (`Actor.K2_GetActorLocation` (`/TempestCombatFramework/Controllers/TCF_MasterEnemy_AIC_BP.Master Enemy` (`self.Master Enemy AIC`)))))
      (bind _patrol_point (`self.Get Next Patrolling Point`))
      (`BlackboardComponent.SetValueAsVector` (`AIController.Blackboard` _master_enemy_aic) (`/TempestCombatFramework/Controllers/TCF_MasterEnemy_AIC_BP.Get Behavior Tree Key Name` _master_enemy_aic (struct :`TagName` "AI.BB.Destination")) _patrol_point)
      (set `CharacterMovementComponent.MaxWalkSpeed` 225.0 (`Character.CharacterMovement` (`/TempestCombatFramework/Controllers/TCF_MasterEnemy_AIC_BP.Master Enemy` (`self.Master Enemy AIC`)))))))

(fn `CanPerformState`
  (returns (ReturnValue :type Boolean))
  (return (`KismetSystemLibrary.IsValid` (`.Spawner_29_F09BD5E34E47067EBE18C39743D73637` (break `/TempestCombatFramework/StructuresEnums/S_Enemy_SpawnInfo` (`/TempestCombatFramework/Characters/TCF_MasterEnemy_BP.Get Enemy Spawn Info` (`/TempestCombatFramework/Controllers/TCF_MasterEnemy_AIC_BP.Master Enemy` (`self.Master Enemy AIC`))))))))

(fn `Get Next Patrolling Point`
  (returns (`Patrol Point` :type "Vector Structure"))
  (locals (`Local Point` :type "Vector Structure"))
  (set `local.Local Point` (`|GetArrayItem` (`self.Patrolling Points Locations`) (`self.Current Point`)))
  (if (`self.Flipped Path`)
    (set `self.Current Point` (- (`self.Current Point`) 1))
    (set `self.Flipped Path` (not (== (`self.Current Point`) 0)))
    (else
      (set `self.Current Point` (+ (`self.Current Point`) 1))
      (set `self.Flipped Path` (== (`self.Current Point`) (`KismetArrayLibrary.Array_LastIndex` (`self.Patrolling Points Locations`))))))
  (return (`local.Local Point`)))