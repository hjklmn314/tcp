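; Enemy state for awaiting a fatality, enterable only when Health is at or below zero and an AwaitingFatality ability can run.
; On start it begins the state timer and performs the selected ability through the Tempest ability system.
; After the parent's next-state logic, a random roll tries Attack one third of the time.
; Otherwise, or if Attack fails, it tries Turning, then FollowTarget.
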(event `self.StartState`
  (`self.StartStateTimer`)
  (`TempestBaseAbilityManagerComponent.PerformAbilityOfClass` (`/TempestCombatFramework/Characters/TCF_MasterEnemy_BP.BP_TempestAbilitySystemComponent` (`self.Master Enemy`)) (`self.Get Selected Ability`)))

(fn `CanPerformState`
  (returns (ReturnValue :type Boolean))
  (bind _returnvalue (`TempestAttributesComponents.GetAttributeOfGameplayTag` (`/TempestCombatFramework/Characters/TCF_MasterEnemy_BP.BP_TempestAttributesComponents` (`self.Master Enemy`)) (struct :`TagName` "Attribute.Health")))
  (bind _attributevalues_attributevalue (break `AttributeProperties` (`TempestBaseAttributeObject.AttributeValues` _returnvalue)))
  (`/Engine/EditorBlueprintResources/StandardMacros.IsValid` _returnvalue
    (:`Is Valid`
      (bind _return_value (`self.Check Abilities To Run` (`self.Awaiting Fatality`)))
      (return (and _return_value (<= _attributevalues_attributevalue 0.0))))
    (:`Is Not Valid`
      (return false))))

(fn `Decide Next State`
  (bind _tempest_state_manager_component (`self.Get Tempest State Manager Component`))
  (bind _tempest_state_manager_component_2 (`self.Get Tempest State Manager Component`))
  (`parent.Decide Next State`)
  (switch `int` (`KismetMathLibrary.RandomIntegerInRange` 0 5)
    (:`Default`
      (bind _returnvalue (`TempestBaseStateManagerComponent.TryPerformStateOfClass` _tempest_state_manager_component (`GameplayStatics.GetObjectClass` (`TempestBaseStateManagerComponent.GetStateOfGameplayTag` _tempest_state_manager_component (struct :`TagName` "State.Turning"))) true :!label _label))
      (if (not _returnvalue)
        (`TempestBaseStateManagerComponent.TryPerformStateOfClass` _tempest_state_manager_component (`GameplayStatics.GetObjectClass` (`TempestBaseStateManagerComponent.GetStateOfGameplayTag` _tempest_state_manager_component (struct :`TagName` "State.FollowTarget"))) true)))
    (:`0`
      (bind _returnvalue_2 (`TempestBaseStateManagerComponent.TryPerformStateOfClass` _tempest_state_manager_component_2 (`GameplayStatics.GetObjectClass` (`TempestBaseStateManagerComponent.GetStateOfGameplayTag` _tempest_state_manager_component_2 (struct :`TagName` "State.Attack"))) true :!label _label_2))
      (if (not _returnvalue_2)
        (goto _label)))
    (:`1`
      (goto _label_2))))