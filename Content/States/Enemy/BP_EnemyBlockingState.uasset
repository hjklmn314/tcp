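; Enemy AI blocking state for the Tempest state manager that runs the enemy's blocking ability when the ability check passes.
; On an incoming attack it restarts itself, unless the combat target's active trace objects already hit this enemy or a NoBlockTrigger status tag is set.
; Its next-state decision tries the FollowTarget state, looked up by gameplay tag, with a condition check.
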(event `self.StartState`
  (`TempestBaseStateManagerComponent.SetCurrentActiveState` (`self.Get Tempest State Manager Component`) self)
  (`TempestBaseAbilityManagerComponent.PerformAbilityOfClass` (`/TempestCombatFramework/Characters/TCF_MasterEnemy_BP.BP_TempestAbilitySystemComponent` (`/TempestCombatFramework/Controllers/TCF_MasterEnemy_AIC_BP.Master Enemy` (`self.Master Enemy AIC`))) (`self.Blocking Ability`)))

(event `/TempestCombatFramework/Interfaces/BPI_TempestAbilitiesAndStates.Process Incoming Attack`
  (`/Engine/EditorBlueprintResources/StandardMacros.IsValid` (`TempestBaseStateManagerComponent.GetCurrentActiveState` (`self.Get Tempest State Manager Component`))
    (:`Is Valid`
      (if (and (not (`self.Get Did Target Hit Owner`)) (not (`BlueprintGameplayTagLibrary.HasTag` (`TempestCombatComponent.GetCombatStatus` (`/TempestCombatFramework/Characters/TCF_MasterEnemy_BP.BP_TempestEnemyCombatComponent` (`self.Master Enemy`))) (struct :`TagName` "Status.Combat.No Block Trigger") true)))
        (`self.RestartState` true)))))

(fn `CanPerformState`
  (returns (ReturnValue :type Boolean))
  (bind _return_value (`self.Check Abilities To Run` (`|MakeArray` (`self.Blocking Ability`) :!type "TempestBaseAbilityObject Class Reference")))
  (return _return_value))

(fn `Decide Next State`
  (bind _tempest_state_manager_component (`self.Get Tempest State Manager Component`))
  (`TempestBaseStateManagerComponent.TryPerformStateOfClass` _tempest_state_manager_component (`GameplayStatics.GetObjectClass` (`TempestBaseStateManagerComponent.GetStateOfGameplayTag` _tempest_state_manager_component (struct :`TagName` "State.FollowTarget"))) true))

(fn `Get Block Time Since Last Clicked`
  (returns (`Return Value` :type "Float (double-precision)"))
  (return 0.0))

(fn `Get Did Target Hit Owner`
  (returns (ReturnValue :type Boolean))
  (for _array_element (`TempestCollisionManagerComponent.ActiveTraceObjects` (`Actor.GetComponentByClass` (`/TempestCombatFramework/Components/AI/AICombatComponent.Get Combat Target` (`/TempestCombatFramework/Characters/TCF_MasterEnemy_BP.BP_TempestEnemyCombatComponent` (`self.Master Enemy`))) "/Script/TempestCombatFramework.TempestCollisionManagerComponent"))
    (bind _asbp_base_trace_object (cast `/TempestCombatFramework/Trace/BP_BaseTraceObject` _array_element))
    (bind _returnvalue (`KismetArrayLibrary.Array_Contains` (`/TempestCombatFramework/Trace/BP_BaseTraceObject.Hit Actors` _asbp_base_trace_object) (`self.Master Enemy`)))
    (if _returnvalue
      (return _returnvalue)))
  (return false))

(fn `Get Montage Counter For Ability`
  (returns (`Counter Montage` :type "AnimMontage Object Reference"))
  (return null))