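; Enemy AI state for the Tempest state manager in which the enemy follows at a walk speed set by a distance threshold.
; Each tick it updates speed and switches to ReturnToPost when that state can perform.
; Otherwise, within stop-follow distance, it randomly favors Attack over strafing left or right, with strafing as attack fallback and a restart if strafing fails.
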(event `self.StartState`
  (`self.StartStateTimer`)
  (set `self.Return To Post State` (`TempestBaseStateManagerComponent.GetStateOfGameplayTag` (`self.Get Tempest State Manager Component`) (struct :`TagName` "State.ReturnToPost"))))

(event `self.PrepareStateValues`
  (`self.Adjust Movement Speed Based On Distance`)
  (`/TempestCombatFramework/Characters/TCF_MasterEnemy_BP.OnUpdated_AI_MoveSet` (`/TempestCombatFramework/Controllers/TCF_MasterEnemy_AIC_BP.Master Enemy` (`self.Master Enemy AIC`)) "NewEnumerator1"))

(event `self.TickState`
  (params (TickTime :type "Float (single-precision)"))
  (`self.Process Calculations`))

(fn `Adjust Movement Speed Based On Distance`
  (bind (_followthreshold _followspeedunderfollowthreshold _followspeedabovefollowthreshold) (break `/TempestCombatFramework/StructuresEnums/S_AIFollowBehavior` (`self.Following Behavior Properties`)))
  (bind _returnvalue (`self.Calculate Distance Difference`))
  (if (>= _returnvalue _followthreshold)
    (set `CharacterMovementComponent.MaxWalkSpeed` _followspeedabovefollowthreshold (`Character.CharacterMovement` (`/TempestCombatFramework/Controllers/TCF_MasterEnemy_AIC_BP.Master Enemy` (`self.Master Enemy AIC`))))
    (elif (<= _returnvalue _followthreshold)
      (set `CharacterMovementComponent.MaxWalkSpeed` _followspeedunderfollowthreshold (`Character.CharacterMovement` (`/TempestCombatFramework/Controllers/TCF_MasterEnemy_AIC_BP.Master Enemy` (`self.Master Enemy AIC`)))))))

(fn `CanPerformState`
  (returns (ReturnValue :type Boolean))
  (return true))

(fn `Decide Next State`
  (bind _tempest_state_manager_component (`self.Get Tempest State Manager Component`))
  (bind _tempest_state_manager_component_2 (`self.Get Tempest State Manager Component`))
  (`parent.Decide Next State`)
  (switch `int` (`KismetMathLibrary.RandomIntegerInRange` 0 3)
    (:`Default`
      (bind _returnvalue (`TempestBaseStateManagerComponent.TryPerformStateOfClass` _tempest_state_manager_component (`GameplayStatics.GetObjectClass` (`TempestBaseStateManagerComponent.GetStateOfGameplayTag` _tempest_state_manager_component (select `bool` (`KismetMathLibrary.RandomBool`) :`false` (struct :`TagName` "State.StrafingLeft") :`true` (struct :`TagName` "State.StrafingRight") :!type "GameplayTag Structure"))) true :!label _label))
      (if (not _returnvalue)
        (`self.RestartState` false)))
    (:`0`
      (bind _returnvalue_2 (`self.Calculate Distance Difference`))
      (if (> _returnvalue_2 (`.StopFollowAt_22_288C842943E649C5DFA85282B0CD8F98` (break `/TempestCombatFramework/StructuresEnums/S_AIFollowBehavior` (`self.Following Behavior Properties`))))
        (`self.RestartState` false)
        (else
          (bind _returnvalue_3 (`TempestBaseStateManagerComponent.TryPerformStateOfClass` _tempest_state_manager_component_2 (`GameplayStatics.GetObjectClass` (`TempestBaseStateManagerComponent.GetStateOfGameplayTag` _tempest_state_manager_component_2 (struct :`TagName` "State.Attack"))) true :!label _label_2))
          (if (not _returnvalue_3)
            (goto _label)))))
    (:`1`
      (goto _label_2))
    (:`2`
      (goto _label_2))))

(fn `Process Calculations`
  (bind _return_to_post_state (`self.Return To Post State`))
  (`parent.Process Calculations`)
  (`self.Adjust Movement Speed Based On Distance`)
  (`/Engine/EditorBlueprintResources/StandardMacros.IsValid` _return_to_post_state
    (:`Is Valid`
      (if (`self.CanPerformState` _return_to_post_state)
        (`TempestBaseStateManagerComponent.PerformStateOfClass` (`self.Get Tempest State Manager Component`) (`GameplayStatics.GetObjectClass` (`self.Return To Post State`)))
        (else
          (bind _returnvalue (`self.Calculate Distance Difference` :!label _label))
          (if (<= _returnvalue (`.StopFollowAt_22_288C842943E649C5DFA85282B0CD8F98` (break `/TempestCombatFramework/StructuresEnums/S_AIFollowBehavior` (`self.Following Behavior Properties`))))
            (`self.Decide Next State`)))))
    (:`Is Not Valid`
      (goto _label))))