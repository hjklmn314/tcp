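; Enemy attacking state for the Tempest state manager, driving an AI-controlled enemy's attack abilities.
; It can run only with a valid combat target and a passing check on its attack abilities, and on start performs the selected ability through the enemy's ability system component.
; When deciding the next state, it tries Turning first, then restarting itself, then falls back to FollowTarget.
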(event `self.StartState`
  (`TempestBaseAbilityManagerComponent.PerformAbilityOfClass` (`/TempestCombatFramework/Characters/TCF_MasterEnemy_BP.BP_TempestAbilitySystemComponent` (`/TempestCombatFramework/Controllers/TCF_MasterEnemy_AIC_BP.Master Enemy` (`self.Master Enemy AIC`))) (`self.Get Selected Ability`)))

(fn `CanPerformState`
  (returns (ReturnValue :type Boolean))
  (`/Engine/EditorBlueprintResources/StandardMacros.IsValid` (`/TempestCombatFramework/Components/AI/AICombatComponent.Get Combat Target` (`/TempestCombatFramework/Characters/TCF_MasterEnemy_BP.BP_TempestEnemyCombatComponent` (`/TempestCombatFramework/Controllers/TCF_MasterEnemy_AIC_BP.Master Enemy` (`self.Master Enemy AIC`))))
    (:`Is Valid`
      (bind _return_value (`self.Check Abilities To Run` (`self.Attack Abilities`)))
      (return _return_value))
    (:`Is Not Valid`
      (return false))))

(fn `Decide Next State`
  (bind _tempest_state_manager_component (`self.Get Tempest State Manager Component`))
  (bind _tempest_state_manager_component_2 (`self.Get Tempest State Manager Component`))
  (`parent.Decide Next State`)
  (bind _returnvalue (`TempestBaseStateManagerComponent.TryPerformStateOfClass` _tempest_state_manager_component (`GameplayStatics.GetObjectClass` (`TempestBaseStateManagerComponent.GetStateOfGameplayTag` _tempest_state_manager_component (struct :`TagName` "State.Turning"))) true))
  (if (not _returnvalue)
    (bind _returnvalue_2 (`self.RestartState` true))
    (if (not _returnvalue_2)
      (`TempestBaseStateManagerComponent.TryPerformStateOfClass` _tempest_state_manager_component_2 (`GameplayStatics.GetObjectClass` (`TempestBaseStateManagerComponent.GetStateOfGameplayTag` _tempest_state_manager_component_2 (struct :`TagName` "State.FollowTarget"))) true))))