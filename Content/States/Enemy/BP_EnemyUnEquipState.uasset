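; Enemy AI state that unequips the enemy and takes it out of combat.
; Preparing the state updates the AI move set, and starting it performs the unequip ability through the Tempest ability system component.
; On deciding the next state, it exits combat and clears all perception, activating the spawn state if the enemy data asset defines one, otherwise halting and clearing current state updating.
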(event `self.PrepareStateValues`
  (`/TempestCombatFramework/Characters/TCF_MasterEnemy_BP.OnUpdated_AI_MoveSet` (`/TempestCombatFramework/Controllers/TCF_MasterEnemy_AIC_BP.Master Enemy` (`self.Master Enemy AIC`)) "NewEnumerator0"))

(event `self.StartState`
  (`TempestBaseAbilityManagerComponent.PerformAbilityOfClass` (`/TempestCombatFramework/Characters/TCF_MasterEnemy_BP.BP_TempestAbilitySystemComponent` (`/TempestCombatFramework/Controllers/TCF_MasterEnemy_AIC_BP.Master Enemy` (`self.Master Enemy AIC`))) (`self.UnEquip Ability`)))

(fn `Decide Next State`
  (bind _master_enemy_aic (`self.Master Enemy AIC`))
  (bind _master_enemy_aic_2 (`self.Master Enemy AIC`))
  (bind _master_enemy_aic_3 (`self.Master Enemy AIC`))
  (`parent.Decide Next State`)
  (if (`KismetSystemLibrary.IsValidClass` (`/TempestCombatFramework/DataAssets/DA_Enemyinfo.On Spawn State` (`/TempestCombatFramework/Characters/TCF_MasterEnemy_BP.Get Enemy Data Asset` (`/TempestCombatFramework/Controllers/TCF_MasterEnemy_AIC_BP.Master Enemy` _master_enemy_aic_3))))
    (`/TempestCombatFramework/Controllers/TCF_MasterEnemy_AIC_BP.Activate Spawn State` _master_enemy_aic_3)
    (`/TempestCombatFramework/Components/AI/AICombatComponent.Exit Combat` (`/TempestCombatFramework/Characters/TCF_MasterEnemy_BP.BP_TempestEnemyCombatComponent` (`/TempestCombatFramework/Controllers/TCF_MasterEnemy_AIC_BP.Master Enemy` _master_enemy_aic)))
    (`AIPerceptionComponent.ForgetAll` (`/TempestCombatFramework/Controllers/TCF_MasterEnemy_AIC_BP.AIPerception` _master_enemy_aic))
    (else
      (`/TempestCombatFramework/Components/AI/AICombatComponent.Exit Combat` (`/TempestCombatFramework/Characters/TCF_MasterEnemy_BP.BP_TempestEnemyCombatComponent` (`/TempestCombatFramework/Controllers/TCF_MasterEnemy_AIC_BP.Master Enemy` (`self.Master Enemy AIC`))))
      (`/TempestCombatFramework/Components/AI/AIStateManagerComponent.Halt & Clear Current State Updating Behavior` (`/TempestCombatFramework/Controllers/TCF_MasterEnemy_AIC_BP.EnemyStateManagerComponent` _master_enemy_aic_2))
      (`AIPerceptionComponent.ForgetAll` (`/TempestCombatFramework/Controllers/TCF_MasterEnemy_AIC_BP.AIPerception` _master_enemy_aic_2)))))