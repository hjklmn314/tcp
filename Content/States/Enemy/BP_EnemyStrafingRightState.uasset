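; Enemy AI combat state that strafes the enemy along its right vector for a short randomized time while facing the combat target.
; Each tick feeds movement input and a strafe angle to the anim instance, snapping yaw when the target is within the front cone and interpolating otherwise.
; On ending, a random roll picks between restarting, FollowTarget, StrafingLeft or Attack through the Tempest state manager, with fallbacks if a transition fails.
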(event `self.StartState`
  (`self.StartStateTimer`)
  (set `self.StateTimeLimit` (`KismetMathLibrary.RandomFloatInRange` 1.0 1.5)))

(event `self.TickState`
  (params (TickTime :type "Float (single-precision)"))
  (bind _returnvalue (`self.Get Strafing Direction`))
  (bind _master_enemy_aic (`self.Master Enemy AIC`))
  (bind _master_enemy_aic_2 (`self.Master Enemy AIC`))
  (bind _master_enemy (`/TempestCombatFramework/Controllers/TCF_MasterEnemy_AIC_BP.Master Enemy` (`self.Master Enemy AIC`)))
  (bind _master_enemy_2 (`/TempestCombatFramework/Controllers/TCF_MasterEnemy_AIC_BP.Master Enemy` (`self.Master Enemy AIC`)))
  (bind _master_enemy_3 (`/TempestCombatFramework/Controllers/TCF_MasterEnemy_AIC_BP.Master Enemy` (`self.Master Enemy AIC`)))
  (bind (_returnvalue_roll _returnvalue_pitch) (`KismetMathLibrary.BreakRotator` (`Actor.K2_GetActorRotation` _master_enemy_3)))
  (bind (_returnvalue_roll_2 _returnvalue_pitch_2) (`KismetMathLibrary.BreakRotator` (`Actor.K2_GetActorRotation` _master_enemy_2)))
  (bind (_returnvalue_roll_3 _returnvalue_pitch_3 _returnvalue_yaw) (`KismetMathLibrary.BreakRotator` (`KismetMathLibrary.FindLookAtRotation` (`Actor.K2_GetActorLocation` _master_enemy_3) (`Actor.K2_GetActorLocation` (`self.Actor Target`)))))
  (bind (_returnvalue_roll_4 _returnvalue_pitch_4 _returnvalue_yaw_2) (`KismetMathLibrary.BreakRotator` (`KismetMathLibrary.FindLookAtRotation` (`Actor.K2_GetActorLocation` _master_enemy_2) (`Actor.K2_GetActorLocation` (`self.Actor Target`)))))
  (bind (_returnvalue_roll_5 _returnvalue_pitch_5 _returnvalue_yaw_3) (`KismetMathLibrary.BreakRotator` (`KismetMathLibrary.NormalizedDeltaRotator` (`Actor.K2_GetActorRotation` (`/TempestCombatFramework/Controllers/TCF_MasterEnemy_AIC_BP.Master Enemy` (`self.Master Enemy AIC`))) (`KismetMathLibrary.Conv_VectorToRotator` _returnvalue))))
  (bind (_returnvalue_roll_6 _returnvalue_pitch_6 _returnvalue_yaw_4) (`KismetMathLibrary.BreakRotator` (`KismetMathLibrary.NormalizedDeltaRotator` (`Actor.K2_GetActorRotation` _master_enemy) (`KismetMathLibrary.FindLookAtRotation` (`Actor.K2_GetActorLocation` _master_enemy) (`Actor.K2_GetActorLocation` (`self.Actor Target`))))))
  (`/Engine/EditorBlueprintResources/StandardMacros.IsValid` (`BlackboardComponent.GetValueAsObject` (`AIController.Blackboard` _master_enemy_aic) (`/TempestCombatFramework/Controllers/TCF_MasterEnemy_AIC_BP.Get Behavior Tree Key Name` _master_enemy_aic (struct :`TagName` "AI.BB.CombatTarget")))
    (:`Is Valid`
      (`Pawn.AddMovementInput` (`/TempestCombatFramework/Controllers/TCF_MasterEnemy_AIC_BP.Master Enemy` (`self.Master Enemy AIC`)) _returnvalue 1.0 false)
      (message `/TempestCombatFramework/Interfaces/BPI_EnemyStates.Assign Strafing Values` (`SkeletalMeshComponent.GetAnimInstance` (`Character.Mesh` (`/TempestCombatFramework/Controllers/TCF_MasterEnemy_AIC_BP.Master Enemy` (`self.Master Enemy AIC`)))) (* _returnvalue_yaw_3 -1.0) (0.0 0.0 0.0))
      (bind _asactor (cast `Actor` (`BlackboardComponent.GetValueAsObject` (`AIController.Blackboard` _master_enemy_aic_2) (`/TempestCombatFramework/Controllers/TCF_MasterEnemy_AIC_BP.Get Behavior Tree Key Name` _master_enemy_aic_2 (struct :`TagName` "AI.BB.CombatTarget")))))
      (set `self.Actor Target` _asactor)
      (if (`KismetMathLibrary.InRange_FloatFloat` _returnvalue_yaw_4 -45.0 45.0)
        ;[1 1 1] Instant Rotation
        (`Actor.K2_SetActorRotation` _master_enemy_3 (`KismetMathLibrary.MakeRotator` _returnvalue_roll _returnvalue_pitch _returnvalue_yaw) false)
        (else
          ;[1 1 1] Smooth Rotation
          (`Actor.K2_SetActorRotation` _master_enemy_2 (`KismetMathLibrary.RInterpTo` (`Actor.K2_GetActorRotation` _master_enemy_2) (`KismetMathLibrary.MakeRotator` _returnvalue_roll_2 _returnvalue_pitch_2 _returnvalue_yaw_2) TickTime 10.0) true))))))

(event `self.PrepareStateValues`
  (set `CharacterMovementComponent.MaxWalkSpeed` (`self.Strafing Movement Speed`) (`Character.CharacterMovement` (`/TempestCombatFramework/Controllers/TCF_MasterEnemy_AIC_BP.Master Enemy` (`self.Master Enemy AIC`))))
  (`/TempestCombatFramework/Characters/TCF_MasterEnemy_BP.OnUpdated_AI_MoveSet` (`/TempestCombatFramework/Controllers/TCF_MasterEnemy_AIC_BP.Master Enemy` (`self.Master Enemy AIC`)) "NewEnumerator2"))

(fn `Decide Next State`
  (bind _tempest_state_manager_component (`self.Get Tempest State Manager Component`))
  (bind _tempest_state_manager_component_2 (`self.Get Tempest State Manager Component`))
  (bind _tempest_state_manager_component_3 (`self.Get Tempest State Manager Component`))
  (`self.EndState`)
  (switch `int` (`KismetMathLibrary.RandomIntegerInRange` 0 4)
    (:`Default`
      (bind _returnvalue (`TempestBaseStateManagerComponent.TryPerformStateOfClass` _tempest_state_manager_component_3 (`GameplayStatics.GetObjectClass` (`TempestBaseStateManagerComponent.GetStateOfGameplayTag` _tempest_state_manager_component_3 (struct :`TagName` "State.Attack"))) true))
      (if (not _returnvalue)
        (bind _returnvalue_2 (`TempestBaseStateManagerComponent.TryPerformStateOfClass` _tempest_state_manager_component (`GameplayStatics.GetObjectClass` (`TempestBaseStateManagerComponent.GetStateOfGameplayTag` _tempest_state_manager_component (struct :`TagName` "State.StrafingLeft"))) true :!label _label))
        (if (not _returnvalue_2)
          (`self.RestartState` false))))
    (:`0`
      (bind _returnvalue_3 (`self.RestartState` true))
      (if (not _returnvalue_3)
        (`TempestBaseStateManagerComponent.TryPerformStateOfClass` _tempest_state_manager_component_2 (`GameplayStatics.GetObjectClass` (`TempestBaseStateManagerComponent.GetStateOfGameplayTag` _tempest_state_manager_component_2 (struct :`TagName` "State.FollowTarget"))) true :!label _label_2)))
    (:`1`
      (goto _label_2))
    (:`2`
      (goto _label))))

(fn `Get Strafing Direction`
  (returns (ReturnValue :type "Vector Structure"))
  (return (`Actor.GetActorRightVector` (`/TempestCombatFramework/Controllers/TCF_MasterEnemy_AIC_BP.Master Enemy` (`self.Master Enemy AIC`)))))