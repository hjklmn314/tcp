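; Enemy AI death state that becomes available when Health falls to its minimum, the death ability check passes and the state is not already active.
; On start it performs the selected ability, stops the AI brain logic, adds the State.Death tag and sets the capsule to ignore Pawn collision.
; Deciding a next state is left empty, and ending the state resets the selected ability.
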(event `self.StartState`
  (bind _master_enemy (`/TempestCombatFramework/Controllers/TCF_MasterEnemy_AIC_BP.Master Enemy` (`self.Master Enemy AIC`)))
  (if (`KismetSystemLibrary.IsValidClass` (`self.Get Selected Ability`))
    (`TempestBaseAbilityManagerComponent.PerformAbilityOfClass` (`/TempestCombatFramework/Characters/TCF_MasterEnemy_BP.BP_TempestAbilitySystemComponent` _master_enemy) (`self.Get Selected Ability`)))
  (`BrainComponent.StopLogic` (`AIController.BrainComponent` (`self.Master Enemy AIC`)) "")
  (`BlueprintGameplayTagLibrary.AddGameplayTag` (`TempestBaseCharacter.ActorGameplayTags` _master_enemy) (struct :`TagName` "State.Death"))
  (`PrimitiveComponent.SetCollisionResponseToChannel` (`Character.CapsuleComponent` _master_enemy) "ECC_Pawn" "ECR_Ignore"))

(event `self.EndState`
  (`parent.EndState`)
  (`self.Set Selected Ability` null))

(fn `CanPerformState`
  (returns (ReturnValue :type Boolean))
  (bind (_attributevalue _minattributevalue) (break `AttributeProperties` (`TempestBaseAttributeObject.AttributeValues` (`TempestAttributesComponents.GetAttributeOfGameplayTag` (`/TempestCombatFramework/Characters/TCF_MasterEnemy_BP.BP_TempestAttributesComponents` (`self.Master Enemy`)) (struct :`TagName` "Attribute.Health")))))
  (bind _return_value (`self.Check Abilities To Run` (`self.Death Ability`)))
  (return (and (<= _attributevalue _minattributevalue) _return_value (not (`self.Get Is State Currentely Active`)))))

(fn `Decide Next State`)