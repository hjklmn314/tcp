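; Enemy AI state for being assassinated, run through the Tempest state manager.
; On start it performs the assassinated ability on the enemy's ability system component, and its value preparation updates the enemy's AI move set.
; Entry depends on that ability passing the run check.
; When deciding the next state, it tries a condition-checked switch to the state tagged FollowTarget.
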(event `self.StartState`
  (`TempestBaseAbilityManagerComponent.PerformAbilityOfClass` (`/TempestCombatFramework/Characters/TCF_MasterEnemy_BP.BP_TempestAbilitySystemComponent` (`/TempestCombatFramework/Controllers/TCF_MasterEnemy_AIC_BP.Master Enemy` (`self.Master Enemy AIC`))) (`self.Assasinated Ability`)))

(event `self.PrepareStateValues`
  (`/TempestCombatFramework/Characters/TCF_MasterEnemy_BP.OnUpdated_AI_MoveSet` (`/TempestCombatFramework/Controllers/TCF_MasterEnemy_AIC_BP.Master Enemy` (`self.Master Enemy AIC`)) "NewEnumerator1"))

(fn `CanPerformState`
  (returns (ReturnValue :type Boolean))
  (bind _return_value (`self.Check Abilities To Run` (`|MakeArray` (`self.Assasinated Ability`) :!type "TempestBaseAbilityObject Class Reference")))
  (return _return_value))

(fn `Decide Next State`
  (bind _tempest_state_manager_component (`self.Get Tempest State Manager Component`))
  (`TempestBaseStateManagerComponent.TryPerformStateOfClass` _tempest_state_manager_component (`GameplayStatics.GetObjectClass` (`TempestBaseStateManagerComponent.GetStateOfGameplayTag` _tempest_state_manager_component (struct :`TagName` "State.FollowTarget"))) true))