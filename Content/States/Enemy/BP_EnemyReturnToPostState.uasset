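; Enemy AI state that sends an enemy back to its spawn point when it is far enough from it and a calculated distance difference is also large.
; On start it writes the spawn location to the Blackboard destination and performs the return-to-post ability.
; Deciding the next state updates the move set, exits combat and forgets perception, activating the spawn state if one is defined or otherwise halting state behavior.
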(event `self.StartState`
  (bind _master_enemy_aic (`self.Master Enemy AIC`))
  (bind (_enemy_spawn_info_spawner _enemy_spawn_info_spawnlocation) (break `/TempestCombatFramework/StructuresEnums/S_Enemy_SpawnInfo` (`/TempestCombatFramework/Characters/TCF_MasterEnemy_BP.Get Enemy Spawn Info` (`/TempestCombatFramework/Controllers/TCF_MasterEnemy_AIC_BP.Master Enemy` _master_enemy_aic))))
  (`BlackboardComponent.SetValueAsVector` (`AIController.Blackboard` (`self.Master Enemy AIC`)) (`/TempestCombatFramework/Controllers/TCF_MasterEnemy_AIC_BP.Get Behavior Tree Key Name` _master_enemy_aic (struct :`TagName` "AI.BB.Destination")) _enemy_spawn_info_spawnlocation)
  (`TempestBaseAbilityManagerComponent.PerformAbilityOfClass` (`/TempestCombatFramework/Characters/TCF_MasterEnemy_BP.BP_TempestAbilitySystemComponent` (`/TempestCombatFramework/Controllers/TCF_MasterEnemy_AIC_BP.Master Enemy` (`self.Master Enemy AIC`))) (`self.ReturnToPost Ability`)))

(fn `CanPerformState`
  (returns (ReturnValue :type Boolean))
  (bind _master_enemy (`/TempestCombatFramework/Controllers/TCF_MasterEnemy_AIC_BP.Master Enemy` (`self.Master Enemy AIC`)))
  (bind (_enemy_spawn_info_spawner _enemy_spawn_info_spawnlocation) (break `/TempestCombatFramework/StructuresEnums/S_Enemy_SpawnInfo` (`/TempestCombatFramework/Characters/TCF_MasterEnemy_BP.Get Enemy Spawn Info` _master_enemy)))
  (bind _returnvalue (`self.Calculate Distance Difference`))
  (return (and (>= _returnvalue 1000.0) (>= (`KismetMathLibrary.Vector_Distance` (`Actor.K2_GetActorLocation` _master_enemy) _enemy_spawn_info_spawnlocation) 1000.0))))

(fn `Decide Next State`
  (bind _master_enemy_aic (`self.Master Enemy AIC`))
  (bind _master_enemy_aic_2 (`self.Master Enemy AIC`))
  (bind _master_enemy_aic_3 (`self.Master Enemy AIC`))
  (`parent.Decide Next State`)
  (`/TempestCombatFramework/Characters/TCF_MasterEnemy_BP.OnUpdated_AI_MoveSet` (`/TempestCombatFramework/Controllers/TCF_MasterEnemy_AIC_BP.Master Enemy` (`self.Master Enemy AIC`)) "NewEnumerator0")
  (if (`KismetSystemLibrary.IsValidClass` (`/TempestCombatFramework/DataAssets/DA_Enemyinfo.On Spawn State` (`/TempestCombatFramework/Characters/TCF_MasterEnemy_BP.Get Enemy Data Asset` (`/TempestCombatFramework/Controllers/TCF_MasterEnemy_AIC_BP.Master Enemy` _master_enemy_aic_2))))
    (`/TempestCombatFramework/Controllers/TCF_MasterEnemy_AIC_BP.Activate Spawn State` _master_enemy_aic_2)
    (`/TempestCombatFramework/Components/AI/AICombatComponent.Exit Combat` (`/TempestCombatFramework/Characters/TCF_MasterEnemy_BP.BP_TempestEnemyCombatComponent` (`/TempestCombatFramework/Controllers/TCF_MasterEnemy_AIC_BP.Master Enemy` _master_enemy_aic)))
    (`AIPerceptionComponent.ForgetAll` (`/TempestCombatFramework/Controllers/TCF_MasterEnemy_AIC_BP.AIPerception` _master_enemy_aic))
    (else
      (`/TempestCombatFramework/Components/AI/AICombatComponent.Exit Combat` (`/TempestCombatFramework/Characters/TCF_MasterEnemy_BP.BP_TempestEnemyCombatComponent` (`/TempestCombatFramework/Controllers/TCF_MasterEnemy_AIC_BP.Master Enemy` _master_enemy_aic_3)))
      (`/TempestCombatFramework/Components/AI/AIStateManagerComponent.Halt & Clear Current State Updating Behavior` (`/TempestCombatFramework/Controllers/TCF_MasterEnemy_AIC_BP.EnemyStateManagerComponent` _master_enemy_aic_3))
      (`AIPerceptionComponent.ForgetAll` (`/TempestCombatFramework/Controllers/TCF_MasterEnemy_AIC_BP.AIPerception` _master_enemy_aic_3)))))