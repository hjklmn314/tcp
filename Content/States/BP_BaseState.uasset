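; Base state for a Tempest state machine, providing shared lifecycle, timing and ability selection for character states.
; It caches the state manager from the character's controller, registering as active on start and clearing itself on end.
; An opt-in looping timer accumulates elapsed time, resetting at the limit, and calls EndState if another state is active.
; A helper selects the first performable ability through the actor's ability manager.
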(event `self.ConstructState`
  (bind _ascharacter (cast `Character` (`self.GetPerformingActor`)))
  (`self.Set Tempest State Manager Component` (`Actor.GetComponentByClass` (`Pawn.GetController` _ascharacter) "/Script/TempestCombatFramework.TempestBaseStateManagerComponent")))

(event `self.StartState`
  (`parent.StartState`)
  (`TempestBaseStateManagerComponent.SetCurrentActiveState` (`self.Get Tempest State Manager Component`) self))

(event `self.TickState`
  (params (TickTime :type "Float (single-precision)")))

(event `self.EndState`
  (if (`self.Get Is State Currentely Active`)
    (`TempestBaseStateManagerComponent.SetCurrentActiveState` (`self.Get Tempest State Manager Component`) null)
    (`self.ClearStateValues`)))

(event `self.ClearStateValues`
  (`KismetSystemLibrary.K2_PauseTimer` null "IncrementPassedTime")
  (`KismetSystemLibrary.K2_ClearTimer` null "IncrementPassedTime")
  (`self.ClearPassedTime`))

(event `self.PrepareStateValues`
  (`self.ClearPassedTime`))

(event `self.StartStateTimer`
  (`KismetSystemLibrary.K2_SetTimer` null "IncrementPassedTime" (`self.TimerUpdateRate`) true))

(event `self.ClearPassedTime`
  (set `self.TimePassed` 0.0))

(event `self.StopStateTimer`
  (`KismetSystemLibrary.K2_PauseTimer` null "IncrementPassedTime")
  (`KismetSystemLibrary.K2_ClearTimer` null "IncrementPassedTime")
  (`self.ClearPassedTime`))

(event `self.IncrementPassedTime`
  (bind _returnvalue (`TempestBaseStateManagerComponent.GetCurrentActiveState` (`self.Get Tempest State Manager Component`)))
  (`/Engine/EditorBlueprintResources/StandardMacros.IsValid` _returnvalue
    (:`Is Valid`
      (if (== _returnvalue self)
        (bind _returnvalue_2 (`self.IncrementTimeByUpdateRate`))
        (if (>= _returnvalue_2 (`self.StateTimeLimit`))
          (`self.ClearPassedTime`))
        (else
          (`self.EndState`))))))

(fn `CanPerformState`
  (returns (ReturnValue :type Boolean))
  (return true))

(fn `CanSetAsQueueState`
  (returns (ReturnValue :type Boolean))
  (return false))

(fn `Check Abilities To Run`
  (params (`Abilities To Check` :type "Array of TempestBaseAbilityObject Class Reference"))
  (returns (`Return Value` :type Boolean))
  (locals (`Local Tempest Ability Component` :type "TempestBaseAbilityManagerComponent Object Reference"))
  (bind _local_tempest_ability_component (`local.Local Tempest Ability Component`))
  (bind _output_get (set `local.Local Tempest Ability Component` (`Actor.GetComponentByClass` (`self.GetPerformingActor`) "/Script/TempestCombatFramework.TempestBaseAbilityManagerComponent")))
  (`/Engine/EditorBlueprintResources/StandardMacros.IsValid` _output_get
    (:`Is Valid`
      (for _array_element `Abilities To Check`
        (if (`TempestBaseAbilityManagerComponent.GetCanPerformAbilityOfClass` _local_tempest_ability_component _array_element)
          (set `self.Selected Ability To Trigger` _array_element)
          (`/Engine/EditorBlueprintResources/StandardMacros.IsValid` (`TempestBaseAbilityManagerComponent.GetAbilityOfClass` _local_tempest_ability_component _array_element)
            (:`Is Valid`
              (return true))
            (:`Is Not Valid`
              (return false))))))
    (:`Is Not Valid`
      _))
  (return false))

(fn `Get Is State Currentely Active`
  (returns (ReturnValue :type Boolean))
  (return (== (`TempestBaseStateManagerComponent.GetCurrentActiveState` (`self.Get Tempest State Manager Component`)) self)))

(fn `Get Selected Ability`
  (returns (`Selected Ability To Trigger` :type "TempestBaseAbilityObject Class Reference"))
  (return (`self.Selected Ability To Trigger`)))

(fn `Get Tempest State Manager Component`
  (returns (`Tempest State Manager Component` :type "TempestBaseStateManagerComponent Object Reference"))
  (return (`self.Tempest State Manager Component`)))

(fn `IncrementTimeByUpdateRate`
  (returns (ReturnValue :type "Float (single-precision)"))
  (bind _output_get (set `self.TimePassed` (+ (`self.TimerUpdateRate`) (`self.TimePassed`))))
  (return _output_get))

(fn `RestartState`
  (params (ConditionCheck :type Boolean))
  (returns (ReturnValue :type Boolean))
  (if ConditionCheck
    (if (`self.CanPerformState`)
      _
      (else
        (return false))))
  (`self.PrepareStateValues`)
  (`self.StartState`)
  (return true))

(fn `Set Selected Ability`
  (params (`Selected Ability` :type "TempestBaseAbilityObject Class Reference"))
  (set `self.Selected Ability To Trigger` `Selected Ability`))

(fn `Set Tempest State Manager Component`
  (params (`New State Manager Component` :type "TempestBaseStateManagerComponent Object Reference"))
  (set `self.Tempest State Manager Component` `New State Manager Component`))