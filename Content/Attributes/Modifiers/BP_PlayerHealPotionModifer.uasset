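; Player heal potion attribute modifier that changes an attribute over time until the player enters the hit state.
; Each tick of the modification lazily fetches the Tempest state manager from the owning character's controller and reads the active state's gameplay tag.
; It runs the parent modification unless that tag is State.Hit, in which case it removes itself from the active modifiers.
; A separate function re-enables regeneration through a flag.
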(fn `Allow Regeneration`
  (locals (`Can Regenrate` :type Boolean))
  (set `local.Can Regenrate` true))

(fn `Modify Attribute OverTime`
  (locals (`Local Gameplay Tag` :type "GameplayTag Structure"))
  (bind _returnvalue (`TempestBaseStateManagerComponent.GetCurrentActiveState` (`self.Tempest State Manager Component`)))
  (`/Engine/EditorBlueprintResources/StandardMacros.IsValid` (`self.Tempest State Manager Component`)
    (:`Is Valid`
      _)
    (:`Is Not Valid`
      (bind _ascharacter (cast `Character` (`self.Owner Actor`)))
      (bind _output_get (set `self.Tempest State Manager Component` (`Actor.GetComponentByClass` (`Pawn.GetController` _ascharacter) "/Script/TempestCombatFramework.TempestBaseStateManagerComponent")))
      (`/Engine/EditorBlueprintResources/StandardMacros.IsValid` _output_get
        (:`Is Valid`
          _))))
  (`/Engine/EditorBlueprintResources/StandardMacros.IsValid` _returnvalue
    (:`Is Valid`
      (bind _output_get_2 (set `local.Local Gameplay Tag` (`TempestBaseStateObject.StateGameplayTag` _returnvalue)))
      (if (!= _output_get_2 (struct :`TagName` "State.Hit"))
        (`parent.Modify Attribute OverTime`)
        (else
          (`TempestAttributesComponents.RemoveFromActiveAttributeModifiers` (`self.Attributes Component`) self))))))