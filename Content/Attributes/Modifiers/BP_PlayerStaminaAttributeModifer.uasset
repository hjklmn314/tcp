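; Player stamina attribute modifier that gates the inherited over-time stamina change on the character's current state.
; It overrides ModifyAttributeOverTime, lazily caching the Tempest state manager component found on the owning character's controller.
; The parent logic runs only when a valid active state exists and its gameplay tag is outside the death, combat-action and sprint states it excludes.
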(fn `Modify Attribute OverTime`
  (locals (`Local Gameplay Tag` :type "GameplayTag Structure"))
  (bind _local_gameplay_tag (`local.Local Gameplay Tag`))
  (bind _returnvalue (`TempestBaseStateManagerComponent.GetCurrentActiveState` (`self.Tempest State Manager Component`)))
  (`/Engine/EditorBlueprintResources/StandardMacros.IsValid` (`self.Tempest State Manager Component`)
    (:`Is Valid`
      _)
    (:`Is Not Valid`
      (bind _ascharacter (cast `Character` (`self.Owner Actor`)))
      (bind _output_get (set `self.Tempest State Manager Component` (`Actor.GetComponentByClass` (`Pawn.GetController` _ascharacter) "/Script/TempestCombatFramework.TempestBaseStateManagerComponent")))
      (`/Engine/EditorBlueprintResources/StandardMacros.IsValid` _output_get
        (:`Is Valid`
          _))))
  (`/Engine/EditorBlueprintResources/StandardMacros.IsValid` _returnvalue
    (:`Is Valid`
      (set `local.Local Gameplay Tag` (`TempestBaseStateObject.StateGameplayTag` _returnvalue))
      (if (and (!= _local_gameplay_tag (struct :`TagName` "State.Death")) (!= _local_gameplay_tag (struct :`TagName` "State.Attack")) (!= _local_gameplay_tag (struct :`TagName` "State.Dodge")) (!= _local_gameplay_tag (struct :`TagName` "State.Normal Block")) (!= _local_gameplay_tag (struct :`TagName` "State.Sprint")))
        (`parent.Modify Attribute OverTime`)))))