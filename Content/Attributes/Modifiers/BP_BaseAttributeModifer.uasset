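; Base attribute modifier object that changes a gameplay-tagged attribute on the actor that is its outer, either instantly or over time.
; On construction it finds the owner's TempestAttributesComponents, looks up the attribute and registers itself as an active modifier.
; A zero duration applies the amount once and unregisters; otherwise a looping named timer applies it each interval.
; Timed modifiers track elapsed time and unregister on expiry, while indefinite ones keep ticking.
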(event `self.ConstructAttributeModifier`
  (bind _asactor (cast `Actor` (`KismetSystemLibrary.GetOuterObject` self)))
  (set `self.Owner Actor` _asactor)
  (set `self.Attributes Component` (`Actor.GetComponentByClass` (`self.Owner Actor`) "/Script/TempestCombatFramework.TempestAttributesComponents"))
  (`self.StartAttributeModifier`))

(event `self.StartAttributeModifier`
  (bind (_attributetomodify _bindefinite _modificationduration _modificationinterval _amounttoadd) (break `AttributeModifierProperties` (`self.ModiferProperties`)))
  (`/Engine/EditorBlueprintResources/StandardMacros.IsValid` (`self.Attributes Component`)
    (:`Is Valid`
      (bind _output_get (set `self.Attribute To Modify` (`TempestAttributesComponents.GetAttributeOfGameplayTag` (`self.Attributes Component`) (`.AttributeToModify` (break `AttributeModifierProperties` (`self.ModiferProperties`))))))
      (`/Engine/EditorBlueprintResources/StandardMacros.IsValid` _output_get
        (:`Is Valid`
          (`TempestAttributesComponents.AddToActiveAttributeModifiers` (`self.Attributes Component`) self)
          (if (== _modificationduration 0.0)
            (`TempestBaseAttributeObject.ModifyAttribute` (`self.Attribute To Modify`) _amounttoadd)
            (`TempestAttributesComponents.RemoveFromActiveAttributeModifiers` (`self.Attributes Component`) self)
            (else
              (`KismetSystemLibrary.K2_SetTimer` null "Modify Attribute OverTime" _modificationinterval true)
              (`self.Modify Attribute OverTime`))))))))

(fn `Modify Attribute OverTime`
  (bind (_attributetomodify _bindefinite _modificationduration _modificationinterval _amounttoadd) (break `AttributeModifierProperties` (`self.ModiferProperties`)))
  (if (not _bindefinite)
    (if (>= (`self.Passed Time`) _modificationduration)
      (`KismetSystemLibrary.K2_PauseTimer` null "Modify Attribute OverTime")
      (`KismetSystemLibrary.K2_ClearTimer` null "Modify Attribute OverTime")
      (`TempestAttributesComponents.RemoveFromActiveAttributeModifiers` (`self.Attributes Component`) self)
      (else
        (`TempestBaseAttributeObject.ModifyAttribute` (`self.Attribute To Modify`) _amounttoadd :!label _label)
        (set `self.Passed Time` (+ (`self.Passed Time`) _modificationinterval))))
    (else
      (goto _label))))