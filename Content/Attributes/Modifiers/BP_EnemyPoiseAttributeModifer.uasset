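; Enemy poise attribute modifier that applies its parent's over-time modification only while the owner is in a suitable state.
; It lazily caches the owning Character and the Tempest state manager component found on that Character's controller.
; Each modification calls the parent logic only if an active state exists and its gameplay tag is neither Death nor Hit.
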(fn `Modify Attribute OverTime`
  (locals (`Local Gameplay Tag` :type "GameplayTag Structure") (`Local Character` :type "Character Object Reference"))
  (bind _local_gameplay_tag (`local.Local Gameplay Tag`))
  (bind _local_character (`local.Local Character`))
  (bind _returnvalue (`Pawn.GetController` _local_character))
  (bind _returnvalue_2 (`TempestBaseStateManagerComponent.GetCurrentActiveState` (`self.Tempest State Manager Component`)))
  (`/Engine/EditorBlueprintResources/StandardMacros.IsValid` (`self.Tempest State Manager Component`)
    (:`Is Valid`
      _)
    (:`Is Not Valid`
      (bind _ascharacter (cast `Character` (`self.Owner Actor`)))
      (set `local.Local Character` _ascharacter)
      (`/Engine/EditorBlueprintResources/StandardMacros.IsValid` _local_character
        (:`Is Valid`
          (`/Engine/EditorBlueprintResources/StandardMacros.IsValid` _returnvalue
            (:`Is Valid`
              (bind _output_get (set `self.Tempest State Manager Component` (`Actor.GetComponentByClass` _returnvalue "/Script/TempestCombatFramework.TempestBaseStateManagerComponent")))
              (`/Engine/EditorBlueprintResources/StandardMacros.IsValid` _output_get
                (:`Is Valid`
                  _))))))))
  (`/Engine/EditorBlueprintResources/StandardMacros.IsValid` (`local.Local Character`)
    (:`Is Valid`
      (`/Engine/EditorBlueprintResources/StandardMacros.IsValid` _returnvalue_2
        (:`Is Valid`
          (set `local.Local Gameplay Tag` (`TempestBaseStateObject.StateGameplayTag` _returnvalue_2))
          (if (and (!= _local_gameplay_tag (struct :`TagName` "State.Death")) (!= _local_gameplay_tag (struct :`TagName` "State.Hit")))
            (`parent.Modify Attribute OverTime`)))))))