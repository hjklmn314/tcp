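; Base ability Blueprint that links to the performing actor's TempestBaseAbilityManagerComponent and provides shared cooldown, state and montage logic.
; On construct it caches that component, and on start it registers itself as the active ability.
; A timer clears the cooldown flag, which CanPerformAbility and CanRePerformAbility return uninverted.
; PlayAbilityMontage plays a montage on the Character's mesh, records it and optionally jumps to a section.
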(event `self.ConstructAbility`
  (`self.Set Tempest Ability Component` (`Actor.GetComponentByClass` (`self.GetPerformingActor`) "/Script/TempestCombatFramework.TempestBaseAbilityManagerComponent")))

(event `self.StartAbility`
  (`TempestBaseAbilityManagerComponent.SetCurrentActiveAbility` (`self.Get Tempest Ability Component`) self))

(event `self.CooldownReset`
  (set `self.bAbilityOnCooldown` false))

(event `self.ApplyAbilityCooldown`
  (bind _cooldownduration (`self.CooldownDuration`))
  (if (> _cooldownduration 0.0)
    (set `self.bAbilityOnCooldown` true)
    (`KismetSystemLibrary.K2_SetTimer` null "CooldownReset" _cooldownduration)
    (else
      (set `self.bAbilityOnCooldown` false))))

(fn `CanAbilityBeCanceled`
  (returns (ReturnValue :type Boolean))
  (return true))

(fn `CanPerformAbility`
  (returns (ReturnValue :type Boolean))
  (return (`self.GetIsAbilityOnCooldown`)))

(fn `CanRePerformAbility`
  (returns (ReturnValue :type Boolean))
  (return (`self.CanPerformAbility`)))

(fn `Get Is Current Ability Active`
  (returns (ReturnValue :type Boolean))
  (return (== (`TempestBaseAbilityManagerComponent.GetCurrentActiveAbility` (`self.Get Tempest Ability Component`)) self)))

(fn `Get Tempest Ability Component`
  (returns (TempestAbilityComponent :type "TempestBaseAbilityManagerComponent Object Reference"))
  (return (`self.TempestAbilityComponent`)))

(fn `GetIsAbilityOnCooldown`
  (returns (ReturnValue :type Boolean))
  (return (`self.bAbilityOnCooldown`)))

(fn `PlayAbilityMontage`
  (params (MontageToPlay :type "AnimMontage Object Reference") (InPlayRate :type "Float (double-precision)" :default 1.0) (ReturnValueType :type "EMontagePlayReturnType Enum" :default "Duration") (InTimeToStartMontageAt :type "Float (double-precision)" :default 0.0) (StartSectionName :type Name :default "None") (bStopAllMontages :type Boolean :default true))
  (returns (ReturnValue :type "Float (double-precision)"))
  (bind _startsectionname (`local.StartSectionName`))
  (bind _ascharacter (cast `Character` (`self.GetPerformingActor`)))
  (bind _returnvalue (`SkeletalMeshComponent.GetAnimInstance` (`Character.Mesh` _ascharacter)))
  (bind _returnvalue_2 (`AnimInstance.Montage_Play` _returnvalue MontageToPlay InPlayRate ReturnValueType InTimeToStartMontageAt bStopAllMontages))
  (`self.SetActiveAbilityMontage` (`local.MontageToPlay`))
  (if (!= _startsectionname "None")
    (`AnimInstance.Montage_JumpToSection` _returnvalue _startsectionname (`local.MontageToPlay`)))
  (return _returnvalue_2))

(fn `Set Tempest Ability Component`
  (params (`New TempestAbilityComponent` :type "TempestBaseAbilityManagerComponent Object Reference"))
  (set `self.TempestAbilityComponent` `New TempestAbilityComponent`))