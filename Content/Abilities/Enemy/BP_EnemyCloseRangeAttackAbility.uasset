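; Close-range enemy attack ability that plays a random attack montage and puts the enemy into its Attack state.
; StartAbility registers itself as the active ability, falling back to the enemy's montages for this class when none are set.
; CanPerformAbility requires a valid montage and a short-range distance check.
; Deflect and clash notifications switch the enemy's state manager to Deflected or Clashed through gameplay-tag lookups.
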(event `self.StartAbility`
  (bind (_outitem _outindex) (`KismetArrayLibrary.Array_Random` (`self.Attack Montages`)))
  (bind _enemystatemanagercomponent (`/TempestCombatFramework/Controllers/TCF_MasterEnemy_AIC_BP.EnemyStateManagerComponent` (`/TempestCombatFramework/Characters/TCF_MasterEnemy_BP.Master Enemy AIC` (`self.Master Enemy BP`))))
  (`TempestBaseAbilityManagerComponent.SetCurrentActiveAbility` (`self.Get Tempest Ability Component`) self)
  (if (not (> (`KismetArrayLibrary.Array_Length` (`self.Attack Montages`)) 0))
    (bind _list_of_montages (`self.Get Enemy Ability's Montages` (`GameplayStatics.GetObjectClass` self)))
    (set `self.Attack Montages` _list_of_montages))
  (`self.PlayAbilityMontage` _outitem)
  (set `self.Choosen Attack Index` _outindex)
  (`TempestBaseStateManagerComponent.SetCurrentActiveState` _enemystatemanagercomponent (`TempestBaseStateManagerComponent.GetStateOfGameplayTag` _enemystatemanagercomponent (struct :`TagName` "State.Attack"))))

(event `/TempestCombatFramework/Interfaces/BPI_TempestAbilitiesAndStates.Inform Target Of Deflect`
  (bind _enemystatemanagercomponent (`/TempestCombatFramework/Controllers/TCF_MasterEnemy_AIC_BP.EnemyStateManagerComponent` (`/TempestCombatFramework/Characters/TCF_MasterEnemy_BP.Master Enemy AIC` (`self.Master Enemy BP`))))
  (`TempestBaseStateManagerComponent.TryPerformStateOfClass` _enemystatemanagercomponent (`GameplayStatics.GetObjectClass` (`TempestBaseStateManagerComponent.GetStateOfGameplayTag` _enemystatemanagercomponent (struct :`TagName` "State.Deflected"))) true))

(event `/TempestCombatFramework/Interfaces/BPI_TempestAbilitiesAndStates.Inform Target Of Clash`
  (bind _enemystatemanagercomponent (`/TempestCombatFramework/Controllers/TCF_MasterEnemy_AIC_BP.EnemyStateManagerComponent` (`/TempestCombatFramework/Characters/TCF_MasterEnemy_BP.Master Enemy AIC` (`self.Master Enemy BP`))))
  (`TempestBaseStateManagerComponent.TryPerformStateOfClass` _enemystatemanagercomponent (`GameplayStatics.GetObjectClass` (`TempestBaseStateManagerComponent.GetStateOfGameplayTag` _enemystatemanagercomponent (struct :`TagName` "State.Clashed"))) true))

(fn `CanPerformAbility`
  (returns (ReturnValue :type Boolean))
  (bind _list_of_montages (`self.Get Enemy Ability's Montages` (`GameplayStatics.GetObjectClass` self)))
  (if (or (`KismetSystemLibrary.IsValid` (`|GetArrayItem` (`self.Attack Montages`))) (`KismetSystemLibrary.IsValid` (`|GetArrayItem` _list_of_montages)))
    (bind _returnvalue (`self.Calculate Distance Difference `))
    (return (`KismetMathLibrary.InRange_FloatFloat` _returnvalue 1.0 300.0))
    (else
      (return false))))

(fn `Get Block Time Since Last Clicked`
  (returns (`Return Value` :type "Float (double-precision)"))
  (return 0.0))

(fn `Get Montage Counter For Ability`
  (returns (`Counter Montage` :type "AnimMontage Object Reference"))
  (return null))