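; Base enemy ability for the Tempest combat framework that caches its owning master enemy on construction and supplies shared helpers.
; On end, it clears the active ability and has the AI controller's current state decide the next one, handing control back to the state machine.
; Helpers measure distance and pitch/yaw offset to the combat target, returning zero without one.
; Another pulls an ability class's montages from the enemy data asset.
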(event `self.ConstructAbility`
  (`parent.ConstructAbility`)
  (bind _astcf_master_enemy_bp (cast `/TempestCombatFramework/Characters/TCF_MasterEnemy_BP` (`self.GetPerformingActor`)))
  (set `self.Master Enemy BP` _astcf_master_enemy_bp))

(event `self.EndAbility`
  (`TempestBaseAbilityManagerComponent.SetCurrentActiveAbility` (`self.Get Tempest Ability Component`) null)
  (bind _asbp_base_ai_state (cast `/TempestCombatFramework/States/Enemy/BP_Base_AI_State` (`TempestBaseStateManagerComponent.GetCurrentActiveState` (`/TempestCombatFramework/Controllers/TCF_MasterEnemy_AIC_BP.EnemyStateManagerComponent` (`/TempestCombatFramework/Characters/TCF_MasterEnemy_BP.Master Enemy AIC` (`self.Master Enemy BP`))))))
  (`/TempestCombatFramework/States/Enemy/BP_Base_AI_State.Decide Next State` _asbp_base_ai_state))

(fn `Calculate Distance Difference `
  (returns (ReturnValue :type "Float (double-precision)"))
  (bind _master_enemy_bp (`self.Master Enemy BP`))
  (bind _return_value (`/TempestCombatFramework/Components/AI/AICombatComponent.Get Combat Target` (`/TempestCombatFramework/Characters/TCF_MasterEnemy_BP.BP_TempestEnemyCombatComponent` _master_enemy_bp)))
  (`/Engine/EditorBlueprintResources/StandardMacros.IsValid` _return_value
    (:`Is Valid`
      (return (`KismetMathLibrary.VSize` (- (`Actor.K2_GetActorLocation` _return_value) (`Actor.K2_GetActorLocation` _master_enemy_bp)))))
    (:`Is Not Valid`
      (return 0.0))))

(fn `Calculate Pitch & Yaw Difference `
  (returns (`Return Value Y (Pitch)` :type "Float (double-precision)") (`Return Value Z (Yaw)` :type "Float (double-precision)"))
  (bind _master_enemy_bp (`self.Master Enemy BP`))
  (bind _return_value (`/TempestCombatFramework/Components/AI/AICombatComponent.Get Combat Target` (`/TempestCombatFramework/Characters/TCF_MasterEnemy_BP.BP_TempestEnemyCombatComponent` _master_enemy_bp)))
  (bind (_returnvalue_roll _returnvalue_pitch _returnvalue_yaw) (`KismetMathLibrary.BreakRotator` (`KismetMathLibrary.NormalizedDeltaRotator` (`Actor.K2_GetActorRotation` _master_enemy_bp) (`KismetMathLibrary.FindLookAtRotation` (`Actor.K2_GetActorLocation` _master_enemy_bp) (`Actor.K2_GetActorLocation` _return_value)))))
  (`/Engine/EditorBlueprintResources/StandardMacros.IsValid` _return_value
    (:`Is Valid`
      (return _returnvalue_pitch _returnvalue_yaw))
    (:`Is Not Valid`
      (return 0.0 0.0))))

(fn `Get Enemy Ability's Montages`
  (params (`Class To Check For` :type "/Game/Abilities/Enemy/BP_BaseEnemyAbility Class Reference"))
  (returns (`List Of Montages` :type "Array of AnimMontage Object Reference"))
  (bind _master_enemy_bp (`self.Master Enemy BP`))
  (bind _enemy_info (`/TempestCombatFramework/Characters/TCF_MasterEnemy_BP.Get Enemy Data Asset` _master_enemy_bp))
  (`/Engine/EditorBlueprintResources/StandardMacros.IsValid` _master_enemy_bp
    (:`Is Valid`
      (`/Engine/EditorBlueprintResources/StandardMacros.IsValid` _enemy_info
        (:`Is Valid`
          (for _array_element (`/TempestCombatFramework/DataAssets/DA_Enemyinfo.Abilities Animations` _enemy_info)
            (bind (_ability _listofmontages) (break `/TempestCombatFramework/StructuresEnums/S_AbilityMontages` _array_element))
            (if (== _ability `Class To Check For`)
              (return _listofmontages))))))))