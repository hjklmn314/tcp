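; Enemy ability, named for a 180-degree left turn, that rotates the enemy toward its combat target during a turn montage.
; It is allowed when the yaw difference falls within an angle range and a montage exists for the class.
; On start it caches the transform and plays a random montage.
; Each tick, a positive animation curve scales the divided yaw delta to the target, and actor rotation blends halfway toward that result.
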(event `self.StartAbility`
  (bind _master_enemy_bp (`self.Master Enemy BP`))
  (`TempestBaseAbilityManagerComponent.SetCurrentActiveAbility` (`self.Get Tempest Ability Component`) self)
  (bind _list_of_montages (`self.Get Enemy Ability's Montages` (`GameplayStatics.GetObjectClass` self)))
  (bind _outitem (`KismetArrayLibrary.Array_Random` _list_of_montages))
  (`/Engine/EditorBlueprintResources/StandardMacros.IsValid` _outitem
    (:`Is Valid`
      (set `self.Turning Montage` _outitem)
      (set `self.Original Location` (`Actor.K2_GetActorLocation` _master_enemy_bp))
      (set `self.Original Rotation` (`Actor.K2_GetActorRotation` _master_enemy_bp)))
    (:`Is Not Valid`
      _))
  (`self.PlayAbilityMontage` (`self.Turning Montage`) 1.0 "MontageLength"))

(event `self.TickAbility`
  (params (TickTime :type "Float (single-precision)"))
  (bind _master_enemy_bp (`self.Master Enemy BP`))
  (bind _returnvalue (`SkeletalMeshComponent.GetAnimInstance` (`Character.Mesh` (`self.Master Enemy BP`))))
  (bind _returnvalue_2 (`AnimInstance.GetCurveValue` _returnvalue (`self.Curve Name`)))
  (`parent.TickAbility` TickTime)
  (if (and (!= (`self.Original Location`) (0.0 0.0 0.0)) (`AnimInstance.Montage_IsPlaying` _returnvalue (`self.GetActiveAbilityMontage`)))
    (if (> _returnvalue_2 0.0)
      (`Actor.K2_SetActorRotation` _master_enemy_bp (`KismetMathLibrary.RLerp` (`Actor.K2_GetActorRotation` _master_enemy_bp) (`KismetMathLibrary.MakeRotator` (.roll (`self.Original Rotation`)) (.pitch (`self.Original Rotation`)) (+ (.yaw (`self.Original Rotation`)) (* _returnvalue_2 (/ (.yaw (`KismetMathLibrary.NormalizedDeltaRotator` (`KismetMathLibrary.FindLookAtRotation` (`self.Original Location`) (`Actor.K2_GetActorLocation` (`/TempestCombatFramework/Components/AI/AICombatComponent.Get Combat Target` (`/TempestCombatFramework/Characters/TCF_MasterEnemy_BP.BP_TempestEnemyCombatComponent` (`self.Master Enemy BP`))))) (`self.original rotation`))) (`self.Division Amount`))))) 0.5 true) true))))

(fn `CanPerformAbility`
  (returns (ReturnValue :type Boolean))
  (bind _list_of_montages (`self.Get Enemy Ability's Montages` (`GameplayStatics.GetObjectClass` self)))
  (bind (_return_value_y__pitch_ _return_value_z__yaw_) (`self.Calculate Pitch & Yaw Difference `))
  (return (and (`KismetMathLibrary.InRange_FloatFloat` _return_value_z__yaw_ (`self.Min Angle`) (`self.Max Angle`)) (`KismetSystemLibrary.IsValid` (`KismetArrayLibrary.Array_Random` _list_of_montages)))))