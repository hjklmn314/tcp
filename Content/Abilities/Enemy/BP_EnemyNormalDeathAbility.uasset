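; Enemy ability that plays a death animation and can always be performed.
; On start it registers as the active ability on the Tempest ability component and stops the enemy's current montage.
; It then picks a random montage from those mapped to its class and plays it as the ability montage.
; EndAbility adds no logic.
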(event `self.StartAbility`
  (`TempestBaseAbilityManagerComponent.SetCurrentActiveAbility` (`self.Get Tempest Ability Component`) self)
  (`Character.StopAnimMontage` (`self.Master Enemy BP`) null)
  (bind _list_of_montages (`self.Get Enemy Ability's Montages` (`GameplayStatics.GetObjectClass` self)))
  (bind _outitem (`KismetArrayLibrary.Array_Random` _list_of_montages))
  (`/Engine/EditorBlueprintResources/StandardMacros.IsValid` _outitem
    (:`Is Valid`
      (set `self.Death Montage` _outitem))
    (:`Is Not Valid`
      _))
  (`self.PlayAbilityMontage` (`self.Death Montage`) 1.0 "MontageLength"))

(event `self.EndAbility`)

(fn `CanPerformAbility`
  (returns (ReturnValue :type Boolean))
  (return true))