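; Enemy blocking ability that plays a random block montage from the enemy's montage set for this ability class and registers itself as the active ability.
; It can activate only when the enemy is not dead, parried or deflecting, no normal deflect ability is active, and it is not already active.
; Activation also requires passing distance and facing-angle checks.
; On end, it resets the enemy's widget location offset.
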(event `self.StartAbility`
  (`TempestBaseAbilityManagerComponent.SetCurrentActiveAbility` (`self.Get Tempest Ability Component`) self)
  (bind _list_of_montages (`self.Get Enemy Ability's Montages` (`GameplayStatics.GetObjectClass` self)))
  (set `self.Blocking Montages` _list_of_montages)
  (`self.PlayAbilityMontage` (`KismetArrayLibrary.Array_Random` (`self.Blocking Montages`)) 1.0 "MontageLength"))

(event `self.EndAbility`
  (`parent.EndAbility`)
  (message `/TempestCombatFramework/Interfaces/BPI_TargetingSystem.Offset Widget Location` (`self.Master Enemy BP`) (0.0 0.0 0.0)))

(fn `CanPerformAbility`
  (returns (ReturnValue :type Boolean))
  (bind _master_enemy_bp (`self.Master Enemy BP`))
  (bind _stategameplaytag (`TempestBaseStateObject.StateGameplayTag` (`TempestBaseStateManagerComponent.GetCurrentActiveState` (`/TempestCombatFramework/Controllers/TCF_MasterEnemy_AIC_BP.EnemyStateManagerComponent` (`/TempestCombatFramework/Characters/TCF_MasterEnemy_BP.Master Enemy AIC` _master_enemy_bp)))))
  (if (and (!= _stategameplaytag (struct :`TagName` "State.Death")) (!= _stategameplaytag (struct :`TagName` "State.Parried")) (!= _stategameplaytag (struct :`TagName` "State.Deflect")))
    (bind _returnvalue (`self.Calculate Distance Difference `))
    (bind (_return_value_y__pitch_ _return_value_z__yaw_) (`self.Calculate Pitch & Yaw Difference `))
    (return (and (`KismetMathLibrary.InRange_FloatFloat` _return_value_z__yaw_ -60.0 60.0) (`KismetMathLibrary.InRange_FloatFloat` _returnvalue 0.0 350.0) (not (`self.Get Is Current Ability Active`)) (!= (`/TempestCombatFramework/Components/BP_TempestAbilitySystemComponent.Get Current Active Ability Tag` (`/TempestCombatFramework/Characters/TCF_MasterEnemy_BP.BP_TempestAbilitySystemComponent` _master_enemy_bp)) (struct :`TagName` "Ability.Deflect.Normal"))))
    (else
      (return false))))