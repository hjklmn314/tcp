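; Enemy ability that plays the reaction to being riposted, allowed only when the enemy is not dead, is prone to riposte and the ability is off cooldown.
; On start it picks one of two montages by yaw difference, applies an impact effect through the defense property and shakes the camera.
; A brief custom time dilation on both attacker and enemy creates hit stop.
; Ending the ability resets the enemy's widget offset.
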(event `self.StartAbility`
  (bind _master_enemy_bp (`self.Master Enemy BP`))
  (bind _returnvalue (`TempestAttackPropertiesObject.GetAttackPropertyOwner` (`TempestCombatComponent.ReceivedAttackProperty` (`/TempestCombatFramework/Characters/TCF_MasterEnemy_BP.BP_TempestEnemyCombatComponent` _master_enemy_bp))))
  (`TempestBaseAbilityManagerComponent.SetCurrentActiveAbility` (`self.Get Tempest Ability Component`) self)
  (bind _list_of_montages (`self.Get Enemy Ability's Montages` (`GameplayStatics.GetObjectClass` self)))
  (set `self.Riposted Montages` _list_of_montages)
  (bind (_return_value_y__pitch_ _return_value_z__yaw_) (`self.Calculate Pitch & Yaw Difference `))
  (bind _output_get (set `self.Selected Index` (select `bool` (`KismetMathLibrary.InRange_FloatFloat` _return_value_z__yaw_ -90.0 90.0) :`false` 1)))
  (`self.PlayAbilityMontage` (`|GetArrayItem` (`self.Riposted Montages`) _output_get) 1.0 "MontageLength")
  (bind _asbp_base_defense_property (cast `/TempestCombatFramework/DefenseProperties/BP_BaseDefenseProperty` (`TempestCombatComponent.OwnerDefenseProperty` (`/TempestCombatFramework/Characters/TCF_MasterEnemy_BP.BP_TempestEnemyCombatComponent` (`self.Master Enemy BP`)))))
  (`/TempestCombatFramework/DefenseProperties/BP_BaseDefenseProperty.Apply Hit Effect Of Class` _asbp_base_defense_property (`self.Impact Effect Class`))
  (`PlayerCameraManager.StartCameraShake` :`self` (`GameplayStatics.GetPlayerCameraManager` 0) :`ShakeClass` "/Game/TempestCombatFramework/Camera/CameraShake/BP_NormalHitCameraShake.BP_NormalHitCameraShake_C")
  (`KismetSystemLibrary.Delay` 0.05)
  (bind _output_get_2 (set `Actor.CustomTimeDilation` 0.1 _returnvalue))
  (set `Actor.CustomTimeDilation` _output_get_2 _master_enemy_bp)
  (`KismetSystemLibrary.Delay` 0.05)
  (bind _output_get_3 (set `Actor.CustomTimeDilation` 1.0 _returnvalue))
  (set `Actor.CustomTimeDilation` _output_get_3 _master_enemy_bp))

(event `self.EndAbility`
  (`parent.EndAbility`)
  (message `/TempestCombatFramework/Interfaces/BPI_TargetingSystem.Offset Widget Location` (`self.Master Enemy BP`) (0.0 0.0 0.0)))

(fn `CanPerformAbility`
  (returns (ReturnValue :type Boolean))
  (bind _master_enemy_bp (`self.Master Enemy BP`))
  (bind _returnvalue (`TempestBaseStateManagerComponent.GetCurrentActiveState` (`/TempestCombatFramework/Controllers/TCF_MasterEnemy_AIC_BP.EnemyStateManagerComponent` (`/TempestCombatFramework/Characters/TCF_MasterEnemy_BP.Master Enemy AIC` _master_enemy_bp))))
  (bind _returnvalue_2 (`BlueprintGameplayTagLibrary.HasTag` (`TempestCombatComponent.GetCombatStatus` (`/TempestCombatFramework/Characters/TCF_MasterEnemy_BP.BP_TempestEnemyCombatComponent` _master_enemy_bp)) (struct :`TagName` "Status.Combat.Weakness.Prone To Riposte")))
  (`/Engine/EditorBlueprintResources/StandardMacros.IsValid` _returnvalue
    (:`Is Valid`
      (if (!= (`TempestBaseStateObject.StateGameplayTag` _returnvalue) (struct :`TagName` "State.Death"))
        (if _returnvalue_2
          (return (and _returnvalue_2 (not (`self.GetIsAbilityOnCooldown`))))
          (else
            _))))
    (:`Is Not Valid`
      _))
  (return false))