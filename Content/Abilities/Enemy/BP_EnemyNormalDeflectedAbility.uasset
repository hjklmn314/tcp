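; Enemy ability that plays a deflected reaction when the enemy's normal attack is deflected.
; On start it registers as the current active ability, then plays a random montage from the enemy's montage set for this ability class.
; It can only run while the enemy is not in the Death state and the computed yaw difference lies within a frontal cone.
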(event `self.StartAbility`
  (`TempestBaseAbilityManagerComponent.SetCurrentActiveAbility` (`self.Get Tempest Ability Component`) self)
  (bind _list_of_montages (`self.Get Enemy Ability's Montages` (`GameplayStatics.GetObjectClass` self)))
  (set `self.Deflected Montages` _list_of_montages)
  (`self.PlayAbilityMontage` (`KismetArrayLibrary.Array_Random` (`self.Deflected Montages`)) 1.0 "MontageLength"))

(fn `CanPerformAbility`
  (returns (ReturnValue :type Boolean))
  (if (!= (`TempestBaseStateObject.StateGameplayTag` (`TempestBaseStateManagerComponent.GetCurrentActiveState` (`/TempestCombatFramework/Controllers/TCF_MasterEnemy_AIC_BP.EnemyStateManagerComponent` (`/TempestCombatFramework/Characters/TCF_MasterEnemy_BP.Master Enemy AIC` (`self.Master Enemy BP`))))) (struct :`TagName` "State.Death"))
    (bind (_return_value_y__pitch_ _return_value_z__yaw_) (`self.Calculate Pitch & Yaw Difference `))
    (return (`KismetMathLibrary.InRange_FloatFloat` _return_value_z__yaw_ -65.0 65.0))
    (else
      (return false))))