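; Enemy ability for being assassinated, built on the Tempest ability and combat components and allowed only while the enemy's combat status lacks the InCombat tag.
; On start it registers as the active ability and plays a montage picked at random from those mapped to its class.
; It then adds the InCombat tag and switches the AI controller's state manager to the Death state.
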(event `self.StartAbility`
  (bind _enemystatemanagercomponent (`/TempestCombatFramework/Controllers/TCF_MasterEnemy_AIC_BP.EnemyStateManagerComponent` (`/TempestCombatFramework/Characters/TCF_MasterEnemy_BP.Master Enemy AIC` (`self.Master Enemy BP`))))
  (`TempestBaseAbilityManagerComponent.SetCurrentActiveAbility` (`self.Get Tempest Ability Component`) self)
  (bind _list_of_montages (`self.Get Enemy Ability's Montages` (`GameplayStatics.GetObjectClass` self)))
  (bind _outitem (`KismetArrayLibrary.Array_Random` _list_of_montages))
  (`/Engine/EditorBlueprintResources/StandardMacros.IsValid` _outitem
    (:`Is Valid`
      (set `self.Assasinated Montage` _outitem))
    (:`Is Not Valid`
      _))
  (`self.PlayAbilityMontage` (`self.Assasinated Montage`) 1.0 "MontageLength")
  (`TempestCombatComponent.ModifyCombatStatus` (`/TempestCombatFramework/Characters/TCF_MasterEnemy_BP.BP_TempestEnemyCombatComponent` (`self.Master Enemy BP`)) (struct :`TagName` "Status.Combat.InCombat") "Add")
  (`TempestBaseStateManagerComponent.SetCurrentActiveState` _enemystatemanagercomponent (`TempestBaseStateManagerComponent.GetStateOfGameplayTag` _enemystatemanagercomponent (struct :`TagName` "State.Death"))))

(fn `CanPerformAbility`
  (returns (ReturnValue :type Boolean))
  (return (not (`BlueprintGameplayTagLibrary.HasTag` (`TempestCombatComponent.GetCombatStatus` (`/TempestCombatFramework/Characters/TCF_MasterEnemy_BP.BP_TempestEnemyCombatComponent` (`self.Master Enemy BP`))) (struct :`TagName` "Status.Combat.InCombat")))))