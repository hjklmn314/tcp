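; Enemy ability that plays an unequip montage.
; On start it registers itself as the active ability on the Tempest ability component, then looks up the enemy's montages for this ability class.
; A random valid entry replaces the default UnEquipMontage before playback.
; The validity check and assignment each read a separate Random output, so the assigned montage can differ from the checked one.
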(event `self.StartAbility`
  (`TempestBaseAbilityManagerComponent.SetCurrentActiveAbility` (`self.Get Tempest Ability Component`) self)
  (bind _list_of_montages (`self.Get Enemy Ability's Montages` (`GameplayStatics.GetObjectClass` self)))
  (bind _outitem (`KismetArrayLibrary.Array_Random` _list_of_montages))
  (`/Engine/EditorBlueprintResources/StandardMacros.IsValid` _outitem
    (:`Is Valid`
      (set `self.UnEquip Montage` _outitem))
    (:`Is Not Valid`
      _))
  (`self.PlayAbilityMontage` (`self.UnEquip Montage`) 1.0 "MontageLength"))