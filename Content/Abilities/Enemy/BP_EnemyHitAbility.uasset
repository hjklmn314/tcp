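; BP_EnemyHitAbility is an enemy hit ability that plays a random montage from those registered for its class.
; On start it sets itself as the Tempest ability component's current active ability.
; It looks up montages by its own class, stores them in HitMontages and plays a random one through PlayAbilityMontage.
; CanPerformAbility always returns true, so the ability itself never blocks activation.
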(event `self.StartAbility`
  (`TempestBaseAbilityManagerComponent.SetCurrentActiveAbility` (`self.Get Tempest Ability Component`) self)
  (bind _list_of_montages (`self.Get Enemy Ability's Montages` (`GameplayStatics.GetObjectClass` self)))
  (bind _output_get (set `self.Hit Montages` _list_of_montages))
  (`self.PlayAbilityMontage` (`KismetArrayLibrary.Array_Random` _output_get) 1.0 "MontageLength"))

(fn `CanPerformAbility`
  (returns (ReturnValue :type Boolean))
  (return true))