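; Enemy ability that reacts to a blocked hit, allowed only while the enemy is not dead and the calculated yaw difference is within a frontal cone.
; On start it registers as the active ability, boosts Poise by a huge amount, plays a blocked montage and applies the defense property's impact effect.
; A brief hit-stop then slows and restores custom time dilation on both attacker and enemy.
; Ending the ability zeroes the enemy's widget offset.
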(event `self.StartAbility`
  (bind _master_enemy_bp (`self.Master Enemy BP`))
  (bind _returnvalue (`TempestAttackPropertiesObject.GetAttackPropertyOwner` (`TempestCombatComponent.ReceivedAttackProperty` (`/TempestCombatFramework/Characters/TCF_MasterEnemy_BP.BP_TempestEnemyCombatComponent` _master_enemy_bp))))
  (`TempestBaseAbilityManagerComponent.SetCurrentActiveAbility` (`self.Get Tempest Ability Component`) self)
  (`TempestBaseAttributeObject.ModifyAttribute` (`TempestAttributesComponents.GetAttributeOfGameplayTag` (`/TempestCombatFramework/Characters/TCF_MasterEnemy_BP.BP_TempestAttributesComponents` (`self.Master Enemy BP`)) (struct :`TagName` "Attribute.Poise")) 1000000.0)
  (`self.PlayAbilityMontage` (`|GetArrayItem` (`self.Blocked Montages`)) 1.0 "MontageLength")
  (bind _asbp_base_defense_property (cast `/TempestCombatFramework/DefenseProperties/BP_BaseDefenseProperty` (`TempestCombatComponent.OwnerDefenseProperty` (`/TempestCombatFramework/Characters/TCF_MasterEnemy_BP.BP_TempestEnemyCombatComponent` (`self.Master Enemy BP`)))))
  (`/TempestCombatFramework/DefenseProperties/BP_BaseDefenseProperty.Apply Hit Effect Of Class` _asbp_base_defense_property (`self.Impact Effect Class`))
  (`KismetSystemLibrary.Delay` 0.05)
  (bind _output_get (set `Actor.CustomTimeDilation` 0.1 _returnvalue))
  (set `Actor.CustomTimeDilation` _output_get _master_enemy_bp)
  (`KismetSystemLibrary.Delay` 0.05)
  (bind _output_get_2 (set `Actor.CustomTimeDilation` 1.0 _returnvalue))
  (set `Actor.CustomTimeDilation` _output_get_2 _master_enemy_bp))

(event `self.EndAbility`
  (`parent.EndAbility`)
  (message `/TempestCombatFramework/Interfaces/BPI_TargetingSystem.Offset Widget Location` (`self.Master Enemy BP`) (0.0 0.0 0.0)))

(fn `CanPerformAbility`
  (returns (ReturnValue :type Boolean))
  (if (!= (`TempestBaseStateObject.StateGameplayTag` (`TempestBaseStateManagerComponent.GetCurrentActiveState` (`/TempestCombatFramework/Controllers/TCF_MasterEnemy_AIC_BP.EnemyStateManagerComponent` (`/TempestCombatFramework/Characters/TCF_MasterEnemy_BP.Master Enemy AIC` (`self.Master Enemy BP`))))) (struct :`TagName` "State.Death"))
    (bind (_return_value_y__pitch_ _return_value_z__yaw_) (`self.Calculate Pitch & Yaw Difference `))
    (return (`KismetMathLibrary.InRange_FloatFloat` _return_value_z__yaw_ -65.0 65.0))
    (else
      (return false))))