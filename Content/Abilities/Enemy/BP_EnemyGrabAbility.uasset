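; Enemy grab attack ability that plays a grab montage chosen by the found index in the owner's grab attack property.
; On start it lets the capsule pass through pawns, async-loads that montage, plays it from the GrabSection and registers itself as the active ability.
; It then constructs the property entry's syncing object and ticks it while the ability runs.
; Ending clears the object and restores pawn blocking.
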(event `self.StartAbility`
  (bind _asbp_grab_attack_property (cast `/TempestCombatFramework/AttackProperties/BP_GrabAttackProperty` (`TempestCombatComponent.OwnerAttackProperty` (`/TempestCombatFramework/Characters/TCF_MasterEnemy_BP.BP_TempestEnemyCombatComponent` (`self.Master Enemy BP`)))))
  (bind _found_index (`/TempestCombatFramework/AttackProperties/BP_GrabAttackProperty.Get Found Index` _asbp_grab_attack_property))
  (`PrimitiveComponent.SetCollisionResponseToChannel` (`Character.CapsuleComponent` (`self.Master Enemy BP`)) "ECC_Pawn" "ECR_Ignore")
  (bind (_hittargettag _targetanimmontages _owneranimmontage _syncingobject) (break `/TempestCombatFramework/StructuresEnums/S_GrabProperties` (`|GetArrayItem` (`/TempestCombatFramework/AttackProperties/BP_GrabAttackProperty.Grab Anim Montages` _asbp_grab_attack_property) _found_index)))
  (bind _object (`|LoadAsset` _owneranimmontage)
    (:`Completed`
      (bind _asanim_montage (cast `AnimMontage` _object))
      (set `self.Grab Montage` _asanim_montage)
      (`self.PlayAbilityMontage` (`self.Grab Montage`) 1.0 "MontageLength" 0.0 "GrabSection")
      (`TempestBaseAbilityManagerComponent.SetCurrentActiveAbility` (`self.Get Tempest Ability Component`) self)
      (bind _returnvalue (`|GenericCreateObject` (`self.Master Enemy BP`) _syncingobject))
      (bind _output_get (set `self.Syncing Object` _returnvalue))
      (`/TempestCombatFramework/Animation/Objects/BP_BaseSyncObject.Construct Syncing Object` _output_get))))

(event `self.TickAbility`
  (params (TickTime :type "Float (single-precision)"))
  (bind _syncing_object (`self.Syncing Object`))
  (`/Engine/EditorBlueprintResources/StandardMacros.IsValid` _syncing_object
    (:`Is Valid`
      (`/TempestCombatFramework/Animation/Objects/BP_BaseSyncObject.Tick Syncing Object` _syncing_object))))

(event `self.EndAbility`
  (`parent.EndAbility`)
  (set `self.Syncing Object` null)
  (`PrimitiveComponent.SetCollisionResponseToChannel` (`Character.CapsuleComponent` (`self.Master Enemy BP`)) "ECC_Pawn" "ECR_Block"))

(fn `CanPerformAbility`
  (returns (ReturnValue :type Boolean))
  (return true))