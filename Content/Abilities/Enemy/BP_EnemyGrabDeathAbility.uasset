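; Enemy ability that plays a death montage when an enemy dies during a grab hit reaction.
; It can run only while the active ability is the grab hit react and the Health attribute is at or below its minimum.
; On start it becomes the active ability, switches the AI state manager to the Death state and plays a random montage from this ability's montage set.
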(event `self.StartAbility`
  (bind _enemystatemanagercomponent (`/TempestCombatFramework/Controllers/TCF_MasterEnemy_AIC_BP.EnemyStateManagerComponent` (`/TempestCombatFramework/Characters/TCF_MasterEnemy_BP.Master Enemy AIC` (`self.Master Enemy BP`))))
  (`TempestBaseAbilityManagerComponent.SetCurrentActiveAbility` (`self.Get Tempest Ability Component`) self)
  (`TempestBaseStateManagerComponent.PerformStateOfClass` _enemystatemanagercomponent (`GameplayStatics.GetObjectClass` (`TempestBaseStateManagerComponent.GetStateOfGameplayTag` _enemystatemanagercomponent (struct :`TagName` "State.Death"))))
  (bind _list_of_montages (`self.Get Enemy Ability's Montages` (`GameplayStatics.GetObjectClass` self)))
  (bind _outitem (`KismetArrayLibrary.Array_Random` _list_of_montages))
  (`/Engine/EditorBlueprintResources/StandardMacros.IsValid` _outitem
    (:`Is Valid`
      (set `self.Death Montage` _outitem))
    (:`Is Not Valid`
      _))
  (`self.PlayAbilityMontage` (`self.Death Montage`) 1.0 "MontageLength"))

(event `self.EndAbility`)

(fn `CanPerformAbility`
  (returns (ReturnValue :type Boolean))
  (bind _returnvalue (`TempestBaseAbilityManagerComponent.GetCurrentActiveAbility` (`self.Get Tempest Ability Component`)))
  (bind (_attributevalue _minattributevalue) (break `AttributeProperties` (`TempestBaseAttributeObject.AttributeValues` (`TempestAttributesComponents.GetAttributeOfGameplayTag` (`/TempestCombatFramework/Characters/TCF_MasterEnemy_BP.BP_TempestAttributesComponents` (`self.Master Enemy BP`)) (struct :`TagName` "Attribute.Health")))))
  (`/Engine/EditorBlueprintResources/StandardMacros.IsValid` _returnvalue
    (:`Is Valid`
      (return (and (== (`TempestBaseAbilityObject.AbilityGameplayTag` _returnvalue) (struct :`TagName` "Ability.Hit React.Grab")) (<= _attributevalue _minattributevalue))))
    (:`Is Not Valid`
      (return false))))