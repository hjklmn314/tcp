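; Enemy equip ability that plays an equip montage and puts the enemy into combat.
; On start it registers itself as the active ability on the Tempest ability component and picks a random montage from those mapped to its class, assigning it when the validity check passes.
; It plays that montage, then adds the InCombat status through the enemy's combat component.
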(event `self.StartAbility`
  (`TempestBaseAbilityManagerComponent.SetCurrentActiveAbility` (`self.Get Tempest Ability Component`) self)
  (bind _list_of_montages (`self.Get Enemy Ability's Montages` (`GameplayStatics.GetObjectClass` self)))
  (bind _outitem (`KismetArrayLibrary.Array_Random` _list_of_montages))
  (`/Engine/EditorBlueprintResources/StandardMacros.IsValid` _outitem
    (:`Is Valid`
      (set `self.Equip Montage` _outitem))
    (:`Is Not Valid`
      _))
  (`self.PlayAbilityMontage` (`self.Equip Montage`) 1.0 "MontageLength")
  (`TempestCombatComponent.ModifyCombatStatus` (`/TempestCombatFramework/Characters/TCF_MasterEnemy_BP.BP_TempestEnemyCombatComponent` (`self.Master Enemy BP`)) (struct :`TagName` "Status.Combat.InCombat") "Add"))