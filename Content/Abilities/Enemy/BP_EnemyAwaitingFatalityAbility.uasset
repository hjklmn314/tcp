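; An enemy ability Blueprint, named for the state of awaiting a fatality, that plays a randomly chosen montage when it starts.
; StartAbility registers itself as the active ability on the Tempest ability component, then looks up montages by its own class.
; A random valid pick becomes MontageToPlay, which PlayAbilityMontage plays.
; The random pick is read separately for the validity check and the assignment.
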(event `self.StartAbility`
  (`TempestBaseAbilityManagerComponent.SetCurrentActiveAbility` (`self.Get Tempest Ability Component`) self)
  (bind _list_of_montages (`self.Get Enemy Ability's Montages` (`GameplayStatics.GetObjectClass` self)))
  (bind _outitem (`KismetArrayLibrary.Array_Random` _list_of_montages))
  (`/Engine/EditorBlueprintResources/StandardMacros.IsValid` _outitem
    (:`Is Valid`
      (set `self.Montage To Play` _outitem))
    (:`Is Not Valid`
      _))
  (`self.PlayAbilityMontage` (`self.Montage To Play`) 1.0 "MontageLength"))