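; Player heal ability that plays a montage and spends one of a limited number of heal charges.
; It uses HealMontage if set, otherwise picks a random montage registered for the ability's class.
; Activation requires an available montage, an Idle, Walk or Sprint state, in-combat status, an equipped weapon and remaining charges.
; Ending the ability returns the Tempest state manager to Idle; health restoration itself is not handled in this graph.
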(event `self.StartAbility`
  (bind _heal_montage (`self.Heal Montage`))
  (`parent.StartAbility`)
  (`/Engine/EditorBlueprintResources/StandardMacros.IsValid` _heal_montage
    (:`Is Valid`
      (`self.PlayAbilityMontage` _heal_montage))
    (:`Is Not Valid`
      (bind _list_of_montages (`self.Get Ability Montages` (`GameplayStatics.GetObjectClass` self)))
      (`self.PlayAbilityMontage` (`KismetArrayLibrary.Array_Random` _list_of_montages))))
  (`/Engine/EditorBlueprintResources/StandardMacros.DecrementFloat` (`self.Amount Of Heals`)))

(event `self.EndAbility`
  (bind _tempest_state_manager_component (`self.Tempest State Manager Component`))
  (`parent.EndAbility`)
  (`TempestBaseStateManagerComponent.PerformStateOfClass` _tempest_state_manager_component (`GameplayStatics.GetObjectClass` (`TempestBaseStateManagerComponent.GetStateOfGameplayTag` _tempest_state_manager_component (struct :`TagName` "State.Idle")))))

(fn `CanPerformAbility`
  (returns (ReturnValue :type Boolean))
  (bind _bp_tempestplayercombatcomponent (`/TempestCombatFramework/Characters/BP_TCF_DefaultThirdPersonCharacter.BP_TempestPlayerCombatComponent` (`self.Player Character`)))
  (bind _stategameplaytag (`TempestBaseStateObject.StateGameplayTag` (`TempestBaseStateManagerComponent.CurrentActiveState` (`self.Tempest State Manager Component`))))
  (bind _list_of_montages (`self.Get Ability Montages` (`GameplayStatics.GetObjectClass` self)))
  (return (and (or (> (`KismetArrayLibrary.Array_Length` _list_of_montages) 0) (`KismetSystemLibrary.IsValid` (`self.Heal Montage`))) (or (== _stategameplaytag (struct :`TagName` "State.Idle")) (== _stategameplaytag (struct :`TagName` "State.Walk")) (== _stategameplaytag (struct :`TagName` "State.Sprint"))) (`BlueprintGameplayTagLibrary.HasTag` (`TempestCombatComponent.GetCombatStatus` _bp_tempestplayercombatcomponent) (struct :`TagName` "Status.Combat.InCombat")) (`KismetSystemLibrary.IsValid` (`/TempestCombatFramework/Components/BP_TempestPlayerCombatComponent.Get Equipped Weapon` _bp_tempestplayercombatcomponent)) (> (`self.Amount Of Heals`) 0.0))))