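; Player counter-attack ability that can only fire out of a block hit.
; It requires the BlockHit state, an active normal or large block-hit ability, in-combat status, an equipped weapon and at least one montage registered for the class.
; On start it plays the assigned attack montage, falling back to a random one from the class's montage list.
; On end it returns the Tempest state manager to the Idle state.
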(event `self.StartAbility`
  (bind _attack_montage (`self.Attack Montage`))
  (`parent.StartAbility`)
  (`/Engine/EditorBlueprintResources/StandardMacros.IsValid` _attack_montage
    (:`Is Valid`
      (`self.PlayAbilityMontage` _attack_montage))
    (:`Is Not Valid`
      (bind _list_of_montages (`self.Get Ability Montages` (`GameplayStatics.GetObjectClass` self)))
      (`self.PlayAbilityMontage` (`KismetArrayLibrary.Array_Random` _list_of_montages)))))

(event `self.EndAbility`
  (bind _tempest_state_manager_component (`self.Tempest State Manager Component`))
  (`parent.EndAbility`)
  (`TempestBaseStateManagerComponent.PerformStateOfClass` _tempest_state_manager_component (`GameplayStatics.GetObjectClass` (`TempestBaseStateManagerComponent.GetStateOfGameplayTag` _tempest_state_manager_component (struct :`TagName` "State.Idle")))))

(fn `CanPerformAbility`
  (returns (ReturnValue :type Boolean))
  (bind _returnvalue (`TempestBaseStateManagerComponent.GetCurrentActiveState` (`self.Tempest State Manager Component`)))
  (bind _bp_tempestplayercombatcomponent (`/TempestCombatFramework/Characters/BP_TCF_DefaultThirdPersonCharacter.BP_TempestPlayerCombatComponent` (`self.Player Character`)))
  (bind _abilitygameplaytag (`TempestBaseAbilityObject.AbilityGameplayTag` (`TempestBaseAbilityManagerComponent.GetCurrentActiveAbility` (`self.Get Tempest Ability Component`))))
  (`/Engine/EditorBlueprintResources/StandardMacros.IsValid` (`TempestBaseAbilityManagerComponent.GetCurrentActiveAbility` (`self.Get Tempest Ability Component`))
    (:`Is Valid`
      (`/Engine/EditorBlueprintResources/StandardMacros.IsValid` _returnvalue
        (:`Is Valid`
          (bind _list_of_montages (`self.Get Ability Montages` (`GameplayStatics.GetObjectClass` self)))
          (return (and (== (`TempestBaseStateObject.StateGameplayTag` _returnvalue) (struct :`TagName` "State.BlockHit")) (> (`KismetArrayLibrary.Array_Length` _list_of_montages) 0) (`BlueprintGameplayTagLibrary.HasTag` (`TempestCombatComponent.GetCombatStatus` _bp_tempestplayercombatcomponent) (struct :`TagName` "Status.Combat.InCombat")) (`KismetSystemLibrary.IsValid` (`/TempestCombatFramework/Components/BP_TempestPlayerCombatComponent.Get Equipped Weapon` _bp_tempestplayercombatcomponent)) (or (== _abilitygameplaytag (struct :`TagName` "Ability.BlockHit.Normal")) (== _abilitygameplaytag (struct :`TagName` "Ability.BlockHit.Large"))))))
        (:`Is Not Valid`
          _)))
    (:`Is Not Valid`
      _))
  (return false))