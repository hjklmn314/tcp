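; Base class for player abilities in a Tempest-based third-person character setup.
; On construction it warns when no ability gameplay tag is set, then caches the player character, controller and the controller's state manager component.
; Ending the ability clears it from the ability component if currently active.
; A helper looks up an ability's montage list in the equipped weapon's data asset, making animations weapon-specific.
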(event `self.ConstructAbility`
  (`parent.ConstructAbility`)
  (if (not (`BlueprintGameplayTagLibrary.IsGameplayTagValid` (`self.AbilityGameplayTag`)))
    (`KismetSystemLibrary.PrintString` (`KismetStringLibrary.Concat_StrStr` "Developer Notice: You Forgot To Specify Gameplay Tag For Ability " (`KismetSystemLibrary.GetDisplayName` self))))
  (bind _asbp_tcf_default_third_person_character (cast `/TempestCombatFramework/Characters/BP_TCF_DefaultThirdPersonCharacter` (`self.GetPerformingActor`)))
  (bind _output_get (set `self.Player Character` _asbp_tcf_default_third_person_character))
  (bind _returnvalue (`Pawn.GetController` _output_get))
  (bind _asplayer_controller (cast `PlayerController` _returnvalue))
  (set `self.Player Controller` _asplayer_controller)
  (set `self.Tempest State Manager Component` (`Actor.GetComponentByClass` _returnvalue "/Script/TempestCombatFramework.TempestBaseStateManagerComponent")))

(event `self.EndAbility`
  (if (`self.Get Is Current Ability Active`)
    (`TempestBaseAbilityManagerComponent.SetCurrentActiveAbility` (`self.Get Tempest Ability Component`) null)))

(fn `Get Ability Montages`
  (params (`Ability To Look For` :type "/Game/Abilities/Player/BP_BasePlayerAbility Class Reference"))
  (returns (`List Of Montages` :type "Array of AnimMontage Object Reference"))
  (bind _asbp_base_player_weapon (cast `/TempestCombatFramework/Actors/Weapons/Player/BP_BasePlayerWeapon` (`/TempestCombatFramework/Components/BP_TempestPlayerCombatComponent.Get Equipped Weapon` (`/TempestCombatFramework/Characters/BP_TCF_DefaultThirdPersonCharacter.BP_TempestPlayerCombatComponent` (`self.Player Character`))))
    (:`then`
      (for _array_element (`/TempestCombatFramework/DataAssets/BasePlayer_PDA.Abilities` (`/TempestCombatFramework/Actors/Weapons/Player/BP_BasePlayerWeapon.Associated Data Asset` _asbp_base_player_weapon))
        (bind (_ability _listofmontages) (break `/TempestCombatFramework/StructuresEnums/S_AbilityMontages` _array_element))
        (if (== _ability `Ability To Look For`)
          (return _listofmontages))))
    (:`CastFailed`
      _))
  (return))