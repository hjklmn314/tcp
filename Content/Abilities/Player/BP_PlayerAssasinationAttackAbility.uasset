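; Player assassination ability that performs a synced attack on a character directly in front, approached from outside its frontal arc.
; Activation requires a sphere-trace hit, an equipped weapon, in-combat status and an available Assassinated state on the target's controller.
; On start it plays an assigned or random montage, triggers that state, disables lock-on and creates a syncing object.
; The syncing object updates each tick, and ending returns the player to Idle.
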(event `self.StartAbility`
  (bind _assasination_montage (`self.Assasination Montage`))
  (`parent.StartAbility`)
  (`/Engine/EditorBlueprintResources/StandardMacros.IsValid` _assasination_montage
    (:`Is Valid`
      (`self.PlayAbilityMontage` _assasination_montage))
    (:`Is Not Valid`
      (bind _list_of_montages (`self.Get Ability Montages` (`GameplayStatics.GetObjectClass` self)))
      (`self.PlayAbilityMontage` (`KismetArrayLibrary.Array_Random` _list_of_montages))))
  (bind _ascharacter (cast `Character` (`self.Hit Actor`)))
  (bind _returnvalue (`Actor.GetComponentByClass` (`Pawn.GetController` _ascharacter) "/Script/TempestCombatFramework.TempestBaseStateManagerComponent"))
  (`TempestBaseStateManagerComponent.PerformStateOfClass` _returnvalue (`GameplayStatics.GetObjectClass` (`TempestBaseStateManagerComponent.GetStateOfGameplayTag` _returnvalue (struct :`TagName` "State.Assasinated"))))
  (bind _returnvalue_2 (`|GenericCreateObject` (`self.Player Character`) "/TempestCombatFramework/Animation/Objects/BP_AssasinationSyncingObject.BP_AssasinationSyncingObject_C" (`self.Hit Actor`) 100.0))
  (bind _output_get (set `self.Syncing Object` _returnvalue_2))
  (`/TempestCombatFramework/Animation/Objects/BP_BaseSyncObject.Construct Syncing Object` _output_get)
  (`TempestTargetingComponent.DisableLockOn` (`/TempestCombatFramework/Characters/BP_TCF_DefaultThirdPersonCharacter.BP_TempestTargetingComponent` (`self.Player Character`))))

(event `self.EndAbility`
  (bind _tempest_state_manager_component (`self.Tempest State Manager Component`))
  (`parent.EndAbility`)
  (`TempestBaseStateManagerComponent.PerformStateOfClass` _tempest_state_manager_component (`GameplayStatics.GetObjectClass` (`TempestBaseStateManagerComponent.GetStateOfGameplayTag` _tempest_state_manager_component (struct :`TagName` "State.Idle")))))

(event `self.TickAbility`
  (params (TickTime :type "Float (single-precision)"))
  (bind _syncing_object (`self.Syncing Object`))
  (`/Engine/EditorBlueprintResources/StandardMacros.IsValid` _syncing_object
    (:`Is Valid`
      (`/TempestCombatFramework/Animation/Objects/BP_BaseSyncObject.Tick Syncing Object` _syncing_object))))

(fn `CanPerformAbility`
  (returns (ReturnValue :type Boolean))
  (bind _player_character (`self.Player Character`))
  (bind _returnvalue (`Actor.K2_GetActorLocation` _player_character))
  (bind _bp_tempestplayercombatcomponent (`/TempestCombatFramework/Characters/BP_TCF_DefaultThirdPersonCharacter.BP_TempestPlayerCombatComponent` (`self.Player Character`)))
  (bind (_outhit _returnvalue_2) (`KismetSystemLibrary.SphereTraceSingle` _returnvalue (+ _returnvalue (* (`Actor.GetActorForwardVector` _player_character) 150.0)) 35.0 "TraceTypeQuery3" false (`|MakeArray` _player_character :!type "Actor Object Reference")))
  (if _returnvalue_2
    (bind _output_get (set `self.Hit Actor` (`.HitActor` (`GameplayStatics.BreakHitResult` _outhit))))
    (bind _ascharacter (cast `Character` (`self.Hit Actor`))
      (:`then`
        (bind (_return_value_y__pitch_ _return_value_z__yaw_) (`/TempestCombatFramework/Libraries/BFL_TempestGeneralFunctions.Calculate Angle Between Actors` _output_get (`self.Player Character`)))
        (bind _returnvalue_3 (`TempestBaseStateManagerComponent.GetStateOfGameplayTag` (`Actor.GetComponentByClass` (`Pawn.GetController` _ascharacter) "/Script/TempestCombatFramework.TempestBaseStateManagerComponent") (struct :`TagName` "State.Assasinated")))
        (`/Engine/EditorBlueprintResources/StandardMacros.IsValid` _returnvalue_3
          (:`Is Valid`
            (return (and (not (`KismetMathLibrary.InRange_FloatFloat` (`KismetMathLibrary.Abs` _return_value_z__yaw_) 0.0 120.0)) (`KismetSystemLibrary.IsValid` (`/TempestCombatFramework/Components/BP_TempestPlayerCombatComponent.Get Equipped Weapon` _bp_tempestplayercombatcomponent)) (`BlueprintGameplayTagLibrary.HasTag` (`TempestCombatComponent.GetCombatStatus` _bp_tempestplayercombatcomponent) (struct :`TagName` "Status.Combat.InCombat")) (`TempestBaseStateObject.CanPerformState` _returnvalue_3))))
          (:`Is Not Valid`
            _)))
      (:`CastFailed`
        _))
    (return false)))