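; Player riposte attack ability that executes a synced riposte on a character directly in front of the player.
; It is allowed only when a forward sphere trace finds a target able to enter Riposted and the player is armed, in combat and idle, walking or sprinting.
; On start it plays an attack montage, forces the target into Riposted and creates a syncing object, ticked with the ability.
; Ending returns the player to Idle.
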(event `self.StartAbility`
  (bind _attack_montage (`self.Attack Montage`))
  (`parent.StartAbility`)
  (`/Engine/EditorBlueprintResources/StandardMacros.IsValid` _attack_montage
    (:`Is Valid`
      (`self.PlayAbilityMontage` _attack_montage))
    (:`Is Not Valid`
      (bind _list_of_montages (`self.Get Ability Montages` (`GameplayStatics.GetObjectClass` self)))
      (`self.PlayAbilityMontage` (`KismetArrayLibrary.Array_Random` _list_of_montages))))
  (bind _ascharacter (cast `Character` (`self.Hit Actor`)))
  (bind _returnvalue (`Actor.GetComponentByClass` (`Pawn.GetController` _ascharacter) "/Script/TempestCombatFramework.TempestBaseStateManagerComponent"))
  (`TempestBaseStateManagerComponent.PerformStateOfClass` _returnvalue (`GameplayStatics.GetObjectClass` (`TempestBaseStateManagerComponent.GetStateOfGameplayTag` _returnvalue (struct :`TagName` "State.Riposted"))))
  (bind _returnvalue_2 (`|GenericCreateObject` (`self.Player Character`) "/TempestCombatFramework/Animation/Objects/BP_RiposteSyncingObject.BP_RiposteSyncingObject_C" (`self.Hit Actor`)))
  (bind _output_get (set `self.Riposte Syncing Object` _returnvalue_2))
  (`/TempestCombatFramework/Animation/Objects/BP_BaseSyncObject.Construct Syncing Object` _output_get))

(event `self.TickAbility`
  (params (TickTime :type "Float (single-precision)"))
  (bind _riposte_syncing_object (`self.Riposte Syncing Object`))
  (`/Engine/EditorBlueprintResources/StandardMacros.IsValid` _riposte_syncing_object
    (:`Is Valid`
      (`/TempestCombatFramework/Animation/Objects/BP_BaseSyncObject.Tick Syncing Object` _riposte_syncing_object))))

(event `self.EndAbility`
  (bind _tempest_state_manager_component (`self.Tempest State Manager Component`))
  (`parent.EndAbility`)
  (`TempestBaseStateManagerComponent.PerformStateOfClass` _tempest_state_manager_component (`GameplayStatics.GetObjectClass` (`TempestBaseStateManagerComponent.GetStateOfGameplayTag` _tempest_state_manager_component (struct :`TagName` "State.Idle")))))

(fn `CanPerformAbility`
  (returns (ReturnValue :type Boolean))
  (bind _player_character (`self.Player Character`))
  (bind _returnvalue (`Actor.K2_GetActorLocation` _player_character))
  (bind _bp_tempestplayercombatcomponent (`/TempestCombatFramework/Characters/BP_TCF_DefaultThirdPersonCharacter.BP_TempestPlayerCombatComponent` (`self.Player Character`)))
  (bind _stategameplaytag (`TempestBaseStateObject.StateGameplayTag` (`TempestBaseStateManagerComponent.CurrentActiveState` (`self.Tempest State Manager Component`))))
  (bind (_outhit _returnvalue_2) (`KismetSystemLibrary.SphereTraceSingle` _returnvalue (+ _returnvalue (* (`Actor.GetActorForwardVector` _player_character) 150.0)) 35.0 "TraceTypeQuery3" false (`|MakeArray` _player_character :!type "Actor Object Reference")))
  (if _returnvalue_2
    (bind _output_get (set `self.Hit Actor` (`.HitActor` (`GameplayStatics.BreakHitResult` _outhit))))
    (bind _ascharacter (cast `Character` _output_get))
    (bind _returnvalue_3 (`Actor.GetComponentByClass` (`Pawn.GetController` _ascharacter) "/Script/TempestCombatFramework.TempestBaseStateManagerComponent"))
    (`/Engine/EditorBlueprintResources/StandardMacros.IsValid` _returnvalue_3
      (:`Is Valid`
        (if (`TempestBaseStateManagerComponent.GetCanPerformStateOfClass` _returnvalue_3 (`GameplayStatics.GetObjectClass` (`TempestBaseStateManagerComponent.GetStateOfGameplayTag` _returnvalue_3 (struct :`TagName` "State.Riposted"))))
          (bind _list_of_montages (`self.Get Ability Montages` (`GameplayStatics.GetObjectClass` self)))
          (return (and (or (> (`KismetArrayLibrary.Array_Length` _list_of_montages) 0) (`KismetSystemLibrary.IsValid` (`self.Attack Montage`))) (or (== _stategameplaytag (struct :`TagName` "State.Idle")) (== _stategameplaytag (struct :`TagName` "State.Walk")) (== _stategameplaytag (struct :`TagName` "State.Sprint"))) (`BlueprintGameplayTagLibrary.HasTag` (`TempestCombatComponent.GetCombatStatus` _bp_tempestplayercombatcomponent) (struct :`TagName` "Status.Combat.InCombat")) (`KismetSystemLibrary.IsValid` (`/TempestCombatFramework/Components/BP_TempestPlayerCombatComponent.Get Equipped Weapon` _bp_tempestplayercombatcomponent))))
          (else
            _)))
      (:`Is Not Valid`
        _)))
  (return false))