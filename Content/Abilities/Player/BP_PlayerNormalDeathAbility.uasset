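; BP_PlayerNormalDeathAbility is a player ability that plays a death animation montage.
; On start it plays DeathMontage when that is valid, otherwise a random montage from those returned by GetAbilityMontages for its class.
; CanPerformAbility allows it only when one of these montage sources is available.
; Start and end events both call their parent implementations.
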(event `self.StartAbility`
  (bind _death_montage (`self.Death Montage`))
  (`parent.StartAbility`)
  (`/Engine/EditorBlueprintResources/StandardMacros.IsValid` _death_montage
    (:`Is Valid`
      (`self.PlayAbilityMontage` _death_montage))
    (:`Is Not Valid`
      (bind _list_of_montages (`self.Get Ability Montages` (`GameplayStatics.GetObjectClass` self)))
      (`self.PlayAbilityMontage` (`KismetArrayLibrary.Array_Random` _list_of_montages)))))

(event `self.EndAbility`
  (`parent.EndAbility`))

(fn `CanPerformAbility`
  (returns (ReturnValue :type Boolean))
  (bind _list_of_montages (`self.Get Ability Montages` (`GameplayStatics.GetObjectClass` self)))
  (return (or (> (`KismetArrayLibrary.Array_Length` _list_of_montages) 0) (`KismetSystemLibrary.IsValid` (`self.Death Montage`)))))