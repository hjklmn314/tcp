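; Player perfect dodge ability that plays a directional dodge montage based on movement input.
; CalculateDodgeAngle measures input yaw relative to the character, defaulting to zero, and StartAbility maps it to one of four montages.
; EndAbility returns the state manager to Idle.
; CanPerformAbility always returns true; its disconnected logic checks combat status, equipped weapon and nearby characters' active weapon trace sockets.
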(event `self.StartAbility`
  (`parent.StartAbility`)
  (bind _list_of_montages (`self.Get Ability Montages` (`GameplayStatics.GetObjectClass` self)))
  (set `self.Dodge Montages` _list_of_montages)
  (bind _return_value (`self.Calculate Dodge Angle`))
  (if (`KismetMathLibrary.InRange_FloatFloat` _return_value -45.0 50.0)
    (`self.PlayAbilityMontage` (`|GetArrayItem` (`self.Dodge Montages`)))
    (elif (`KismetMathLibrary.InRange_FloatFloat` _return_value 45.0 135.0)
      (`self.PlayAbilityMontage` (`|GetArrayItem` (`self.Dodge Montages`) 1))
      (elif (`KismetMathLibrary.InRange_FloatFloat` _return_value -135.0 -45.0)
        (`self.PlayAbilityMontage` (`|GetArrayItem` (`self.Dodge Montages`) 2))
        (else
          (`self.PlayAbilityMontage` (`|GetArrayItem` (`self.Dodge Montages`) 3)))))))

(event `self.EndAbility`
  (bind _tempest_state_manager_component (`self.Tempest State Manager Component`))
  (`parent.EndAbility`)
  (`TempestBaseStateManagerComponent.PerformStateOfClass` _tempest_state_manager_component (`GameplayStatics.GetObjectClass` (`TempestBaseStateManagerComponent.GetStateOfGameplayTag` _tempest_state_manager_component (struct :`TagName` "State.Idle")))))

(fn `Calculate Dodge Angle`
  (returns (`Return Value` :type "Float (double-precision)"))
  (bind _player_character (`self.Player Character`))
  (bind _return_value (message `/TempestCombatFramework/Interfaces/BPI_PlayerInputs.Get Direction From Movement Inputs` (`Pawn.GetController` _player_character)))
  (if (!= _return_value (0.0 0.0 0.0))
    (return (.yaw (`KismetMathLibrary.NormalizedDeltaRotator` (`KismetMathLibrary.Conv_VectorToRotator` (`KismetMathLibrary.Conv_RotatorToVector` (`KismetMathLibrary.Conv_VectorToRotator` _return_value))) (`Actor.K2_GetActorRotation` _player_character))))
    (else
      (return 0.0))))

(fn `CanPerformAbility`
  (returns (ReturnValue :type Boolean))
  (return true))