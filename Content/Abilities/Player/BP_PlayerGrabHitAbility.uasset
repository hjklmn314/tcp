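; Player ability that plays the victim side of an incoming grab attack, gated by attack tag, cooldown, invincibility and an equipped weapon.
; It async-loads the montage matching the player's gameplay tags from the grab property, while pushing the attacker's controller into its Grab state.
; Once loaded, it drops lock-on, plays the grab section with shake, impact effects and brief hit-stop on both actors.
; Camera lag speed changes during the grab; ending restores it and returns to Idle.
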(event `self.StartAbility`
  (bind _player_character (`self.Player Character`))
  (bind _returnvalue (`TempestAttackPropertiesObject.GetAttackPropertyOwner` (`TempestCombatComponent.ReceivedAttackProperty` (`/TempestCombatFramework/Characters/BP_TCF_DefaultThirdPersonCharacter.BP_TempestPlayerCombatComponent` _player_character))))
  (`parent.StartAbility`)
  (bind _target_anim_montages (`self.Find Associated Anim Montage`))
  (bind _object (`|LoadAsset` _target_anim_montages)
    (:`then`
      (bind _ascharacter (cast `Character` (`TempestAttackPropertiesObject.GetAttackPropertyOwner` (`TempestCombatComponent.ReceivedAttackProperty` (`/TempestCombatFramework/Characters/BP_TCF_DefaultThirdPersonCharacter.BP_TempestPlayerCombatComponent` (`self.Player Character`))))))
      (bind _returnvalue_2 (`Actor.GetComponentByClass` (`Pawn.GetController` _ascharacter) "/Script/TempestCombatFramework.TempestBaseStateManagerComponent"))
      (`TempestBaseStateManagerComponent.TryPerformStateOfClass` _returnvalue_2 (`GameplayStatics.GetObjectClass` (`TempestBaseStateManagerComponent.GetStateOfGameplayTag` _returnvalue_2 (struct :`TagName` "State.Grab"))) true))
    (:`Completed`
      (bind _asanim_montage (cast `AnimMontage` _object))
      (`TempestTargetingComponent.DisableLockOn` (`/TempestCombatFramework/Characters/BP_TCF_DefaultThirdPersonCharacter.BP_TempestTargetingComponent` (`self.Player Character`)))
      (`self.PlayAbilityMontage` _asanim_montage 1.0 "MontageLength" 0.0 "GrabSection")
      (`PlayerCameraManager.StartCameraShake` :`self` (`GameplayStatics.GetPlayerCameraManager` 0) :`ShakeClass` "/Game/TempestCombatFramework/Camera/CameraShake/BP_NormalHitCameraShake.BP_NormalHitCameraShake_C")
      (bind _asbp_base_defense_property (cast `/TempestCombatFramework/DefenseProperties/BP_BaseDefenseProperty` (`TempestCombatComponent.OwnerDefenseProperty` (`/TempestCombatFramework/Characters/BP_TCF_DefaultThirdPersonCharacter.BP_TempestPlayerCombatComponent` (`self.Player Character`)))))
      (`/TempestCombatFramework/DefenseProperties/BP_BaseDefenseProperty.Apply Hit Effect Of Class` _asbp_base_defense_property "/TempestCombatFramework/ImpactEffects/BP_NormalImpactEffects.BP_NormalImpactEffects_C")
      (set `SpringArmComponent.CameraLagSpeed` 10.0 (`/TempestCombatFramework/Characters/BP_TCF_DefaultThirdPersonCharacter.CameraBoom` (`self.Player Character`)))
      (`KismetSystemLibrary.Delay` 0.05)
      (bind _output_get (set `Actor.CustomTimeDilation` 0.05 _returnvalue))
      (set `Actor.CustomTimeDilation` _output_get _player_character)
      (`KismetSystemLibrary.Delay` 0.1)
      (bind _output_get_2 (set `Actor.CustomTimeDilation` 1.0 _returnvalue))
      (set `Actor.CustomTimeDilation` _output_get_2 _player_character))))

(event `self.EndAbility`
  (bind _tempest_state_manager_component (`self.Tempest State Manager Component`))
  (`parent.EndAbility`)
  (`TempestBaseStateManagerComponent.PerformStateOfClass` _tempest_state_manager_component (`GameplayStatics.GetObjectClass` (`TempestBaseStateManagerComponent.GetStateOfGameplayTag` _tempest_state_manager_component (struct :`TagName` "State.Idle"))))
  (set `SpringArmComponent.CameraLagSpeed` 5.0 (`/TempestCombatFramework/Characters/BP_TCF_DefaultThirdPersonCharacter.CameraBoom` (`self.Player Character`))))

(fn `CanPerformAbility`
  (returns (ReturnValue :type Boolean))
  (bind _bp_tempestplayercombatcomponent (`/TempestCombatFramework/Characters/BP_TCF_DefaultThirdPersonCharacter.BP_TempestPlayerCombatComponent` (`self.Player Character`)))
  (if (not (`BlueprintGameplayTagLibrary.HasTag` (`TempestCombatComponent.GetCombatStatus` _bp_tempestplayercombatcomponent) (struct :`TagName` "Status.Combat.Invincible")))
    (bind _asbp_base_attack_properties (cast `/TempestCombatFramework/AttackProperties/BP_BaseAttackProperties` (`TempestCombatComponent.ReceivedAttackProperty` _bp_tempestplayercombatcomponent)))
    (return (and (== (`/TempestCombatFramework/AttackProperties/BP_BaseAttackProperties.Attack Property Tag` _asbp_base_attack_properties) (struct :`TagName` "Property.Attack.Grab")) (not (`self.GetIsAbilityOnCooldown`)) (`KismetSystemLibrary.IsValid` (`/TempestCombatFramework/Components/BP_TempestPlayerCombatComponent.Get Equipped Weapon` (`/TempestCombatFramework/Characters/BP_TCF_DefaultThirdPersonCharacter.BP_TempestPlayerCombatComponent` (`self.Player Character`))))))
    (else
      (return false))))

(fn `Find Associated Anim Montage`
  (returns (`Target Anim Montages` :type "AnimMontage Soft Object Reference"))
  (bind _asbp_grab_attack_property (cast `/TempestCombatFramework/AttackProperties/BP_GrabAttackProperty` (`TempestCombatComponent.ReceivedAttackProperty` (`/TempestCombatFramework/Characters/BP_TCF_DefaultThirdPersonCharacter.BP_TempestPlayerCombatComponent` (`self.Player Character`)))))
  (for (_array_element _array_index) (`/TempestCombatFramework/AttackProperties/BP_GrabAttackProperty.Grab Anim Montages` _asbp_grab_attack_property)
    (bind (_hittargettag _targetanimmontages) (break `/TempestCombatFramework/StructuresEnums/S_GrabProperties` _array_element))
    (if (`BlueprintGameplayTagLibrary.HasTag` (`TempestBaseCharacter.ActorGameplayTags` (`self.Player Character`)) _hittargettag)
      (`/TempestCombatFramework/AttackProperties/BP_GrabAttackProperty.Set Found Index` _asbp_grab_attack_property _array_index)
      (return _targetanimmontages))))