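; Player ability that plays a get-up montage and can always be performed.
; On start it plays GetUpMontage if valid, otherwise a random montage from those returned for its own class.
; On end it switches the state manager to the State.Idle state and sets the player camera boom's lag speed to a fixed value.
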(event `self.StartAbility`
  (bind _get_up_montage (`self.Get Up Montage`))
  (`parent.StartAbility`)
  (`/Engine/EditorBlueprintResources/StandardMacros.IsValid` _get_up_montage
    (:`Is Valid`
      (`self.PlayAbilityMontage` _get_up_montage))
    (:`Is Not Valid`
      (bind _list_of_montages (`self.Get Ability Montages` (`GameplayStatics.GetObjectClass` self)))
      (`self.PlayAbilityMontage` (`KismetArrayLibrary.Array_Random` _list_of_montages)))))

(event `self.EndAbility`
  (bind _tempest_state_manager_component (`self.Tempest State Manager Component`))
  (`parent.EndAbility`)
  (`TempestBaseStateManagerComponent.PerformStateOfClass` _tempest_state_manager_component (`GameplayStatics.GetObjectClass` (`TempestBaseStateManagerComponent.GetStateOfGameplayTag` _tempest_state_manager_component (struct :`TagName` "State.Idle"))))
  (set `SpringArmComponent.CameraLagSpeed` 5.0 (`/TempestCombatFramework/Characters/BP_TCF_DefaultThirdPersonCharacter.CameraBoom` (`self.Player Character`))))

(fn `CanPerformAbility`
  (returns (ReturnValue :type Boolean))
  (return true))