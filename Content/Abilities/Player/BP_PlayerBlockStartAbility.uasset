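; Player ability that begins a block, available only while the combat component reports in-combat status and has a valid equipped weapon.
; On start it plays BlockStartMontage, falling back to a random montage registered for the ability class.
; With no valid montage, it tries to perform BP_PlayerBlockLoopAbility directly.
; On end it stops the character's montage and switches the Tempest state manager to the Idle state.
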(event `self.StartAbility`
  (bind _block_start_montage (`self.Block Start Montage`))
  (`parent.StartAbility`)
  (`/Engine/EditorBlueprintResources/StandardMacros.IsValid` _block_start_montage
    (:`Is Valid`
      (`self.PlayAbilityMontage` _block_start_montage))
    (:`Is Not Valid`
      (bind _list_of_montages (`self.Get Ability Montages` (`GameplayStatics.GetObjectClass` self)))
      (bind _outitem (`KismetArrayLibrary.Array_Random` _list_of_montages))
      (`/Engine/EditorBlueprintResources/StandardMacros.IsValid` _outitem
        (:`Is Valid`
          (`self.PlayAbilityMontage` _outitem))
        (:`Is Not Valid`
          (`TempestBaseAbilityManagerComponent.TryPerformAbilityOfClass` (`self.Get Tempest Ability Component`) "/TempestCombatFramework/Abilities/Player/BP_PlayerBlockLoopAbility.BP_PlayerBlockLoopAbility_C" true))))))

(event `self.EndAbility`
  (bind _tempest_state_manager_component (`self.Tempest State Manager Component`))
  (`parent.EndAbility`)
  (`Character.StopAnimMontage` (`self.Player Character`) null)
  (`TempestBaseStateManagerComponent.PerformStateOfClass` _tempest_state_manager_component (`GameplayStatics.GetObjectClass` (`TempestBaseStateManagerComponent.GetStateOfGameplayTag` _tempest_state_manager_component (struct :`TagName` "State.Idle")))))

(fn `CanPerformAbility`
  (returns (ReturnValue :type Boolean))
  (bind _returnvalue (`Actor.GetComponentByClass` (`self.Player Character`) "/TempestCombatFramework/Components/BP_TempestBaseCombatComponent.BP_TempestBaseCombatComponent_C"))
  (return (and (`BlueprintGameplayTagLibrary.HasTag` (`TempestCombatComponent.GetCombatStatus` _returnvalue) (struct :`TagName` "Status.Combat.InCombat")) (`KismetSystemLibrary.IsValid` (`/TempestCombatFramework/Components/BP_TempestPlayerCombatComponent.Get Equipped Weapon` _returnvalue)))))