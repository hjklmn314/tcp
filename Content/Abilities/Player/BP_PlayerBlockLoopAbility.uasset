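; Player ability for the looping block, available while the player is in combat with a weapon equipped and the right mouse input is clicked.
; On start it sends a moveset message to the character mesh's anim instance to switch its animation.
; On end it has the Tempest state manager perform the state tagged State.Idle.
; The condition check reads combat status tags from the combat component and input from the controller's mapping context.
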(event `self.StartAbility`
  (`parent.StartAbility`)
  (message `/TempestCombatFramework/Interfaces/BPI_GeneralInterface.Assign Moveset` (`SkeletalMeshComponent.GetAnimInstance` (`Character.Mesh` (`self.Player Character`))) "NewEnumerator3"))

(event `self.EndAbility`
  (bind _tempest_state_manager_component (`self.Tempest State Manager Component`))
  (`parent.EndAbility`)
  (`TempestBaseStateManagerComponent.PerformStateOfClass` _tempest_state_manager_component (`GameplayStatics.GetObjectClass` (`TempestBaseStateManagerComponent.GetStateOfGameplayTag` _tempest_state_manager_component (struct :`TagName` "State.Idle")))))

(fn `CanPerformAbility`
  (returns (ReturnValue :type Boolean))
  (bind _returnvalue (`Actor.GetComponentByClass` (`self.Player Character`) "/TempestCombatFramework/Components/BP_TempestBaseCombatComponent.BP_TempestBaseCombatComponent_C"))
  (bind _mapping_context (message `/TempestCombatFramework/Interfaces/BPI_PlayerInputs.Get Mapping Context` (`Pawn.GetController` (`self.Player Character`))))
  (return (and (`BlueprintGameplayTagLibrary.HasTag` (`TempestCombatComponent.GetCombatStatus` _returnvalue) (struct :`TagName` "Status.Combat.InCombat")) (`KismetSystemLibrary.IsValid` (`/TempestCombatFramework/Components/BP_TempestPlayerCombatComponent.Get Equipped Weapon` _returnvalue)) (`/TempestCombatFramework/Libraries/BFL_TempestInputs.Get Is Input Clicked` _mapping_context "/TempestCombatFramework/Input/RightMouse_Input.RightMouse_Input" (`self.Player Controller`)))))