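; Player ability that plays the death that follows being riposted, built on the Tempest ability and state framework.
; It can perform only while the active ability is tagged Riposted and the player's Health attribute is at or below its minimum.
; On start it switches the state manager to the Death state, then plays the DeathMontage, or a random montage from the ability's list if none is set.
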(event `self.StartAbility`
  (bind _death_montage (`self.Death Montage`))
  (bind _tempest_state_manager_component (`self.Tempest State Manager Component`))
  (`parent.StartAbility`)
  (`TempestBaseStateManagerComponent.PerformStateOfClass` _tempest_state_manager_component (`GameplayStatics.GetObjectClass` (`TempestBaseStateManagerComponent.GetStateOfGameplayTag` _tempest_state_manager_component (struct :`TagName` "State.Death"))))
  (`/Engine/EditorBlueprintResources/StandardMacros.IsValid` _death_montage
    (:`Is Valid`
      (`self.PlayAbilityMontage` _death_montage))
    (:`Is Not Valid`
      (bind _list_of_montages (`self.Get Ability Montages` (`GameplayStatics.GetObjectClass` self)))
      (`self.PlayAbilityMontage` (`KismetArrayLibrary.Array_Random` _list_of_montages)))))

(event `self.EndAbility`
  (`parent.EndAbility`))

(fn `CanPerformAbility`
  (returns (ReturnValue :type Boolean))
  (bind _returnvalue (`TempestBaseAbilityManagerComponent.GetCurrentActiveAbility` (`self.Get Tempest Ability Component`)))
  (bind (_attributevalue _minattributevalue) (break `AttributeProperties` (`TempestBaseAttributeObject.AttributeValues` (`TempestAttributesComponents.GetAttributeOfGameplayTag` (`/TempestCombatFramework/Characters/BP_TCF_DefaultThirdPersonCharacter.BP_TempestAttributesComponents` (`self.Player Character`)) (struct :`TagName` "Attribute.Health")))))
  (`/Engine/EditorBlueprintResources/StandardMacros.IsValid` _returnvalue
    (:`Is Valid`
      (return (and (== (`TempestBaseAbilityObject.AbilityGameplayTag` _returnvalue) (struct :`TagName` "Ability.Riposted")) (<= _attributevalue _minattributevalue))))
    (:`Is Not Valid`
      (return false))))