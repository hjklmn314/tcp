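; Player ability that plays a hit reaction when struck by normal, thrust, gunshot or normal-knock attacks, gated on not being invincible, cooldown and an equipped weapon.
; It picks a montage from the attacker's front/back position and swing direction, mirroring left/right from behind and using a default for other property classes.
; It then applies impact effects, camera shake and a brief time-dilation hit-stop on both characters.
; Ending the ability returns to Idle state.
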(event `self.StartAbility`
  (bind _player_character (`self.Player Character`))
  (bind _player_character_2 (`self.Player Character`))
  (bind _returnvalue (`TempestAttackPropertiesObject.GetAttackPropertyOwner` (`TempestCombatComponent.ReceivedAttackProperty` (`/TempestCombatFramework/Characters/BP_TCF_DefaultThirdPersonCharacter.BP_TempestPlayerCombatComponent` _player_character))))
  (`parent.StartAbility`)
  (bind _list_of_montages (`self.Get Ability Montages` (`GameplayStatics.GetObjectClass` self)))
  (set `self.Hit Reaction Montages` _list_of_montages)
  (bind _asbp_normal_attack_property (cast `/TempestCombatFramework/AttackProperties/BP_NormalAttackProperty` (`TempestCombatComponent.ReceivedAttackProperty` (`Actor.GetComponentByClass` _player_character_2 "/Script/TempestCombatFramework.TempestCombatComponent")))
    (:`then`
      (bind _output_get (set `self.Normal Attack Property` _asbp_normal_attack_property))
      (bind (_return_value_y__pitch_ _return_value_z__yaw_) (`/TempestCombatFramework/Libraries/BFL_TempestGeneralFunctions.Calculate Angle Between Actors` _player_character_2 (`TempestAttackPropertiesObject.GetAttackPropertyOwner` _output_get)))
      (set `self.Direction` (select `bool` (`KismetMathLibrary.InRange_FloatFloat` _return_value_z__yaw_ -90.0 90.0) :`false` "NewEnumerator9" :`true` "NewEnumerator8" :!type "/TempestCombatFramework/StructuresEnums/E_4DDirection Enum"))
      (switch `/TempestCombatFramework/StructuresEnums/E_4DDirection` (`self.Direction`)
        (:`NewEnumerator3`
          (switch `/TempestCombatFramework/StructuresEnums/E_SwingDirection` (`/TempestCombatFramework/AttackProperties/BP_NormalAttackProperty.Swing Direction` (`self.Normal Attack Property`)) :!label _label
            (:`NewEnumerator3`
              (`self.PlayAbilityMontage` (`|GetArrayItem` (`self.Hit Reaction Montages`) 1) 1.0 "MontageLength" :!label _label_2))
            (:`NewEnumerator5`
              (`self.PlayAbilityMontage` (`|GetArrayItem` (`self.Hit Reaction Montages`) 2) 1.0 "MontageLength" :!label _label_3))
            (:`NewEnumerator8`
              (`self.PlayAbilityMontage` (`|GetArrayItem` (`self.Hit Reaction Montages`)) 1.0 "MontageLength" :!label _label_4))
            (:`NewEnumerator9`
              (goto _label_4))))
        (:`NewEnumerator5`
          (goto _label))
        (:`NewEnumerator8`
          (goto _label))
        (:`NewEnumerator9`
          (switch `/TempestCombatFramework/StructuresEnums/E_SwingDirection` (`/TempestCombatFramework/AttackProperties/BP_NormalAttackProperty.Swing Direction` (`self.Normal Attack Property`))
            (:`NewEnumerator3`
              (goto _label_3))
            (:`NewEnumerator5`
              (goto _label_2))
            (:`NewEnumerator8`
              _)
            (:`NewEnumerator9`
              _))
          (`self.PlayAbilityMontage` (`|GetArrayItem` (`self.Hit Reaction Montages`) 3) 1.0 "MontageLength"))))
    (:`CastFailed`
      (goto _label_4)))
  (bind _asbp_base_defense_property (cast `/TempestCombatFramework/DefenseProperties/BP_BaseDefenseProperty` (`TempestCombatComponent.OwnerDefenseProperty` (`/TempestCombatFramework/Characters/BP_TCF_DefaultThirdPersonCharacter.BP_TempestPlayerCombatComponent` (`self.Player Character`)))))
  (`/TempestCombatFramework/DefenseProperties/BP_BaseDefenseProperty.Apply Hit Effect Of Class` _asbp_base_defense_property "/TempestCombatFramework/ImpactEffects/BP_NormalImpactEffects.BP_NormalImpactEffects_C")
  (`PlayerCameraManager.StartCameraShake` :`self` (`GameplayStatics.GetPlayerCameraManager` 0) :`ShakeClass` "/Game/TempestCombatFramework/Camera/CameraShake/BP_NormalHitCameraShake.BP_NormalHitCameraShake_C")
  (`KismetSystemLibrary.Delay` 0.05)
  (bind _output_get_2 (set `Actor.CustomTimeDilation` 0.1 _returnvalue))
  (set `Actor.CustomTimeDilation` _output_get_2 _player_character)
  (`KismetSystemLibrary.Delay` 0.05)
  (bind _output_get_3 (set `Actor.CustomTimeDilation` 1.0 _returnvalue))
  (set `Actor.CustomTimeDilation` _output_get_3 _player_character))

(event `self.EndAbility`
  (bind _tempest_state_manager_component (`self.Tempest State Manager Component`))
  (`parent.EndAbility`)
  (`TempestBaseStateManagerComponent.PerformStateOfClass` _tempest_state_manager_component (`GameplayStatics.GetObjectClass` (`TempestBaseStateManagerComponent.GetStateOfGameplayTag` _tempest_state_manager_component (struct :`TagName` "State.Idle")))))

(fn `CanPerformAbility`
  (returns (ReturnValue :type Boolean))
  (bind _bp_tempestplayercombatcomponent (`/TempestCombatFramework/Characters/BP_TCF_DefaultThirdPersonCharacter.BP_TempestPlayerCombatComponent` (`self.Player Character`)))
  (if (not (`BlueprintGameplayTagLibrary.HasTag` (`TempestCombatComponent.GetCombatStatus` _bp_tempestplayercombatcomponent) (struct :`TagName` "Status.Combat.Invincible")))
    (bind _asbp_base_attack_properties (cast `/TempestCombatFramework/AttackProperties/BP_BaseAttackProperties` (`TempestCombatComponent.ReceivedAttackProperty` _bp_tempestplayercombatcomponent)))
    (bind _attack_property_tag (`/TempestCombatFramework/AttackProperties/BP_BaseAttackProperties.Attack Property Tag` _asbp_base_attack_properties))
    (return (and (or (== _attack_property_tag (struct :`TagName` "Property.Attack.Normal")) (== _attack_property_tag (struct :`TagName` "Property.Attack.Thrust")) (== _attack_property_tag (struct :`TagName` "Property.Attack.Projectile.GunShot")) (== _attack_property_tag (struct :`TagName` "Property.Attack.Normal & Knock"))) (not (`self.GetIsAbilityOnCooldown`)) (`KismetSystemLibrary.IsValid` (`/TempestCombatFramework/Components/BP_TempestPlayerCombatComponent.Get Equipped Weapon` (`/TempestCombatFramework/Characters/BP_TCF_DefaultThirdPersonCharacter.BP_TempestPlayerCombatComponent` (`self.Player Character`))))))
    (else
      (return false))))