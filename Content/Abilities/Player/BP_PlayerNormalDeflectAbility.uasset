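; Player deflect ability: a timed parry that is allowed only early in a block against an attack from the front.
; CanPerformAbility requires combat status, an equipped weapon, the attacker within a frontal arc, a short block time, and either the block state or this ability active with right mouse held.
; On start it plays the block-start montage or a random ability montage.
; On end it resumes the block loop if possible with input held, otherwise resets moveset and goes idle.
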(event `self.StartAbility`
  (bind _block_start_montage (`self.Block Start Montage`))
  (`parent.StartAbility`)
  (`/Engine/EditorBlueprintResources/StandardMacros.IsValid` _block_start_montage
    (:`Is Valid`
      (`self.PlayAbilityMontage` _block_start_montage))
    (:`Is Not Valid`
      (bind _list_of_montages (`self.Get Ability Montages` (`GameplayStatics.GetObjectClass` self)))
      (`self.PlayAbilityMontage` (`KismetArrayLibrary.Array_Random` _list_of_montages)))))

(event `self.EndAbility`
  (bind _tempestabilitycomponent (`self.Get Tempest Ability Component`))
  (bind _tempest_state_manager_component (`self.Tempest State Manager Component`))
  (bind _tempest_state_manager_component_2 (`self.Tempest State Manager Component`))
  (bind _returnvalue (`Pawn.GetController` (`self.Player Character`)))
  (bind _returnvalue_2 (`GameplayStatics.GetObjectClass` (`TempestBaseAbilityManagerComponent.GetAbilityOfGameplayTag` _tempestabilitycomponent (struct :`TagName` "Ability.Block.Loop"))))
  (`parent.EndAbility`)
  (bind _mapping_context (message `/TempestCombatFramework/Interfaces/BPI_PlayerInputs.Get Mapping Context` _returnvalue))
  (if (`/TempestCombatFramework/Libraries/BFL_TempestInputs.Get Is Input Clicked` _mapping_context "/TempestCombatFramework/Input/RightMouse_Input.RightMouse_Input" (cast `PlayerController` _returnvalue :!pure true))
    (if (`TempestBaseAbilityManagerComponent.GetCanPerformAbilityOfClass` _tempestabilitycomponent _returnvalue_2)
      (`TempestBaseAbilityManagerComponent.PerformAbilityOfClass` (`self.Get Tempest Ability Component`) _returnvalue_2)
      (`TempestBaseStateManagerComponent.SetCurrentActiveState` _tempest_state_manager_component (`TempestBaseStateManagerComponent.GetStateOfGameplayTag` _tempest_state_manager_component (struct :`TagName` "State.Normal Block")))
      (else
        (message `/TempestCombatFramework/Interfaces/BPI_GeneralInterface.Assign Moveset` (`SkeletalMeshComponent.GetAnimInstance` (`Character.Mesh` (`self.Player Character`))) "NewEnumerator1" :!label _label)
        (`TempestBaseStateManagerComponent.PerformStateOfClass` _tempest_state_manager_component_2 (`GameplayStatics.GetObjectClass` (`TempestBaseStateManagerComponent.GetStateOfGameplayTag` _tempest_state_manager_component_2 (struct :`TagName` "State.Idle"))))))
    (else
      (goto _label))))

(fn `CanPerformAbility`
  (returns (ReturnValue :type Boolean))
  (bind _tempest_state_manager_component (`self.Tempest State Manager Component`))
  (bind _returnvalue (`Actor.GetComponentByClass` (`self.Player Character`) "/TempestCombatFramework/Components/BP_TempestBaseCombatComponent.BP_TempestBaseCombatComponent_C"))
  (bind _mapping_context (message `/TempestCombatFramework/Interfaces/BPI_PlayerInputs.Get Mapping Context` (`Pawn.GetController` (`self.Player Character`))))
  (`/Engine/EditorBlueprintResources/StandardMacros.IsValid` (`TempestBaseStateManagerComponent.GetCurrentActiveState` (`self.Tempest State Manager Component`))
    (:`Is Valid`
      (bind (_return_value_y__pitch_ _return_value_z__yaw_) (`/TempestCombatFramework/Libraries/BFL_TempestGeneralFunctions.Calculate Angle Between Actors` (`self.Player Character`) (`TempestAttackPropertiesObject.GetAttackPropertyOwner` (`TempestCombatComponent.ReceivedAttackProperty` _returnvalue))))
      (bind _asbp_player_block_state (cast `/TempestCombatFramework/States/Player/BP_PlayerBlockState` (`TempestBaseStateManagerComponent.GetStateOfGameplayTag` _tempest_state_manager_component (struct :`TagName` "State.Normal Block"))))
      (return (and (`BlueprintGameplayTagLibrary.HasTag` (`TempestCombatComponent.GetCombatStatus` _returnvalue) (struct :`TagName` "Status.Combat.InCombat")) (`KismetSystemLibrary.IsValid` (`/TempestCombatFramework/Components/BP_TempestPlayerCombatComponent.Get Equipped Weapon` _returnvalue)) (`KismetMathLibrary.InRange_FloatFloat` _return_value_z__yaw_ -65.0 65.0) (or (== (`TempestBaseStateObject.StateGameplayTag` (`TempestBaseStateManagerComponent.GetCurrentActiveState` _tempest_state_manager_component)) (struct :`TagName` "State.Normal Block")) (and (`self.Get Is Current Ability Active`) (`/TempestCombatFramework/Libraries/BFL_TempestInputs.Get Is Input Clicked` _mapping_context "/TempestCombatFramework/Input/RightMouse_Input.RightMouse_Input"))) (<= (`/TempestCombatFramework/States/Player/BP_PlayerBlockState.Block Time` _asbp_player_block_state) 0.15))))
    (:`Is Not Valid`
      (return false))))