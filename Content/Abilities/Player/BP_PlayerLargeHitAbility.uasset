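; Player ability for reacting to a heavy hit, allowed only when not invincible, off cooldown and holding a weapon.
; On start it plays a hit reaction montage, shakes the camera and applies impact effects through the defense property.
; A brief hit-stop follows, dropping CustomTimeDilation on attacker and player, then restoring it.
; Ending the ability returns the state manager to Idle.
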(event `self.StartAbility`
  (bind _player_character (`self.Player Character`))
  (bind _returnvalue (`TempestAttackPropertiesObject.GetAttackPropertyOwner` (`TempestCombatComponent.ReceivedAttackProperty` (`/TempestCombatFramework/Characters/BP_TCF_DefaultThirdPersonCharacter.BP_TempestPlayerCombatComponent` _player_character))))
  (`parent.StartAbility`)
  (bind _list_of_montages (`self.Get Ability Montages` (`GameplayStatics.GetObjectClass` self)))
  (set `self.Hit Reaction Montages` _list_of_montages)
  (`self.PlayAbilityMontage` (`|GetArrayItem` (`self.Hit Reaction Montages`)) 1.0 "MontageLength")
  (`PlayerCameraManager.StartCameraShake` :`self` (`GameplayStatics.GetPlayerCameraManager` 0) :`ShakeClass` "/Game/TempestCombatFramework/Camera/CameraShake/BP_NormalHitCameraShake.BP_NormalHitCameraShake_C")
  (bind _asbp_base_defense_property (cast `/TempestCombatFramework/DefenseProperties/BP_BaseDefenseProperty` (`TempestCombatComponent.OwnerDefenseProperty` (`/TempestCombatFramework/Characters/BP_TCF_DefaultThirdPersonCharacter.BP_TempestPlayerCombatComponent` (`self.Player Character`)))))
  (`/TempestCombatFramework/DefenseProperties/BP_BaseDefenseProperty.Apply Hit Effect Of Class` _asbp_base_defense_property "/TempestCombatFramework/ImpactEffects/BP_NormalImpactEffects.BP_NormalImpactEffects_C")
  (`KismetSystemLibrary.Delay` 0.05)
  (bind _output_get (set `Actor.CustomTimeDilation` 0.05 _returnvalue))
  (set `Actor.CustomTimeDilation` _output_get _player_character)
  (`KismetSystemLibrary.Delay` 0.1)
  (bind _output_get_2 (set `Actor.CustomTimeDilation` 1.0 _returnvalue))
  (set `Actor.CustomTimeDilation` _output_get_2 _player_character))

(event `self.EndAbility`
  (bind _tempest_state_manager_component (`self.Tempest State Manager Component`))
  (`parent.EndAbility`)
  (`TempestBaseStateManagerComponent.PerformStateOfClass` _tempest_state_manager_component (`GameplayStatics.GetObjectClass` (`TempestBaseStateManagerComponent.GetStateOfGameplayTag` _tempest_state_manager_component (struct :`TagName` "State.Idle")))))

(fn `CanPerformAbility`
  (returns (ReturnValue :type Boolean))
  (bind _bp_tempestplayercombatcomponent (`/TempestCombatFramework/Characters/BP_TCF_DefaultThirdPersonCharacter.BP_TempestPlayerCombatComponent` (`self.Player Character`)))
  (if (not (`BlueprintGameplayTagLibrary.HasTag` (`TempestCombatComponent.GetCombatStatus` _bp_tempestplayercombatcomponent) (struct :`TagName` "Status.Combat.Invincible")))
    (bind _asbp_base_attack_properties (cast `/TempestCombatFramework/AttackProperties/BP_BaseAttackProperties` (`TempestCombatComponent.ReceivedAttackProperty` _bp_tempestplayercombatcomponent)))
    (return (and (== (`/TempestCombatFramework/AttackProperties/BP_BaseAttackProperties.Attack Property Tag` _asbp_base_attack_properties) (struct :`TagName` "Property.Attack.Heavy")) (not (`self.GetIsAbilityOnCooldown`)) (`KismetSystemLibrary.IsValid` (`/TempestCombatFramework/Components/BP_TempestPlayerCombatComponent.Get Equipped Weapon` (`/TempestCombatFramework/Characters/BP_TCF_DefaultThirdPersonCharacter.BP_TempestPlayerCombatComponent` (`self.Player Character`))))))
    (else
      (return false))))