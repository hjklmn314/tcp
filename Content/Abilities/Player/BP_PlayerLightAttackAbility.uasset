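; Player light attack ability that plays a combo of montages, advancing a wrapping index on each start and notifying the combat component.
; It can run only when the last fired input is the attack input, montages exist, the player is in combat and a weapon is equipped.
; On end it resets the combo and checks the weapon's pressed inputs, trying NormalBlock if block is held, otherwise returning to Idle.
; Cancelling also resets the combo.
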(event `self.StartAbility`
  (bind _anim_montages (`self.Anim Montages`))
  (bind _returnvalue (+ (`self.Combo Attack Index`) 1))
  (`parent.StartAbility`)
  (bind _list_of_montages (`self.Get Ability Montages` (`GameplayStatics.GetObjectClass` self)))
  (set `self.Anim Montages` _list_of_montages)
  (`self.PlayAbilityMontage` (`|GetArrayItem` _anim_montages (`self.Combo Attack Index`)))
  (set `self.Combo Attack Index` (select `bool` (> _returnvalue (`KismetArrayLibrary.Array_LastIndex` _anim_montages)) :`false` _returnvalue))
  (`/TempestCombatFramework/Components/BP_TempestBaseCombatComponent.On Attack Started` (`Actor.GetComponentByClass` (`self.Player Character`) "/TempestCombatFramework/Components/BP_TempestBaseCombatComponent.BP_TempestBaseCombatComponent_C")))

(event `self.EndAbility`
  (bind _tempest_state_manager_component (`self.Tempest State Manager Component`))
  (bind _tempest_state_manager_component_2 (`self.Tempest State Manager Component`))
  (`parent.EndAbility`)
  (set `self.Combo Attack Index` 0)
  (bind _asplayer_controller (cast `PlayerController` (`Pawn.GetController` (`self.Player Character`))))
  (bind _asbp_base_player_weapon (cast `/TempestCombatFramework/Actors/Weapons/Player/BP_BasePlayerWeapon` (`/TempestCombatFramework/Components/BP_TempestPlayerCombatComponent.Get Equipped Weapon` (`/TempestCombatFramework/Characters/BP_TCF_DefaultThirdPersonCharacter.BP_TempestPlayerCombatComponent` (`self.Player Character`)))))
  (bind _mapping_context (message `/TempestCombatFramework/Interfaces/BPI_PlayerInputs.Get Mapping Context` (`Pawn.GetController` (`self.Player Character`))))
  (bind _associated_tag (`/TempestCombatFramework/Libraries/BFL_TempestInputs.Get Pressed Input Action From Map` (`/TempestCombatFramework/DataAssets/BasePlayer_PDA.Player Inputs` (`/TempestCombatFramework/Actors/Weapons/Player/BP_BasePlayerWeapon.Associated Data Asset` _asbp_base_player_weapon)) _asplayer_controller _mapping_context))
  (if (`BlueprintGameplayTagLibrary.IsGameplayTagValid` _associated_tag)
    (`|SwitchGameplayTag` _associated_tag
      (:`Default`
        (`TempestBaseStateManagerComponent.PerformStateOfClass` _tempest_state_manager_component (`GameplayStatics.GetObjectClass` (`TempestBaseStateManagerComponent.GetStateOfGameplayTag` _tempest_state_manager_component (struct :`TagName` "State.Idle"))) :!label _label))
      (:`Input.Block`
        (`TempestBaseStateManagerComponent.TryPerformStateOfClass` _tempest_state_manager_component_2 (`GameplayStatics.GetObjectClass` (`TempestBaseStateManagerComponent.GetStateOfGameplayTag` _tempest_state_manager_component_2 (struct :`TagName` "State.Normal Block"))) true)))
    (else
      (goto _label))))

(event `self.CancelAbility`
  (set `self.Combo Attack Index` 0))

(fn `CanPerformAbility`
  (returns (ReturnValue :type Boolean))
  (bind _bp_tempestplayercombatcomponent (`/TempestCombatFramework/Characters/BP_TCF_DefaultThirdPersonCharacter.BP_TempestPlayerCombatComponent` (`self.Player Character`)))
  (bind _last_fired_input (message `/TempestCombatFramework/Interfaces/BPI_PlayerInputs.Get Last Fired Input` (`Pawn.GetController` (`self.Player Character`))))
  (if (== _last_fired_input "/TempestCombatFramework/Input/Attack_Input.Attack_Input")
    (bind _list_of_montages (`self.Get Ability Montages` (`GameplayStatics.GetObjectClass` self)))
    (return (and true (> (`KismetArrayLibrary.Array_Length` _list_of_montages) 0) (`BlueprintGameplayTagLibrary.HasTag` (`TempestCombatComponent.GetCombatStatus` _bp_tempestplayercombatcomponent) (struct :`TagName` "Status.Combat.InCombat")) (`KismetSystemLibrary.IsValid` (`/TempestCombatFramework/Components/BP_TempestPlayerCombatComponent.Get Equipped Weapon` _bp_tempestplayercombatcomponent))))
    (else
      (return false))))