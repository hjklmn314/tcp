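; Player ability that reacts to a normal attack landing on the player's block.
; On start it plays a block montage, applies shield impact effects and camera shake, then briefly slows attacker and player via CustomTimeDilation for hit-stop.
; On end it resumes the block loop if right mouse is held and allowed, otherwise returns to Idle.
; It requires combat status, an equipped weapon, a frontal attacker, and active blocking or an active block-hit with input held.
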(event `self.StartAbility`
  (bind _player_character (`self.Player Character`))
  (bind _block_start_montage (`self.Block Start Montage`))
  (bind _returnvalue (`TempestAttackPropertiesObject.GetAttackPropertyOwner` (`TempestCombatComponent.ReceivedAttackProperty` (`/TempestCombatFramework/Characters/BP_TCF_DefaultThirdPersonCharacter.BP_TempestPlayerCombatComponent` _player_character))))
  (`parent.StartAbility`)
  (`/Engine/EditorBlueprintResources/StandardMacros.IsValid` _block_start_montage
    (:`Is Valid`
      (`self.PlayAbilityMontage` _block_start_montage))
    (:`Is Not Valid`
      (bind _list_of_montages (`self.Get Ability Montages` (`GameplayStatics.GetObjectClass` self)))
      (`self.PlayAbilityMontage` (`KismetArrayLibrary.Array_Random` _list_of_montages))))
  (bind _asbp_base_defense_property (cast `/TempestCombatFramework/DefenseProperties/BP_BaseDefenseProperty` (`TempestCombatComponent.OwnerDefenseProperty` (`/TempestCombatFramework/Characters/BP_TCF_DefaultThirdPersonCharacter.BP_TempestPlayerCombatComponent` (`self.Player Character`)))))
  (`/TempestCombatFramework/DefenseProperties/BP_BaseDefenseProperty.Apply Hit Effect Of Class` _asbp_base_defense_property "/TempestCombatFramework/ImpactEffects/BP_ShieldBlockImpactEffects.BP_ShieldBlockImpactEffects_C")
  (`PlayerCameraManager.StartCameraShake` :`self` (`GameplayStatics.GetPlayerCameraManager` 0) :`ShakeClass` "/Game/TempestCombatFramework/Camera/CameraShake/BP_NormalHitCameraShake.BP_NormalHitCameraShake_C")
  (`KismetSystemLibrary.Delay` 0.05)
  (bind _output_get (set `Actor.CustomTimeDilation` 0.1 _returnvalue))
  (set `Actor.CustomTimeDilation` _output_get _player_character)
  (`KismetSystemLibrary.Delay` 0.05)
  (bind _output_get_2 (set `Actor.CustomTimeDilation` 1.0 _returnvalue))
  (set `Actor.CustomTimeDilation` _output_get_2 _player_character))

(event `self.EndAbility`
  (bind _tempestabilitycomponent (`self.Get Tempest Ability Component`))
  (bind _tempest_state_manager_component (`self.Tempest State Manager Component`))
  (bind _tempest_state_manager_component_2 (`self.Tempest State Manager Component`))
  (bind _returnvalue (`GameplayStatics.GetObjectClass` (`TempestBaseAbilityManagerComponent.GetAbilityOfGameplayTag` _tempestabilitycomponent (struct :`TagName` "Ability.Block.Loop"))))
  (`parent.EndAbility`)
  (bind _mapping_context (message `/TempestCombatFramework/Interfaces/BPI_PlayerInputs.Get Mapping Context` (`Pawn.GetController` (`self.Player Character`))))
  (if (`/TempestCombatFramework/Libraries/BFL_TempestInputs.Get Is Input Clicked` _mapping_context "/TempestCombatFramework/Input/RightMouse_Input.RightMouse_Input" (`self.Player Controller`))
    (if (`TempestBaseAbilityManagerComponent.GetCanPerformAbilityOfClass` _tempestabilitycomponent _returnvalue)
      (`TempestBaseAbilityManagerComponent.PerformAbilityOfClass` (`self.Get Tempest Ability Component`) _returnvalue)
      (`TempestBaseStateManagerComponent.SetCurrentActiveState` _tempest_state_manager_component (`TempestBaseStateManagerComponent.GetStateOfGameplayTag` _tempest_state_manager_component (struct :`TagName` "State.Normal Block")))
      (else
        (message `/TempestCombatFramework/Interfaces/BPI_GeneralInterface.Assign Moveset` (`SkeletalMeshComponent.GetAnimInstance` (`Character.Mesh` (`self.Player Character`))) "NewEnumerator1" :!label _label)
        (`TempestBaseStateManagerComponent.PerformStateOfClass` _tempest_state_manager_component_2 (`GameplayStatics.GetObjectClass` (`TempestBaseStateManagerComponent.GetStateOfGameplayTag` _tempest_state_manager_component_2 (struct :`TagName` "State.Idle"))))))
    (else
      (goto _label))))

(fn `CanPerformAbility`
  (returns (ReturnValue :type Boolean))
  (bind _returnvalue (`Actor.GetComponentByClass` (`self.Player Character`) "/TempestCombatFramework/Components/BP_TempestBaseCombatComponent.BP_TempestBaseCombatComponent_C"))
  (`/Engine/EditorBlueprintResources/StandardMacros.IsValid` (`TempestBaseStateManagerComponent.GetCurrentActiveState` (`self.Tempest State Manager Component`))
    (:`Is Valid`
      (bind _mapping_context (message `/TempestCombatFramework/Interfaces/BPI_PlayerInputs.Get Mapping Context` (`Pawn.GetController` (`self.Player Character`))))
      (bind (_return_value_y__pitch_ _return_value_z__yaw_) (`/TempestCombatFramework/Libraries/BFL_TempestGeneralFunctions.Calculate Angle Between Actors` (`self.Player Character`) (`TempestAttackPropertiesObject.GetAttackPropertyOwner` (`TempestCombatComponent.ReceivedAttackProperty` _returnvalue))))
      (return (and (`BlueprintGameplayTagLibrary.HasTag` (`TempestCombatComponent.GetCombatStatus` _returnvalue) (struct :`TagName` "Status.Combat.InCombat")) (`KismetSystemLibrary.IsValid` (`/TempestCombatFramework/Components/BP_TempestPlayerCombatComponent.Get Equipped Weapon` _returnvalue)) (`KismetMathLibrary.InRange_FloatFloat` _return_value_z__yaw_ -65.0 65.0) (or (== (`TempestBaseStateObject.StateGameplayTag` (`TempestBaseStateManagerComponent.GetCurrentActiveState` (`self.Tempest State Manager Component`))) (struct :`TagName` "State.Normal Block")) (and (`self.Get Is Current Ability Active`) (`/TempestCombatFramework/Libraries/BFL_TempestInputs.Get Is Input Clicked` _mapping_context "/TempestCombatFramework/Input/RightMouse_Input.RightMouse_Input" (`self.Player Controller`)))))))
    (:`Is Not Valid`
      (return false))))