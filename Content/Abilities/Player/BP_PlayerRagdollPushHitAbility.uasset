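; Player hit-reaction ability that ragdolls the player away from the attacker on Thrust attacks, gated by invincibility, cooldown and an equipped weapon.
; Activation plays a montage, impact effects, camera shake and a brief time-dilation hit stop.
; A separate toggle event enables impulse-driven physics, while tick keeps the capsule following a bone via interpolated ground traces.
; Recovery saves a pose snapshot, disables physics and plays the second montage.
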(event `self.StartAbility`
  (bind _player_character (`self.Player Character`))
  (bind _returnvalue (`TempestAttackPropertiesObject.GetAttackPropertyOwner` (`TempestCombatComponent.ReceivedAttackProperty` (`/TempestCombatFramework/Characters/BP_TCF_DefaultThirdPersonCharacter.BP_TempestPlayerCombatComponent` _player_character))))
  (`parent.StartAbility`)
  (bind _list_of_montages (`self.Get Ability Montages` (`GameplayStatics.GetObjectClass` self)))
  (bind _output_get (set `self.Hit Reaction Montages` _list_of_montages))
  (`self.PlayAbilityMontage` (`|GetArrayItem` _output_get) 1.0 "MontageLength")
  (`self.ApplyAbilityCooldown`)
  (bind _asbp_base_defense_property (cast `/TempestCombatFramework/DefenseProperties/BP_BaseDefenseProperty` (`TempestCombatComponent.OwnerDefenseProperty` (`/TempestCombatFramework/Characters/BP_TCF_DefaultThirdPersonCharacter.BP_TempestPlayerCombatComponent` (`self.Player Character`)))))
  (`/TempestCombatFramework/DefenseProperties/BP_BaseDefenseProperty.Apply Hit Effect Of Class` _asbp_base_defense_property "/TempestCombatFramework/ImpactEffects/BP_NormalImpactEffects.BP_NormalImpactEffects_C")
  (`PlayerCameraManager.StartCameraShake` :`self` (`GameplayStatics.GetPlayerCameraManager` 0) :`ShakeClass` "/Game/TempestCombatFramework/Camera/CameraShake/BP_NormalHitCameraShake.BP_NormalHitCameraShake_C")
  (`KismetSystemLibrary.Delay` 0.05)
  (bind _output_get_2 (set `Actor.CustomTimeDilation` 0.05 _returnvalue))
  (set `Actor.CustomTimeDilation` _output_get_2 _player_character)
  (`KismetSystemLibrary.Delay` 0.1)
  (bind _output_get_3 (set `Actor.CustomTimeDilation` 1.0 _returnvalue))
  (set `Actor.CustomTimeDilation` _output_get_3 _player_character))

(event `self.EndAbility`
  (bind _tempest_state_manager_component (`self.Tempest State Manager Component`))
  (`parent.EndAbility`)
  (`TempestBaseStateManagerComponent.PerformStateOfClass` _tempest_state_manager_component (`GameplayStatics.GetObjectClass` (`TempestBaseStateManagerComponent.GetStateOfGameplayTag` _tempest_state_manager_component (struct :`TagName` "State.Idle")))))

(event `self.TickAbility`
  (params (TickTime :type "Float (single-precision)"))
  (if (`self.Ragdolling`)
    (`self.CalculateMeshLocation`)
    (`SceneComponent.K2_SetWorldLocation` (`Character.CapsuleComponent` (`self.Player Character`)) (`self.MeshLocation`) false false)
    (else
      (set `self.MeshLocation` (+ (`SceneComponent.GetSocketLocation` (`Character.Mesh` (`self.Player Character`)) (`self.Bone Name`)) (0.0 0.0 97.0))))))

(event `/TempestCombatFramework/Interfaces/BPI_TempestAbilitiesAndStates.Toggle Ragdoll Hit Reaction`
  (params (Value :type Boolean))
  (bind _player_character (`self.Player Character`))
  (bind _returnvalue (`Actor.K2_GetActorLocation` _player_character))
  (bind _mesh (`Character.Mesh` _player_character))
  (bind _mesh_2 (`Character.Mesh` (`self.Player Character`)))
  (bind _returnvalue_2 (`SkeletalMeshComponent.GetAnimInstance` _mesh))
  (if Value
    (`PrimitiveComponent.SetSimulatePhysics` _mesh true)
    (`PrimitiveComponent.SetCollisionProfileName` _mesh "Ragdoll" true)
    (`PrimitiveComponent.AddImpulseAtLocation` _mesh (* (`KismetMathLibrary.GetDirectionUnitVector` (`KismetMathLibrary.MakeVector` (.x (`Actor.K2_GetActorLocation` (`TempestAttackPropertiesObject.GetAttackPropertyOwner` (`TempestCombatComponent.ReceivedAttackProperty` (`/TempestCombatFramework/Characters/BP_TCF_DefaultThirdPersonCharacter.BP_TempestPlayerCombatComponent` (`self.Player Character`)))))) (.y (`Actor.K2_GetActorLocation` (`TempestAttackPropertiesObject.GetAttackPropertyOwner` (`TempestCombatComponent.ReceivedAttackProperty` (`/TempestCombatFramework/Characters/BP_TCF_DefaultThirdPersonCharacter.BP_TempestPlayerCombatComponent` (`self.Player Character`)))))) (.z _returnvalue)) _returnvalue) 10000.0) (`SceneComponent.K2_GetComponentLocation` _mesh) "spine_01")
    (message `/TempestCombatFramework/Interfaces/BPI_TempestAbilitiesAndStates.Toggle Ragdoll Hit Reaction` _returnvalue_2 true)
    (set `self.Ragdolling` true)
    (`KismetSystemLibrary.Delay` 2.0))
  (`AnimInstance.SavePoseSnapshot` (`SkeletalMeshComponent.GetAnimInstance` (`Character.Mesh` (`self.Player Character`))) "RagdollSnap")
  (`KismetSystemLibrary.Delay` 0.1)
  (`PrimitiveComponent.SetSimulatePhysics` _mesh_2 false)
  (`PrimitiveComponent.SetCollisionProfileName` _mesh_2 "Pawn" true)
  (`PrimitiveComponent.SetCollisionResponseToChannel` _mesh_2 "ECC_Pawn" "ECR_Ignore")
  (`PrimitiveComponent.SetCollisionResponseToChannel` _mesh_2 "ECC_GameTraceChannel1" "ECR_Block")
  (message `/TempestCombatFramework/Interfaces/BPI_TempestAbilitiesAndStates.Toggle Ragdoll Hit Reaction` _returnvalue_2 false)
  (`self.PlayAbilityMontage` (`|GetArrayItem` (`self.Hit Reaction Montages`) 1) 1.0 "MontageLength")
  (set `self.Ragdolling` false))

(fn `CalculateMeshLocation`
  (bind _returnvalue (`SceneComponent.GetSocketLocation` (`Character.Mesh` (`self.Player Character`)) (`self.Bone Name`)))
  (bind (_outhit _returnvalue_2) (`KismetSystemLibrary.LineTraceSingleForObjects` _returnvalue (+ _returnvalue (* (0.0 0.0 -1.0) 1000.0)) (`|MakeArray` "ObjectTypeQuery1" :!type "EObjectTypeQuery Enum")))
  (if _returnvalue_2
    (set `self.Capsule Location` (+ (`.Location` (`GameplayStatics.BreakHitResult` _outhit)) (0.0 0.0 97.0)))
    (else
      (set `self.Capsule Location` (+ (`SceneComponent.GetSocketLocation` (`Character.Mesh` (`self.Player Character`)) (`self.Bone Name`)) (0.0 0.0 97.0)))))
  (set `self.MeshLocation` (`KismetMathLibrary.VInterpTo` (`self.MeshLocation`) (`self.Capsule Location`) (`GameplayStatics.GetWorldDeltaSeconds`) 30.0)))

(fn `CanPerformAbility`
  (returns (ReturnValue :type Boolean))
  (bind _bp_tempestplayercombatcomponent (`/TempestCombatFramework/Characters/BP_TCF_DefaultThirdPersonCharacter.BP_TempestPlayerCombatComponent` (`self.Player Character`)))
  (if (not (`BlueprintGameplayTagLibrary.HasTag` (`TempestCombatComponent.GetCombatStatus` _bp_tempestplayercombatcomponent) (struct :`TagName` "Status.Combat.Invincible")))
    (bind _asbp_base_attack_properties (cast `/TempestCombatFramework/AttackProperties/BP_BaseAttackProperties` (`TempestCombatComponent.ReceivedAttackProperty` _bp_tempestplayercombatcomponent)))
    (return (and (== (`/TempestCombatFramework/AttackProperties/BP_BaseAttackProperties.Attack Property Tag` _asbp_base_attack_properties) (struct :`TagName` "Property.Attack.Thrust")) (not (`self.GetIsAbilityOnCooldown`)) (`KismetSystemLibrary.IsValid` (`/TempestCombatFramework/Components/BP_TempestPlayerCombatComponent.Get Equipped Weapon` (`/TempestCombatFramework/Characters/BP_TCF_DefaultThirdPersonCharacter.BP_TempestPlayerCombatComponent` (`self.Player Character`))))))
    (else
      (return false))))

(fn `Get Block Time Since Last Clicked`
  (returns (`Return Value` :type "Float (double-precision)"))
  (return 0.0))

(fn `Get Montage Counter For Ability`
  (returns (`Counter Montage` :type "AnimMontage Object Reference"))
  (return null))