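; Statistic that tracks how long its owning character has been active, counting from construction until death, with no separate combat check despite the name.
; On construction it gets the state manager component from the character's controller and starts a looping timer.
; Each tick of that timer adds the timer rate, rolls it into seconds, minutes and hours, and formats the text to save.
; The timer clears when the active state is Death.
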(event `self.ConstructStatistic`
  (`parent.ConstructStatistic`)
  (bind _ascharacter (cast `Character` (`self.Owning Actor`)))
  (set `self.State Component` (`Actor.GetComponentByClass` (`Pawn.GetController` _ascharacter) "/Script/TempestCombatFramework.TempestBaseStateManagerComponent"))
  (`KismetSystemLibrary.K2_SetTimer` null "Increment Time In Game" (`self.Rate`) true)
  (`self.Increment Time In Game`))

(event `Increment Time In Game`
  (bind _state_component (`self.State Component`))
  (bind _returnvalue (`TempestBaseStateManagerComponent.GetCurrentActiveState` _state_component))
  (`/Engine/EditorBlueprintResources/StandardMacros.IsValid` _state_component
    (:`Is Valid`
      (`/Engine/EditorBlueprintResources/StandardMacros.IsValid` _returnvalue
        (:`Is Valid`
          (if (!= (`TempestBaseStateObject.StateGameplayTag` _returnvalue) (struct :`TagName` "State.Death"))
            (bind _output_get (set `self.MilliSeconds` (+ (`self.MilliSeconds`) (`self.Rate`))))
            (if (> (`KismetStringLibrary.Conv_StringToDouble` (`KismetTextLibrary.Conv_TextToString` (`KismetTextLibrary.Conv_DoubleToText` _output_get "HalfToEven" false true 1 324 0 2))) 1.0)
              (set `self.MilliSeconds` (- (`self.MilliSeconds`) 1.0))
              (bind _output_get_2 (set `self.Seconds` (+ (`self.Seconds`) 1)))
              (bind _output_get_3 (set `self.Miutes` (/ _output_get_2 60)))
              (set `self.Hours` (/ _output_get_3 60)))
            (set `self.Text To Save` (`KismetTextLibrary.Conv_StringToText` (`KismetStringLibrary.Concat_StrStr` "Hours:  " (`KismetStringLibrary.Conv_IntToString` (`self.Hours`)) " Minutes:  " (`KismetStringLibrary.Conv_IntToString` (mod (`self.Miutes`) 60)) " Seconds:  " (`KismetStringLibrary.Conv_IntToString` (mod (`self.Seconds`) 60)) " Ms:  " (`KismetTextLibrary.Conv_TextToString` (`KismetTextLibrary.Conv_DoubleToText` (* (`self.MilliSeconds`) 100.0) "HalfToEven" false true 1 324 0 2)))))
            (else
              (`KismetSystemLibrary.K2_ClearTimer` null "Increment Time In Game"))))))))