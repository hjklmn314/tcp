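; BP_BaseStatistic is a base class for a statistic object that belongs to an actor and holds a current value.
; Construction casts the object's outer to Actor and caches it as the owning actor.
; Updates add the passed amount to the current value, and reset restores the value from the class defaults.
; The tick event is an empty hook.
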(event `self.ConstructStatistic`
  (bind _asactor (cast `Actor` (`KismetSystemLibrary.GetOuterObject` self)))
  (set `self.Owning Actor` _asactor))

(event `self.TickStatistic`
  (params (DeltaTime :type "Float (single-precision)")))

(event `self.UpdateStatisticValueBy`
  (params (NewStatisticValue :type "Float (single-precision)"))
  (set `self.StatisticCurrentValue` (+ NewStatisticValue (`self.StatisticCurrentValue`))))

(event `self.ResetStatisticValue`
  (set `self.StatisticCurrentValue` (defaults `Object` (`GameplayStatics.GetObjectClass` self))))