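; BP_BaseWeapon is a base weapon actor that holds a list of weapon parts and snaps their meshes onto the owning character's skeletal mesh.
; Each registered entry stores a mesh plus equipping and unequipping socket names.
; Attach functions move one indexed entry or all of them to either socket, chosen by an EquipSlot flag.
; EquipWeapon and UnEquipWeapon are empty, and the event graph holds no logic.
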(fn `Attach All Weapon`
  (params (`Equip Slot` :type Boolean))
  (bind _ascharacter (cast `Character` (`self.GetOwner`)))
  (for _array_element (`self.Weapon Properties`)
    (bind (_weaponmesh _equippingsocket _unequippingsocket) (break `/TempestCombatFramework/StructuresEnums/S_WeaponDetails` _array_element))
    (`/Engine/EditorBlueprintResources/StandardMacros.IsValid` _weaponmesh
      (:`Is Valid`
        (`SceneComponent.K2_AttachToComponent` _weaponmesh (`Character.Mesh` _ascharacter) (select `bool` `Equip Slot` :`false` _unequippingsocket :`true` _equippingsocket) "SnapToTarget" "SnapToTarget" "SnapToTarget" true)))))

(fn `Attach Weapon At Index`
  (params (Index :type Integer) (`Equip Slot` :type Boolean))
  (bind _weapon_properties (`self.Weapon Properties`))
  (bind (_weaponmesh _equippingsocket _unequippingsocket) (break `/TempestCombatFramework/StructuresEnums/S_WeaponDetails` (`|GetArrayItem` _weapon_properties Index)))
  (if (> (`KismetArrayLibrary.Array_Length` _weapon_properties) 0)
    (bind _ascharacter (cast `Character` (`self.GetOwner`)))
    (`/Engine/EditorBlueprintResources/StandardMacros.IsValid` _weaponmesh
      (:`Is Valid`
        (`SceneComponent.K2_AttachToComponent` _weaponmesh (`Character.Mesh` _ascharacter) (select `bool` `Equip Slot` :`false` _unequippingsocket :`true` _equippingsocket) "SnapToTarget" "SnapToTarget" "SnapToTarget" true)))))

(fn `Equip Weapon`
  (locals (`Local Character` :type "Character Object Reference") (`Local State Manager Component` :type "TempestBaseStateManagerComponent Object Reference")))

(fn `Get Weapon Properties`
  (returns (`Weapon Properties` :type "Array of /TempestCombatFramework/StructuresEnums/S_WeaponDetails Structure"))
  (return (`self.Weapon Properties`)))

(fn `Register Weapon`
  (params (`New Weapon` :type "/TempestCombatFramework/StructuresEnums/S_WeaponDetails Structure (by ref)"))
  (`KismetArrayLibrary.Array_Add` (`self.Weapon Properties`) `New Weapon`))

(fn `UnEquip Weapon`)

(fn `UserConstructionScript`)