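; Base player weapon actor that configures its owning character for combat through Tempest components when it begins play.
; Equipping clears abilities, rebuilds controller states from the associated data asset, enters Idle, assigns attributes, registers the weapon and creates a right-hand trace on character mesh sockets.
; Unequipping clears traces, sends a moveset message to the AnimInstance and removes InCombat status.
; A separate function reapplies states and attributes, clearing old attributes first.
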(event `self.ReceiveBeginPlay`
  (`self.Equip Weapon`))

(fn `Equip Weapon`
  (locals (`Local Character` :type "Character Object Reference") (`Local State Manager Component` :type "TempestBaseStateManagerComponent Object Reference"))
  (bind _local_character (`local.Local Character`))
  (bind _local_state_manager_component (`local.Local State Manager Component`))
  (bind _ascharacter (cast `Character` (`self.GetOwner`)))
  (set `local.Local Character` _ascharacter)
  (bind _output_get (set `local.Local State Manager Component` (`self.GetComponentByClass` (`Pawn.GetController` _local_character) "/Script/TempestCombatFramework.TempestBaseStateManagerComponent")))
  (`TempestBaseStateManagerComponent.ClearStatesComponent` _output_get)
  (`TempestBaseAbilityManagerComponent.ClearAbilityComponent` (`self.GetComponentByClass` _local_character "/TempestCombatFramework/Components/BP_TempestAbilitySystemComponent.BP_TempestAbilitySystemComponent_C"))
  (for _array_element (`/TempestCombatFramework/DataAssets/BasePlayer_PDA.States To Create` (`self.Associated Data Asset`))
    (`TempestBaseStateManagerComponent.ConstructStateOfClass` _local_state_manager_component _array_element))
  (`TempestBaseStateManagerComponent.PerformStateOfClass` _local_state_manager_component (`GameplayStatics.GetObjectClass` (`TempestBaseStateManagerComponent.GetStateOfGameplayTag` _local_state_manager_component (struct :`TagName` "State.Idle"))))
  (`TempestAttributesComponents.AssignAttributes` (`self.GetComponentByClass` _local_character "/Script/TempestCombatFramework.TempestAttributesComponents") (`TempestGeneral_PDA.AttributesToCreate` (`self.Associated Data Asset`)))
  (`/TempestCombatFramework/Components/BP_TempestPlayerCombatComponent.Set Equipped Weapon` (`self.GetComponentByClass` (`local.Local Character`) "/TempestCombatFramework/Components/BP_TempestPlayerCombatComponent.BP_TempestPlayerCombatComponent_C") self)
  (bind _createdtraceobject (`TempestCollisionManagerComponent.ConstructTraceOfClass` (`self.GetComponentByClass` _local_character "/Script/TempestCombatFramework.TempestCollisionManagerComponent") "/TempestCombatFramework/Trace/BP_BaseTraceObject.BP_BaseTraceObject_C"))
  (set `TempestBaseTraceObject.TraceGameplayTag` (struct :`TagName` "Trace.Right Hand Weapon") _createdtraceobject)
  (`TempestBaseTraceObject.SetTraceMeshInfo` _createdtraceobject (`Character.Mesh` (`local.Local Character`)) (`|MakeArray` "Weapon Trace 1" "Weapon Trace 2" "Weapon Trace 3" "Weapon Trace 4" "Weapon Trace 5" "Weapon Trace 6" "Weapon Trace 7" "Weapon Trace 8" "Weapon Trace 9" :!type "Name")))

(fn `Set Attributes & States`
  (locals (`Local Character` :type "Character Object Reference") (`Local State Manager Component` :type "TempestBaseStateManagerComponent Object Reference"))
  (bind _local_character (`local.Local Character`))
  (bind _local_state_manager_component (`local.Local State Manager Component`))
  (bind _returnvalue (`self.GetComponentByClass` _local_character "/Script/TempestCombatFramework.TempestAttributesComponents"))
  (bind _returnvalue_2 (`self.GetComponentByClass` (`Pawn.GetController` _local_character) "/Script/TempestCombatFramework.TempestBaseStateManagerComponent"))
  (bind _ascharacter (cast `Character` (`self.GetOwner`)))
  (set `local.Local Character` _ascharacter)
  (`/Engine/EditorBlueprintResources/StandardMacros.IsValid` _returnvalue_2
    (:`Is Valid`
      (bind _output_get (set `local.Local State Manager Component` _returnvalue_2))
      (`TempestBaseStateManagerComponent.ClearStatesComponent` _output_get)
      (`TempestBaseAbilityManagerComponent.ClearAbilityComponent` (`self.GetComponentByClass` _local_character "/TempestCombatFramework/Components/BP_TempestAbilitySystemComponent.BP_TempestAbilitySystemComponent_C"))
      (for _array_element (`/TempestCombatFramework/DataAssets/BasePlayer_PDA.States To Create` (`self.Associated Data Asset`))
        (`TempestBaseStateManagerComponent.ConstructStateOfClass` _local_state_manager_component _array_element))
      (`TempestBaseStateManagerComponent.PerformStateOfClass` _local_state_manager_component (`GameplayStatics.GetObjectClass` (`TempestBaseStateManagerComponent.GetStateOfGameplayTag` _local_state_manager_component (struct :`TagName` "State.Idle"))))
      (`TempestAttributesComponents.ClearAttributes` _returnvalue)
      (`TempestAttributesComponents.AssignAttributes` _returnvalue (`TempestGeneral_PDA.AttributesToCreate` (`self.Associated Data Asset`))))))

(fn `UnEquip Weapon`
  (bind _returnvalue (`self.GetOwner`))
  (`TempestCollisionManagerComponent.ClearAvailableTraceObjects` (`self.GetComponentByClass` _returnvalue "/Script/TempestCombatFramework.TempestCollisionManagerComponent"))
  (bind _ascharacter (cast `Character` _returnvalue))
  (message `/TempestCombatFramework/Interfaces/BPI_GeneralInterface.Assign Moveset` (`SkeletalMeshComponent.GetAnimInstance` (`Character.Mesh` _ascharacter)) "NewEnumerator0")
  (`TempestCombatComponent.ModifyCombatStatus` (`self.GetComponentByClass` (`self.GetOwner`) "/Script/TempestCombatFramework.TempestCombatComponent") (struct :`TagName` "Status.Combat.InCombat") "Remove"))

(fn `UserConstructionScript`)