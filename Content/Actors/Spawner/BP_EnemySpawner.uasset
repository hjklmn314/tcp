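; BP_EnemySpawner is a proximity spawner that creates an enemy while the player is inside its overlap sphere and destroys it when the player leaves.
; Sphere overlap, or a short-delayed check on BeginPlay, async loads the soft enemy class, with a flag blocking concurrent loads.
; The enemy spawns at SpawnLocation with the Arrow's rotation and receives a spawner reference by message; a missing class triggers a developer warning.
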(event `self.ReceiveBeginPlay`
  (`KismetSystemLibrary.Delay` 0.2)
  (if (`PrimitiveComponent.IsOverlappingActor` (`self.Overlapping Sphere`) (`GameplayStatics.GetPlayerCharacter` 0))
    (if (not (`self.Spawning`)) :!label _label
      (if (`KismetSystemLibrary.IsValidSoftClassReference` (`self.Enemy To Spawn`))
        (set `self.Spawning` true)
        (bind _class (`|LoadAssetClass` (`self.Enemy To Spawn`))
          (:`Completed`
            (bind _asactor (castclass `Actor` _class))
            (bind _returnvalue (`|SpawnActorFromClass` _asactor (`KismetMathLibrary.MakeTransform` (`SceneComponent.K2_GetComponentLocation` (`self.Spawn Location`)) (`SceneComponent.K2_GetComponentRotation` (`self.Arrow`))) "Undefined" "OverrideRootScale" null null))
            (bind _output_get (set `self.Spawned Actor` _returnvalue))
            (message `/TempestCombatFramework/Interfaces/BPI_EnemySpawner.Assign Enemy Spawner` _output_get self)
            (set `self.Spawning` false)))
        (else
          (`/Game/TempestCombatFramework/AI/Enemy/FL_DeveloperWarnings.Warn Developer Of Missing Enemy Spawn Variable` self))))))

(event `self.Overlapping Sphere.OnComponentBeginOverlap`
  (params (OverlappedComponent :type "PrimitiveComponent Object Reference") (OtherActor :type "Actor Object Reference") (OtherComp :type "PrimitiveComponent Object Reference") (OtherBodyIndex :type Integer) (bFromSweep :type Boolean) (SweepResult :type "HitResult Structure (by ref)"))
  (if (== OtherActor (`GameplayStatics.GetPlayerCharacter` 0))
    (goto _label)))

(event `self.Overlapping Sphere.OnComponentEndOverlap`
  (params (OverlappedComponent :type "PrimitiveComponent Object Reference") (OtherActor :type "Actor Object Reference") (OtherComp :type "PrimitiveComponent Object Reference") (OtherBodyIndex :type Integer))
  (if (== OtherActor (`GameplayStatics.GetPlayerCharacter` 0))
    (`/Engine/EditorBlueprintResources/StandardMacros.IsValid` (`self.Spawned Actor`)
      (:`Is Valid`
        (`self.K2_DestroyActor` (`self.Spawned Actor`))
        (set `self.Spawning` false)))))

(fn `UserConstructionScript`)