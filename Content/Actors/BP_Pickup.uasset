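; BP_Pickup is a world pickup that spawns a configured actor when a player touches it.
; Its sphere overlap checks the other actor's gameplay tags for Character.Player, including child tags.
; It then async-loads the soft class in ActorToPickup, spawns it with the overlapping actor as owner, and destroys itself.
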(event `self.Sphere.OnComponentBeginOverlap`
  (params (OverlappedComponent :type "PrimitiveComponent Object Reference") (OtherActor :type "Actor Object Reference") (OtherComp :type "PrimitiveComponent Object Reference") (OtherBodyIndex :type Integer) (bFromSweep :type Boolean) (SweepResult :type "HitResult Structure (by ref)"))
  (bind _tagcontainer (message `GameplayTagAssetInterface.GetOwnedGameplayTags` OtherActor))
  (if (`BlueprintGameplayTagLibrary.HasTag` _tagcontainer (struct :`TagName` "Character.Player"))
    (if (`KismetSystemLibrary.IsValidSoftClassReference` (`self.Actor To Pickup`))
      (bind _class (`|LoadAssetClass` (`self.Actor To Pickup`))
        (:`Completed`
          (bind _asactor (castclass `Actor` _class))
          (`|SpawnActorFromClass` _asactor (`KismetMathLibrary.MakeTransform` (0.0 0.0 0.0)) "Undefined" "OverrideRootScale" OtherActor null)
          (`self.K2_DestroyActor`))))))

(fn `UserConstructionScript`)