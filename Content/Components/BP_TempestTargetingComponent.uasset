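; Lock-on targeting component that lets the owning character lock onto AI enemies during combat.
; CanBeTargeted accepts only living actors tagged Character.AI, and only while the owner's combat component reports InCombat.
; Locking on switches to the targeting melee camera mode, shows the target's targeting point and stops orienting rotation to movement.
; Disabling lock-on clears the target and its targeting point, then restores the melee camera and movement-facing rotation.
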(event `self.InitializeTargetingComponent`
  (params (CameraComponent :type "CameraComponent Object Reference") (SpringArmComponent :type "SpringArmComponent Object Reference"))
  (bind _returnvalue (`self.GetOwner`))
  (`parent.InitializeTargetingComponent` CameraComponent SpringArmComponent)
  (bind _ascharacter (cast `Character` _returnvalue))
  (set `self.Owner Character` _ascharacter)
  (set `self.Tempest Camera Mode Component` (`Actor.GetComponentByClass` _returnvalue "/Script/TempestCameraSystems.TempestCameraModeComponent"))
  (set `self.Combat Component` (`Actor.GetComponentByClass` (`self.Owner Character`) "/Script/TempestCombatFramework.TempestCombatComponent")))

(event `self.DisableLockOn`
  (`/Engine/EditorBlueprintResources/StandardMacros.IsValid` (`self.GetTargetedActor`)
    (:`Is Valid`
      (message `/TempestCombatFramework/Interfaces/BPI_TargetingSystem.Toggle Targeting Point` (`self.GetTargetedActor`) false))
    (:`Is Not Valid`
      _))
  (set `self.TargetedActor` null)
  (`TempestCameraModeComponent.SetCameraModeOfClass` (`self.Tempest Camera Mode Component`) "/TempestCombatFramework/Camera/Modes/BP_MeleeCameraMode.BP_MeleeCameraMode_C")
  (set `CharacterMovementComponent.bOrientRotationToMovement` true (`Character.CharacterMovement` (`self.Owner Character`))))

(event `self.SetLockOnToTarget`
  (bind _tempest_camera_mode_component (`self.Tempest Camera Mode Component`))
  (`/Engine/EditorBlueprintResources/StandardMacros.IsValid` _tempest_camera_mode_component
    (:`Is Valid`
      (`TempestCameraModeComponent.SetCameraModeOfClass` _tempest_camera_mode_component "/TempestCombatFramework/Camera/Modes/BP_TargetingMeleeMode.BP_TargetingMeleeMode_C")
      (message `/TempestCombatFramework/Interfaces/BPI_TargetingSystem.Toggle Targeting Point` (`self.GetTargetedActor`) true)
      (set `CharacterMovementComponent.bOrientRotationToMovement` false (`Character.CharacterMovement` (`self.Owner Character`))))))

(fn `CanBeTargeted`
  (params (ActorToTarget :type "Actor Object Reference"))
  (returns (ReturnValue :type Boolean))
  (bind _tagcontainer (message `GameplayTagAssetInterface.GetOwnedGameplayTags` ActorToTarget))
  (return (and (`BlueprintGameplayTagLibrary.HasTag` _tagcontainer (struct :`TagName` "Character.AI")) (`BlueprintGameplayTagLibrary.HasTag` (`TempestCombatComponent.GetCombatStatus` (`self.Combat Component`)) (struct :`TagName` "Status.Combat.InCombat")) (not (`BlueprintGameplayTagLibrary.HasTag` _tagcontainer (struct :`TagName` "State.Death"))))))