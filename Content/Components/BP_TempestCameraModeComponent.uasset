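; BP_TempestCameraModeComponent is a camera mode component that starts in the melee camera mode and handles temporary camera post-process effects.
; On initialization it runs the parent setup with the camera and spring arm, then sets BP_MeleeCameraMode.
; Applying effects caches the camera's current post-process settings before replacing them, and resetting restores that cache.
; The cache is a single slot, so a second apply before a reset overwrites the saved original.
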(event `self.InitializeCameraModeComponent`
  (params (NewCameraComponent :type "CameraComponent Object Reference") (NewSpringArmComponent :type "SpringArmComponent Object Reference"))
  (`parent.InitializeCameraModeComponent` NewCameraComponent NewSpringArmComponent)
  (`self.SetCameraModeOfClass` "/TempestCombatFramework/Camera/Modes/BP_MeleeCameraMode.BP_MeleeCameraMode_C"))

(event `Apply Camera Effects`
  (params (`Post Process Settings` :type "PostProcessSettings Structure"))
  (bind _cameracomponent (`self.CameraComponent`))
  (set `self.Original Post Process` (`CameraComponent.PostProcessSettings` _cameracomponent))
  (set `CameraComponent.PostProcessSettings` `Post Process Settings` _cameracomponent))

(event `Reset Camera Effects`
  (set `CameraComponent.PostProcessSettings` (`self.Original Post Process`) (`self.CameraComponent`)))