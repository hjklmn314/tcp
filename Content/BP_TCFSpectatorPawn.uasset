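; BP_TCFSpectatorPawn is a spectator pawn that freezes the action while possessed.
; On possession it gathers all Characters and BP_BaseProjectile actors into OverlappedActors and slows each to near zero through CustomTimeDilation, leaving global time untouched.
; The Add key steps the action forward by restoring normal speed for a brief delay, then freezing again.
; Unpossessing restores normal speed on the gathered actors.
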(event `self.ReceivePossessed`
  (params (NewController :type "Controller Object Reference"))
  (bind _outactors (`GameplayStatics.GetAllActorsOfClass` "/TempestCombatFramework/Actors/Projectiles/BP_BaseProjectile.BP_BaseProjectile_C"))
  (bind _outactors_2 (`GameplayStatics.GetAllActorsOfClass` "/Script/Engine.Character"))
  (`KismetArrayLibrary.Array_Append` (`self.Overlapped Actors`) _outactors_2)
  (`KismetArrayLibrary.Array_Append` (`self.Overlapped Actors`) _outactors)
  (for _array_element (`self.Overlapped Actors`) :!label _label
    (set `Actor.CustomTimeDilation` 0.0001 _array_element)))

(event `Key|Add`
  (params (Key :type "Key Structure"))
  (:`Pressed`
    (for _array_element (`self.Overlapped Actors`)
      (set `Actor.CustomTimeDilation` 1.0 _array_element))
    (`KismetSystemLibrary.Delay` 0.02)
    (goto _label)))

(event `self.ReceiveUnpossessed`
  (params (OldController :type "Controller Object Reference"))
  (for _array_element (`self.Overlapped Actors`)
    (set `Actor.CustomTimeDilation` 1.0 _array_element)))

(fn `UserConstructionScript`)