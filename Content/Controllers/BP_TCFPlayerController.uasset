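; BP_TCFPlayerController is a player controller that sets up input, state management and targeting for the controlled pawn.
; InitializeController initializes the Tempest state manager, adds the Enhanced Input mapping context and caches the targeting component and original pawn.
; Helpers expose the last fired input, a Character.Player tag check and camera-yaw-relative movement direction; the mapping lookup always returns false.
; An unconnected FlipFlop holds a spectator-pawn possession toggle that never runs.
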(event `/TempestCombatFramework/Interfaces/BPI_GeneralInterface.Initialize Controller`
  (`TempestBaseStateManagerComponent.InitializeStateManagerComponent` (`self.TempestBaseStateManager`) (`self.K2_GetPawn`))
  (`EnhancedInputSubsystemInterface.AddMappingContext` (subsystem `EnhancedInputLocalPlayerSubsystem`) (`self.Mapping Context`) 0 (struct))
  (set `self.Targeting Component` (`self.GetComponentByClass` (`self.K2_GetPawn`) "/Script/TempestCombatFramework.TempestTargetingComponent"))
  (set `self.Original Controlled Pawn` (`self.K2_GetPawn`)))

(event `/TempestCombatFramework/Interfaces/BPI_PlayerInputs.Set Last Fired Input`
  (params (`New Last Fired Input` :type "InputAction Object Reference"))
  (set `self.Last Fired Input` `New Last Fired Input`))

(event `Key|N`
  (params (Key :type "Key Structure")))

(fn `Does Input Exist in Mapping`
  (params (`Input To Check` :type "InputAction Object Reference"))
  (returns (`Return Value` :type Boolean))
  (return false))

(fn `Get Direction From Movement Inputs`
  (returns (`Return Value` :type "Vector Structure"))
  (bind _returnvalue (`KismetMathLibrary.MakeRotator` 0.0 0.0 (.yaw (`Pawn.GetControlRotation` (`self.K2_GetPawn`)))))
  (return (`KismetMathLibrary.Normal` (+ (* (`KismetMathLibrary.GetRightVector` _returnvalue) (`self.GetInputAxisValue`)) (* (`KismetMathLibrary.GetForwardVector` _returnvalue) (`self.GetInputAxisValue`))))))

(fn `Get Is Controlling Character`
  (returns (ReturnValue :type Boolean))
  (bind _tagcontainer (message `GameplayTagAssetInterface.GetOwnedGameplayTags` (`self.K2_GetPawn`)))
  (return (`BlueprintGameplayTagLibrary.HasTag` _tagcontainer (struct :`TagName` "Character.Player"))))

(fn `Get Last Fired Input`
  (returns (`Last Fired Input` :type "InputAction Object Reference"))
  (return (`self.Last Fired Input`)))

(fn `Get Mapping Context`
  (returns (`Mapping Context` :type "InputMappingContext Object Reference"))
  (return (`self.Mapping Context`)))

(fn `UserConstructionScript`)