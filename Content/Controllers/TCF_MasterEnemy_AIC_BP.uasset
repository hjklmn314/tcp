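; AI controller for master enemies that runs their behavior tree and draws them into combat with the player.
; Initialization reads the enemy data asset to start the state manager, behavior tree and spawn state, then clears perception.
; Active state and ability changes are mirrored to Blackboard keys, looked up by gameplay tag in the data asset.
; Unless dead, sensed player-tagged actors become combat targets, the first starting combat; per-sense handling is unwired.
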(event `Initialize Enemy Controller`
  (bind _enemy_info (`/TempestCombatFramework/Characters/TCF_MasterEnemy_BP.Get Enemy Data Asset` (`self.Master Enemy`)))
  (bind _astcf_master_enemy_bp (cast `/TempestCombatFramework/Characters/TCF_MasterEnemy_BP` (`self.K2_GetPawn`)))
  (bind _output_get (set `self.Master Enemy` _astcf_master_enemy_bp))
  (`/Engine/EditorBlueprintResources/StandardMacros.IsValid` (`/TempestCombatFramework/Characters/TCF_MasterEnemy_BP.Get Enemy Data Asset` _output_get)
    (:`Is Valid`
      (`TempestBaseStateManagerComponent.InitializeStateManagerComponent` (`self.EnemyStateManagerComponent`) (`self.K2_GetPawn`))
      (`/Engine/EditorBlueprintResources/StandardMacros.IsValid` _enemy_info
        (:`Is Valid`
          (bind _returnvalue (`self.RunBehaviorTree` (`/TempestCombatFramework/DataAssets/DA_Enemyinfo.Get Enemy BT` _enemy_info)))
          (if _returnvalue
            (`self.Bind Dispatchers`)
            (`self.Activate Spawn State`)
            ;[1 1 1] Final Node
            (`AIPerceptionComponent.ForgetAll` (`self.AIPerception`))))))))

(event `self.AIPerception.OnTargetPerceptionUpdated`
  (params (Actor :type "Actor Object Reference") (Stimulus :type "AIStimulus Structure"))
  (bind _bp_tempestenemycombatcomponent (`/TempestCombatFramework/Characters/TCF_MasterEnemy_BP.BP_TempestEnemyCombatComponent` (`self.Master Enemy`)))
  (`self.Can Perceive`
    (:`True`
      (`/Engine/EditorBlueprintResources/StandardMacros.IsValid` (`/TempestCombatFramework/Characters/TCF_MasterEnemy_BP.Get Enemy Data Asset` (`self.Master Enemy`))
        (:`Is Valid`
          (bind _tagcontainer (message `GameplayTagAssetInterface.GetOwnedGameplayTags` Actor))
          (if (`BlueprintGameplayTagLibrary.HasAnyTags` _tagcontainer (`BlueprintGameplayTagLibrary.MakeLiteralGameplayTagContainer` (struct :`GameplayTags` (struct :`(TagName` "Character.Player")))))
            (if (`.bSuccessfullySensed` (break `AIStimulus` Stimulus))
              (`/Engine/EditorBlueprintResources/StandardMacros.IsValid` (`/TempestCombatFramework/Components/AI/AICombatComponent.Get Combat Target` (`/TempestCombatFramework/Characters/TCF_MasterEnemy_BP.BP_TempestEnemyCombatComponent` (`self.Master Enemy`)))
                (:`Is Valid`
                  (`/TempestCombatFramework/Components/AI/AICombatComponent.Add Combat Target` (`/TempestCombatFramework/Characters/TCF_MasterEnemy_BP.BP_TempestEnemyCombatComponent` (`self.Master Enemy`)) Actor))
                (:`Is Not Valid`
                  (`/TempestCombatFramework/Components/AI/AICombatComponent.Add Combat Target` _bp_tempestenemycombatcomponent Actor)
                  (`/TempestCombatFramework/Components/AI/AICombatComponent.Set Combat Target` _bp_tempestenemycombatcomponent Actor)
                  (`/TempestCombatFramework/Components/AI/AICombatComponent.Enter Combat` (`/TempestCombatFramework/Characters/TCF_MasterEnemy_BP.BP_TempestEnemyCombatComponent` (`self.Master Enemy`))))))))))))

(event `Activate Spawn State`
  (`TempestBaseStateManagerComponent.TryPerformStateOfClass` (`self.EnemyStateManagerComponent`) (`/TempestCombatFramework/DataAssets/DA_Enemyinfo.On Spawn State` (`/TempestCombatFramework/Characters/TCF_MasterEnemy_BP.Get Enemy Data Asset` (`self.Master Enemy`))) true))

(event `Bind Dispatchers`
  (add `TempestBaseAbilityManagerComponent.OnUpdatedActiveAbility` (`/TempestCombatFramework/Characters/TCF_MasterEnemy_BP.BP_TempestAbilitySystemComponent` (`self.Master Enemy`)) (delegate `OnUpdatedActiveAbility`)))

(event `OnUpdatedActiveAbility`
  (`BlackboardComponent.SetValueAsObject` (`self.Blackboard`) (`self.Get Behavior Tree Key Name` (struct :`TagName` "AI.BB.AbilityValue")) (`TempestBaseAbilityManagerComponent.GetCurrentActiveAbility` (`/TempestCombatFramework/Characters/TCF_MasterEnemy_BP.BP_TempestAbilitySystemComponent` (`self.Master Enemy`)))))

(event `self.EnemyStateManagerComponent.OnUpdatedActiveState`
  (`BlackboardComponent.SetValueAsObject` (`self.Blackboard`) (`self.Get Behavior Tree Key Name` (struct :`TagName` "AI.BB.StateValue")) (`TempestBaseStateManagerComponent.GetCurrentActiveState` (`self.EnemyStateManagerComponent`))))

(fn `Get Behavior Tree Key Name`
  (params (`Required Key` :type "GameplayTag Structure"))
  (returns (`Key Name` :type Name))
  (return (`BlueprintMapLibrary.Map_Find` (`/TempestCombatFramework/DataAssets/DA_Enemyinfo.BT Keys` (`/TempestCombatFramework/Characters/TCF_MasterEnemy_BP.Get Enemy Data Asset` (`self.Master Enemy`))) `Required Key`)))

(fn `Get Enemy Manager Component`
  (returns (`State Manager Component` :type "/TempestCombatFramework/Components/AI/AIStateManagerComponent Object Reference"))
  (return (`self.EnemyStateManagerComponent`)))

(fn `UserConstructionScript`)