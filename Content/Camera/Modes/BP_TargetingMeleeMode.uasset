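; Lock-on melee camera mode that keeps the player's view turned toward the current target.
; On start it caches the owner's TempestTargetingComponent and PlayerController and sets its status to Looping.
; Each tick it lerps control rotation toward the target's lock-on point, or actor location if that is zero, turning faster up close and clamping pitch.
; Without a valid target or controller it switches to BP_MeleeCameraMode.
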(event `self.StartCameraMode`
  (set `self.Targeting Component` (`Actor.GetComponentByClass` (`ActorComponent.GetOwner` (`self.CameraModeComponent`)) "/Script/TempestCombatFramework.TempestTargetingComponent"))
  (bind _ascharacter (cast `Character` (`ActorComponent.GetOwner` (`self.CameraModeComponent`))))
  (bind _asplayer_controller (cast `PlayerController` (`Pawn.GetController` _ascharacter)))
  (set `self.Player Controller` _asplayer_controller)
  (`self.SetCameraModeStatus` (struct :`TagName` "Camera.Mode.Status.Looping")))

(event `self.TickCameraMode`
  (params (TickValue :type "Float (single-precision)"))
  (bind _returnvalue (`Controller.GetControlRotation` (`self.Player Controller`)))
  (bind _returnvalue_2 (`TempestTargetingComponent.GetTargetedActor` (`self.Targeting Component`)))
  (bind _returnvalue_3 (`Actor.K2_GetActorLocation` _returnvalue_2))
  (`/Engine/EditorBlueprintResources/StandardMacros.IsValid` (`self.Player Controller`)
    (:`Is Valid`
      (`/Engine/EditorBlueprintResources/StandardMacros.IsValid` _returnvalue_2
        (:`Is Valid`
          (`|SwitchGameplayTag` (`self.CameraModeStatus`)
            (:`Camera.Mode.Status.Looping`
              (bind _location (message `/TempestCombatFramework/Interfaces/BPI_TargetingSystem.Get Lock On Location` _returnvalue_2))
              (bind (_returnvalue_roll _returnvalue_pitch _returnvalue_yaw) (`KismetMathLibrary.BreakRotator` (`KismetMathLibrary.RLerp` _returnvalue (`KismetMathLibrary.FindLookAtRotation` (+ (`SceneComponent.K2_GetComponentLocation` (`TempestCameraModeComponent.CameraComponent` (`self.CameraModeComponent`))) (0.0 0.0 100.0)) (select `bool` (== _location (0.0 0.0 0.0)) :`false` _location :`true` _returnvalue_3)) (select `bool` (< (`KismetMathLibrary.Vector_Distance` _returnvalue_3 (`Actor.K2_GetActorLocation` (`ActorComponent.GetOwner` (`self.CameraModeComponent`)))) 500.0) :`false` 0.2 :`true` 0.4 :!type "Float (single-precision)") true)))
              (`Controller.SetControlRotation` (`self.Player Controller`) (`KismetMathLibrary.MakeRotator` (.roll _returnvalue) (`KismetMathLibrary.FClamp` _returnvalue_pitch -15.0 30.0) _returnvalue_yaw)))))
        (:`Is Not Valid`
          (`TempestCameraModeComponent.SetCameraModeOfClass` (`self.CameraModeComponent`) "/TempestCombatFramework/Camera/Modes/BP_MeleeCameraMode.BP_MeleeCameraMode_C" :!label _label))))
    (:`Is Not Valid`
      (goto _label))))