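; Base impact effect Blueprint that spawns particle and sound effects matched to the physical surface of a stored hit result.
; Setters supply the hit result and effect table, then ApplyImpactEffect runs the VFX and SFX passes.
; Each pass plays every entry of the first matching surface, attached at the bone's socket location for bone hits or spawned at the hit location otherwise.
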(event `Apply Impact Effect`
  (`self.Apply VFXs`)
  (`self.Apply SFX`))

(fn `Apply SFX`
  (bind _hit_result (`self.Get Hit Result`))
  (bind (_bblockinghit _binitialoverlap _time _distance _location _impactpoint _normal _impactnormal _physmat _hitactor _hitcomponent _hitbonename) (`GameplayStatics.BreakHitResult` _hit_result))
  (for _array_element (`self.Impact Effects`)
    (bind (_physicalsurface _impactvfx _impactsfx) (break `/TempestCombatFramework/StructuresEnums/S_ImpactEffects` _array_element))
    (if (`|EnumEquality` _physicalsurface (`GameplayStatics.GetSurfaceType` _hit_result))
      (for _array_element_2 _impactsfx
        (if (not (== _hitbonename "None"))
          (bind _sound (break `/TempestCombatFramework/StructuresEnums/S_ImpactSFX` _array_element_2))
          (`GameplayStatics.SpawnSoundAttached` _sound _hitcomponent _hitbonename (`SceneComponent.GetSocketLocation` _hitcomponent _hitbonename) (struct) "KeepWorldPosition" false 1.0 1.0 0.0 null null)
          (else
            (`GameplayStatics.SpawnSoundAtLocation` _sound _location (struct) 1.0 1.0 0.0 null null))))
      (return)))
  (return))

(fn `Apply VFXs`
  (bind _hit_result (`self.Get Hit Result`))
  (bind (_bblockinghit _binitialoverlap _time _distance _location _impactpoint _normal _impactnormal _physmat _hitactor _hitcomponent _hitbonename _bonename) (`GameplayStatics.BreakHitResult` _hit_result))
  (for _array_element (`self.Impact Effects`)
    (bind (_physicalsurface _impactvfx) (break `/TempestCombatFramework/StructuresEnums/S_ImpactEffects` _array_element))
    (if (`|EnumEquality` _physicalsurface (`GameplayStatics.GetSurfaceType` _hit_result))
      (for _array_element_2 _impactvfx
        (if (not (== _hitbonename "None"))
          (bind (_emitter _emitterrotation _emitterscale) (break `/TempestCombatFramework/StructuresEnums/S_ImpactVFX` _array_element_2))
          (`GameplayStatics.SpawnEmitterAttached` _emitter _hitcomponent _bonename (`SceneComponent.GetSocketLocation` _hitcomponent _hitbonename) _emitterrotation _emitterscale "KeepWorldPosition")
          (else
            (`GameplayStatics.SpawnEmitterAtLocation` _emitter _location _emitterrotation _emitterscale))))
      (return)))
  (return))

(fn `Get Hit Result`
  (returns (`Hit Result` :type "HitResult Structure"))
  (return (`self.Hit Result`)))

(fn `Set Hit Result`
  (params (`Hit Result` :type "HitResult Structure"))
  (set `self.Hit Result` `Hit Result`)
  (return))

(fn `Set Impact Effect`
  (params (`Impact Effects` :type "Array of /TempestCombatFramework/StructuresEnums/S_ImpactEffects Structure"))
  (set `self.Impact Effects` `Impact Effects`))