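; Enemy defense property that decides how an enemy reacts to an incoming impact.
; Hit, Block, Deflect and Clash results trigger matching states on the state manager, which is fetched from the character's controller when unset.
; Only Hit checks state conditions, falling back to the IK hit-react ability if the state fails.
; Parent impact attributes are skipped during the BrokenStance ability, while buffs/debuffs defer to the parent.
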(fn `Apply Impact Attributes`
  (bind _returnvalue (`TempestBaseAbilityManagerComponent.GetCurrentActiveAbility` (`Actor.GetComponentByClass` (`self.GetDefensePropertyOwner`) "/Script/TempestCombatFramework.TempestBaseAbilityManagerComponent")))
  (`/Engine/EditorBlueprintResources/StandardMacros.IsValid` _returnvalue
    (:`Is Valid`
      (if (!= (`TempestBaseAbilityObject.AbilityGameplayTag` _returnvalue) (struct :`TagName` "Ability.Hit React.Broken Stance"))
        (`parent.Apply Impact Attributes` :!label _label)))
    (:`Is Not Valid`
      (goto _label))))

(fn `Apply Impact Buffs/ Debuffs`
  (`parent.Apply Impact Buffs/ Debuffs`))

(fn `Apply Impact Hit Reactions`
  (locals (`Local State Manager Component` :type "TempestBaseStateManagerComponent Object Reference"))
  (bind _local_state_manager_component (`local.Local State Manager Component`))
  (bind _local_state_manager_component_2 (`local.Local State Manager Component`))
  (bind _local_state_manager_component_3 (`local.Local State Manager Component`))
  (bind _local_state_manager_component_4 (`local.Local State Manager Component`))
  (bind _returnvalue (`TempestBaseAbilityManagerComponent.GetAbilityOfGameplayTag` (`Actor.GetComponentByClass` (`self.GetDefensePropertyOwner`) "/Script/TempestCombatFramework.TempestBaseAbilityManagerComponent") (struct :`TagName` "Ability.Hit React.IK")))
  (`/Engine/EditorBlueprintResources/StandardMacros.IsValid` (`local.Local State Manager Component`)
    (:`Is Valid`
      _)
    (:`Is Not Valid`
      (bind _ascharacter (cast `Character` (`self.GetDefensePropertyOwner`)))
      (set `local.Local State Manager Component` (`Actor.GetComponentByClass` (`Pawn.GetController` _ascharacter) "/Script/TempestCombatFramework.TempestBaseStateManagerComponent"))))
  (`|SwitchGameplayTag` (`self.ImpactResult`)
    (:`Impact.Result.Hit`
      (bind _returnvalue_2 (`TempestBaseStateManagerComponent.TryPerformStateOfClass` _local_state_manager_component_2 (`GameplayStatics.GetObjectClass` (`TempestBaseStateManagerComponent.GetStateOfGameplayTag` _local_state_manager_component_2 (struct :`TagName` "State.Hit"))) true))
      (if (not _returnvalue_2)
        (`/Engine/EditorBlueprintResources/StandardMacros.IsValid` _returnvalue
          (:`Is Valid`
            (if (`TempestBaseAbilityObject.CanPerformAbility` _returnvalue)
              (`TempestBaseAbilityObject.StartAbility` _returnvalue))))))
    (:`Impact.Result.Block`
      (`TempestBaseStateManagerComponent.TryPerformStateOfClass` _local_state_manager_component (`GameplayStatics.GetObjectClass` (`TempestBaseStateManagerComponent.GetStateOfGameplayTag` _local_state_manager_component (struct :`TagName` "State.BlockHit"))) false))
    (:`Impact.Result.Deflect`
      (`TempestBaseStateManagerComponent.TryPerformStateOfClass` _local_state_manager_component_4 (`GameplayStatics.GetObjectClass` (`TempestBaseStateManagerComponent.GetStateOfGameplayTag` _local_state_manager_component_4 (struct :`TagName` "State.Deflect"))) false))
    (:`Impact.Result.Clash`
      (`TempestBaseStateManagerComponent.TryPerformStateOfClass` _local_state_manager_component_3 (`GameplayStatics.GetObjectClass` (`TempestBaseStateManagerComponent.GetStateOfGameplayTag` _local_state_manager_component_3 (struct :`TagName` "State.Clash"))) false))))