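; Player defense property that decides how the owning character reacts to combat impacts.
; Impact result tags map to Hit, BlockHit, Deflect or Clash states on the controller's Tempest state manager.
; Hit is condition-checked and restarts if that attempt fails while already active; the others skip the check.
; The combat component's Invincible status suppresses impact attributes and buffs/debuffs, but not hit reactions.
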(event `self.ConstructDefenseProperty`
  (`parent.ConstructDefenseProperty`)
  (bind _ascharacter (cast `Character` (`self.GetDefensePropertyOwner`)))
  (set `self.Owner Character` _ascharacter))

(fn `Apply Impact Attributes`
  (if (not (`self.Get Is Invincible`))
    (`parent.Apply Impact Attributes`)))

(fn `Apply Impact Buffs/ Debuffs`
  (if (not (`self.Get Is Invincible`))
    (`parent.Apply Impact Buffs/ Debuffs`)))

(fn `Apply Impact Hit Reactions`
  (locals (`Local State Manager Component` :type "TempestBaseStateManagerComponent Object Reference"))
  (bind _local_state_manager_component (`local.Local State Manager Component`))
  (bind _local_state_manager_component_2 (`local.Local State Manager Component`))
  (bind _local_state_manager_component_3 (`local.Local State Manager Component`))
  (bind _local_state_manager_component_4 (`local.Local State Manager Component`))
  (bind _returnvalue (`TempestBaseStateManagerComponent.GetStateOfGameplayTag` _local_state_manager_component_2 (struct :`TagName` "State.Hit")))
  (bind _returnvalue_2 (`TempestBaseStateManagerComponent.GetCurrentActiveState` _local_state_manager_component_2))
  (`/Engine/EditorBlueprintResources/StandardMacros.IsValid` (`local.Local State Manager Component`)
    (:`Is Valid`
      _)
    (:`Is Not Valid`
      (bind _ascharacter (cast `Character` (`self.GetDefensePropertyOwner`)))
      (set `local.Local State Manager Component` (`Actor.GetComponentByClass` (`Pawn.GetController` _ascharacter) "/Script/TempestCombatFramework.TempestBaseStateManagerComponent"))))
  (`|SwitchGameplayTag` (`self.ImpactResult`)
    (:`Impact.Result.Hit`
      (bind _returnvalue_3 (`TempestBaseStateManagerComponent.TryPerformStateOfClass` _local_state_manager_component_2 (`GameplayStatics.GetObjectClass` _returnvalue) true))
      (if (not _returnvalue_3)
        (if (== _returnvalue_2 _returnvalue)
          (`TempestBaseStateObject.RestartState` _returnvalue_2 true))))
    (:`Impact.Result.Block`
      (`TempestBaseStateManagerComponent.TryPerformStateOfClass` _local_state_manager_component (`GameplayStatics.GetObjectClass` (`TempestBaseStateManagerComponent.GetStateOfGameplayTag` _local_state_manager_component (struct :`TagName` "State.BlockHit"))) false))
    (:`Impact.Result.Deflect`
      (`TempestBaseStateManagerComponent.TryPerformStateOfClass` _local_state_manager_component_4 (`GameplayStatics.GetObjectClass` (`TempestBaseStateManagerComponent.GetStateOfGameplayTag` _local_state_manager_component_4 (struct :`TagName` "State.Deflect"))) false))
    (:`Impact.Result.Clash`
      (`TempestBaseStateManagerComponent.TryPerformStateOfClass` _local_state_manager_component_3 (`GameplayStatics.GetObjectClass` (`TempestBaseStateManagerComponent.GetStateOfGameplayTag` _local_state_manager_component_3 (struct :`TagName` "State.Clash"))) false))))

(fn `Get Is Invincible`
  (returns (ReturnValue :type Boolean))
  (return (`BlueprintGameplayTagLibrary.HasTag` (`TempestCombatComponent.GetCombatStatus` (`self.Combat Component`)) (struct :`TagName` "Status.Combat.Invincible"))))