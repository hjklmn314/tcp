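; Base defense property that resolves an attack received by its owner through the Tempest combat component.
; It picks Deflect, Block or Hit from state availability; the Clash check is unwired.
; It divides that result's damage by defender attributes, writing back into the attack property, then applies it (Health only on Hit) and starts buffs on Hit.
; Hit reactions are an empty stub, and helpers reuse one impact effect instance per class.
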(event `self.ConstructDefenseProperty`
  (set `self.Combat Component` (`Actor.GetComponentByClass` (`self.GetDefensePropertyOwner`) "/Script/TempestCombatFramework.TempestCombatComponent")))

(event `self.ProcessReceivedAttack`
  (`self.Determine Impact Result`)
  (`TempestAttackPropertiesObject.ProcessAttackPropertry` (`TempestCombatComponent.ReceivedAttackProperty` (`self.Combat Component`)))
  (`self.Set Defense Impact Values`)
  (`self.Apply Impact Hit Reactions`)
  (`self.Apply Impact Attributes`)
  (`self.Apply Impact Buffs/ Debuffs`))

(fn `Apply Hit Effect Of Class`
  (params (`Impact Effect Class` :type "/TempestCombatFramework/ImpactEffects/BP_BaseImpactEffect Class Reference"))
  (locals (`Local Created Impact Effect` :type "/TempestCombatFramework/ImpactEffects/BP_BaseImpactEffect Object Reference"))
  (bind _found_impact_effect (`self.Get Hit Effect Of Class` `Impact Effect Class`))
  (bind _impact_effect_class (`local.Impact Effect Class`))
  (bind _receivedattackproperty (`TempestCombatComponent.ReceivedAttackProperty` (`self.Combat Component`)))
  (`/Engine/EditorBlueprintResources/StandardMacros.IsValid` _found_impact_effect
    (:`Is Valid`
      (`/TempestCombatFramework/ImpactEffects/BP_BaseImpactEffect.Set Hit Result` _found_impact_effect (`TempestAttackPropertiesObject.GetHitResult` (`TempestCombatComponent.ReceivedAttackProperty` (`self.Combat Component`))))
      (`/TempestCombatFramework/ImpactEffects/BP_BaseImpactEffect.Apply Impact Effect` _found_impact_effect)
      (return))
    (:`Is Not Valid`
      (if (`KismetSystemLibrary.IsValidClass` (`local.Impact Effect Class`))
        (`/Engine/EditorBlueprintResources/StandardMacros.IsValid` _receivedattackproperty
          (:`Is Valid`
            (bind _returnvalue (`|GenericCreateObject` (`self.GetDefensePropertyOwner`) _impact_effect_class (`TempestAttackPropertiesObject.GetHitResult` _receivedattackproperty)))
            (set `local.Local Created Impact Effect` _returnvalue))
          (:`Is Not Valid`
            (bind _returnvalue_2 (`|GenericCreateObject` :`self` (`self.GetDefensePropertyOwner`) :`Class` _impact_effect_class))
            (set `local.Local Created Impact Effect` _returnvalue_2)))
        (`KismetArrayLibrary.Array_AddUnique` (`self.Created Impact Effects`) (`local.Local Created Impact Effect`))
        (`/TempestCombatFramework/ImpactEffects/BP_BaseImpactEffect.Apply Impact Effect` (`local.Local Created Impact Effect`))
        (return)))))

(fn `Apply Impact Attributes`
  (locals (`Local Received Attack Property` :type "/TempestCombatFramework/AttackProperties/BP_BaseAttackProperties Object Reference") (`Local Attributes Component` :type "TempestAttributesComponents Object Reference"))
  (bind _receivedattackproperty (`TempestCombatComponent.ReceivedAttackProperty` (`self.Combat Component`)))
  (set `local.Local Attributes Component` (`Actor.GetComponentByClass` (`self.GetDefensePropertyOwner`) "/Script/TempestCombatFramework.TempestAttributesComponents"))
  (if (and (`KismetSystemLibrary.IsValid` (`local.Local Attributes Component`)) (`KismetSystemLibrary.IsValid` (`self.Combat Component`)))
    (`/Engine/EditorBlueprintResources/StandardMacros.IsValid` _receivedattackproperty
      (:`Is Valid`
        (bind _asbp_base_attack_properties (cast `/TempestCombatFramework/AttackProperties/BP_BaseAttackProperties` _receivedattackproperty))
        (bind _output_get (set `local.Local Received Attack Property` _asbp_base_attack_properties))
        (bind (_value _returnvalue) (`BlueprintMapLibrary.Map_Find` (`/TempestCombatFramework/AttackProperties/BP_BaseAttackProperties.Damage Applications Per Impact Result` _output_get) (`self.ImpactResult`)))
        (if _returnvalue
          (for _array_element (`.DamageToApply_31_E5B87B0B4F2CC52CCF2141B256ECEE4A` (break `/TempestCombatFramework/StructuresEnums/S_DamageApplications` _value))
            (bind (_targetattributetoeffect _targetattributeamounttoapply) (break `/TempestCombatFramework/StructuresEnums/S_DamageToApply` _array_element))
            (`|SwitchGameplayTag` _targetattributetoeffect
              (:`Default`
                _)
              (:`Attribute.Health`
                (`|SwitchGameplayTag` (`self.ImpactResult`)
                  (:`Impact.Result.Hit`
                    _))))
            (bind _returnvalue_2 (`TempestAttributesComponents.GetAttributeOfGameplayTag` (`local.Local Attributes Component`) _targetattributetoeffect))
            (`/Engine/EditorBlueprintResources/StandardMacros.IsValid` _returnvalue_2
              (:`Is Valid`
                (`TempestBaseAttributeObject.ModifyAttribute` _returnvalue_2 (* _targetattributeamounttoapply -1.0)))))
          (return))))))

(fn `Apply Impact Buffs/ Debuffs`
  (locals (`Local ReceivedAttack Property` :type "/TempestCombatFramework/AttackProperties/BP_BaseAttackProperties Object Reference") (`Local Constructed Buff ` :type "TempestBaseBuffObject Object Reference"))
  (bind _local_constructed_buff_ (`local.Local Constructed Buff `))
  (bind _receivedattackproperty (`TempestCombatComponent.ReceivedAttackProperty` (`self.Combat Component`)))
  (`|SwitchGameplayTag` (`self.ImpactResult`)
    (:`Impact.Result.Hit`
      (if (`KismetSystemLibrary.IsValid` (`self.Combat Component`))
        (`/Engine/EditorBlueprintResources/StandardMacros.IsValid` _receivedattackproperty
          (:`Is Valid`
            (bind _asbp_base_attack_properties (cast `/TempestCombatFramework/AttackProperties/BP_BaseAttackProperties` _receivedattackproperty))
            (bind _output_get (set `local.Local ReceivedAttack Property` _asbp_base_attack_properties))
            (bind (_value _returnvalue) (`BlueprintMapLibrary.Map_Find` (`/TempestCombatFramework/AttackProperties/BP_BaseAttackProperties.Buffs Applications Per Impact Result` _output_get) (`self.ImpactResult`)))
            (if _returnvalue
              (for _array_element (`.BuffsToApply_41_E5B87B0B4F2CC52CCF2141B256ECEE4A` (break `/TempestCombatFramework/StructuresEnums/S_BuffsApplications` _value))
                (bind _returnvalue_2 (`TempestAttackPropertiesObject.GetAttackPropertyOwner` _output_get))
                (bind _returnvalue_3 (`|GenericCreateObject` _returnvalue_2 _array_element))
                (bind _output_get_2 (set `local.Local Constructed Buff ` _returnvalue_3))
                (`TempestBaseBuffObject.SetDamageDealer` _output_get_2 _returnvalue_2)
                (`TempestBaseBuffObject.SetDamageReceiver` (`local.Local Constructed Buff `) (`self.GetDefensePropertyOwner`))
                (`TempestCombatComponent.AddToAppliedBuffs` (`self.Combat Component`) _local_constructed_buff_)
                (`TempestBaseBuffObject.StartBuff` _local_constructed_buff_)))))))))

(fn `Apply Impact Hit Reactions`)

(fn `Determine Impact Result`
  (locals (`Local Character` :type "Character Object Reference") (`Local State Manager Component` :type "TempestBaseStateManagerComponent Object Reference"))
  (bind _returnvalue (`TempestBaseStateManagerComponent.GetStateOfGameplayTag` (`local.Local State Manager Component`) (struct :`TagName` "State.BlockHit")))
  (bind _returnvalue_2 (`TempestBaseStateManagerComponent.GetStateOfGameplayTag` (`local.Local State Manager Component`) (struct :`TagName` "State.Deflect")))
  (bind _ascharacter (cast `Character` (`self.GetDefensePropertyOwner`)))
  (bind _output_get (set `local.Local Character` _ascharacter))
  (`/Engine/EditorBlueprintResources/StandardMacros.IsValid` _output_get
    (:`Is Valid`
      (set `local.Local State Manager Component` (`Actor.GetComponentByClass` (`Pawn.GetController` (`local.Local Character`)) "/Script/TempestCombatFramework.TempestBaseStateManagerComponent"))
      (`/Engine/EditorBlueprintResources/StandardMacros.IsValid` _returnvalue_2
        (:`Is Valid`
          (if (`TempestBaseStateObject.CanPerformState` _returnvalue_2)
            (`self.SetImpactResult` (struct :`TagName` "Impact.Result.Deflect"))
            (return)
            (else
              _)))
        (:`Is Not Valid`
          _))
      (`/Engine/EditorBlueprintResources/StandardMacros.IsValid` _returnvalue
        (:`Is Valid`
          (if (`TempestBaseStateObject.CanPerformState` _returnvalue)
            (`self.SetImpactResult` (struct :`TagName` "Impact.Result.Block"))
            (return)
            (else
              _)))
        (:`Is Not Valid`
          _))
      (`self.SetImpactResult` (struct :`TagName` "Impact.Result.Hit"))
      (return))
    (:`Is Not Valid`
      (`self.SetImpactResult` (struct :`TagName` "Impact.Result.Hit"))
      (return))))

(fn `Find Damage To Apply Of Gameplay Tag`
  (params (`Attribute To Find` :type "GameplayTag Structure"))
  (returns (`Return value` :type "Float (double-precision)"))
  (bind _asbp_base_attack_properties (cast `/TempestCombatFramework/AttackProperties/BP_BaseAttackProperties` (`TempestCombatComponent.ReceivedAttackProperty` (`self.Combat Component`)))
    (:`then`
      (bind (_value _returnvalue) (`BlueprintMapLibrary.Map_Find` (`/TempestCombatFramework/AttackProperties/BP_BaseAttackProperties.Damage Applications Per Impact Result` _asbp_base_attack_properties) (`self.ImpactResult`)))
      (if _returnvalue
        (for _array_element (`.DamageToApply_31_E5B87B0B4F2CC52CCF2141B256ECEE4A` (break `/TempestCombatFramework/StructuresEnums/S_DamageApplications` _value))
          (bind (_targetattributetoeffect _targetattributeamounttoapply) (break `/TempestCombatFramework/StructuresEnums/S_DamageToApply` _array_element))
          (if (== _targetattributetoeffect `Attribute To Find`)
            (return _targetattributeamounttoapply)))
        (return 0.0)))
    (:`CastFailed`
      (return 0.0))))

(fn `Get Hit Effect Of Class`
  (params (`Impact Effect` :type "/TempestCombatFramework/ImpactEffects/BP_BaseImpactEffect Class Reference"))
  (returns (`Found Impact Effect` :type "/TempestCombatFramework/ImpactEffects/BP_BaseImpactEffect Object Reference"))
  (if (`KismetSystemLibrary.IsValidClass` `Impact Effect`)
    (for _array_element (`self.Created Impact Effects`)
      (if (== (`GameplayStatics.GetObjectClass` _array_element) `Impact Effect`)
        (return _array_element))))
  (return null))

(fn `Influence Attribute Value To Receive`
  (params (`Gameplay Tags` :type "Array of GameplayTag Structure") (`Amount To Apply` :type "Float (double-precision)"))
  (returns (`Return Value` :type "Float (double-precision)"))
  (locals (`Local Amount To Apply` :type "Float (double-precision)"))
  (if (> (`KismetArrayLibrary.Array_Length` `Gameplay Tags`) 0)
    (bind _output_get (set `self.Local Attributes Component` (`Actor.GetComponentByClass` (`self.GetDefensePropertyOwner`) "/Script/TempestCombatFramework.TempestAttributesComponents")))
    (`/Engine/EditorBlueprintResources/StandardMacros.IsValid` _output_get
      (:`Is Valid`
        (set `local.Local Amount To Apply` `Amount To Apply`)
        (for _array_element `Gameplay Tags`
          (bind _returnvalue (`TempestAttributesComponents.GetAttributeOfGameplayTag` (`self.Local Attributes Component`) _array_element))
          (`/Engine/EditorBlueprintResources/StandardMacros.IsValid` _returnvalue
            (:`Is Valid`
              (set `local.Local Amount To Apply` (/ (`local.Local Amount To Apply`) (`.AttributeValue` (break `AttributeProperties` (`TempestBaseAttributeObject.AttributeValues` _returnvalue))))))))
        (return (`local.Local Amount To Apply`))))
    (else
      (return `Amount To Apply`))))

(fn `Set Defense Impact Values`
  (locals (`Local Received Attack Property` :type "/TempestCombatFramework/AttackProperties/BP_BaseAttackProperties Object Reference") (`Local Damage To Apply` :type "Array of /TempestCombatFramework/StructuresEnums/S_DamageToApply Structure"))
  (bind _impactresult (`self.ImpactResult`))
  (bind _receivedattackproperty (`TempestCombatComponent.ReceivedAttackProperty` (`self.Combat Component`)))
  (if (`KismetSystemLibrary.IsValid` (`self.Combat Component`))
    (`/Engine/EditorBlueprintResources/StandardMacros.IsValid` _receivedattackproperty
      (:`Is Valid`
        (bind _asbp_base_attack_properties (cast `/TempestCombatFramework/AttackProperties/BP_BaseAttackProperties` _receivedattackproperty))
        (bind _output_get (set `local.Local Received Attack Property` _asbp_base_attack_properties))
        (bind _damage_applications_per_impact_result (`/TempestCombatFramework/AttackProperties/BP_BaseAttackProperties.Damage Applications Per Impact Result` _output_get))
        (bind (_value _returnvalue) (`BlueprintMapLibrary.Map_Find` _damage_applications_per_impact_result (`self.ImpactResult`)))
        (if _returnvalue
          (bind _output_get_2 (set `local.Local Damage To Apply` (`.DamageToApply_31_E5B87B0B4F2CC52CCF2141B256ECEE4A` (break `/TempestCombatFramework/StructuresEnums/S_DamageApplications` _value))))
          (for (_array_element _array_index) _output_get_2
            (bind (_targetattributetoeffect _targetattributeamounttoapply) (break `/TempestCombatFramework/StructuresEnums/S_DamageToApply` _array_element))
            (bind (_value_2 _returnvalue_2) (`BlueprintMapLibrary.Map_Find` (`self.Received Attributes Modified By`) _targetattributetoeffect))
            (if _returnvalue_2
              (bind _return_value (`self.Influence Attribute Value To Receive` (`BlueprintGameplayTagLibrary.BreakGameplayTagContainer` _value_2) _targetattributeamounttoapply))
              (setmembers `/TempestCombatFramework/StructuresEnums/S_DamageToApply` :`StructRef` (`|GetArrayItem` (`local.Local Damage To Apply`) _array_index) :`Target Attribute Amount To Apply` _return_value)))
          (`BlueprintMapLibrary.Map_Remove` _damage_applications_per_impact_result _impactresult)
          (`BlueprintMapLibrary.Map_Add` _damage_applications_per_impact_result _impactresult (make `/TempestCombatFramework/StructuresEnums/S_DamageApplications` (`local.Local Damage To Apply`)))
          (return))))))