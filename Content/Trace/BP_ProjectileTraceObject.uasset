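; BP_ProjectileTraceObject is a projectile trace object that detects hits around its primitive component on behalf of a trace owner.
; DoCollisionTrace runs a stationary sphere trace at each named socket, falling back to the component's location when a socket is missing.
; Only the socket trace ignores the owner.
; Each hit reaches OnTraceHit only while this object remains in the owner's TempestCollisionManagerComponent active trace list.
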(event `self.DoCollisionTrace`
  (bind _traceprimitivecomponent (`self.TracePrimitiveComponent`))
  (bind _returnvalue (`SceneComponent.K2_GetComponentLocation` _traceprimitivecomponent))
  (`/Engine/EditorBlueprintResources/StandardMacros.IsValid` (`self.TraceOwner`)
    (:`Is Valid`
      (`/Engine/EditorBlueprintResources/StandardMacros.IsValid` (`self.TracePrimitiveComponent`)
        (:`Is Valid`
          (for _array_element (`self.TracePrimitiveComponentSocketNames`)
            (if (`SceneComponent.DoesSocketExist` _traceprimitivecomponent _array_element)
              (bind _returnvalue_2 (`SceneComponent.GetSocketLocation` _traceprimitivecomponent _array_element))
              (bind (_outhits _returnvalue_3) (`KismetSystemLibrary.SphereTraceMulti` _returnvalue_2 _returnvalue_2 50.0 "TraceTypeQuery3" false (`|MakeArray` (`self.TraceOwner`)) "None" true (struct :`R` 1.0 :`A` 1.0) (struct :`G` 1.0 :`A` 1.0) 0.1))
              (if _returnvalue_3
                (for _array_element_2 _outhits
                  (if (`KismetArrayLibrary.Array_Contains` (`TempestCollisionManagerComponent.ActiveTraceObjects` (`Actor.GetComponentByClass` (`self.TraceOwner`) "/Script/TempestCombatFramework.TempestCollisionManagerComponent")) self)
                    (`self.OnTraceHit` _array_element_2))))
              (else
                (bind (_outhits_2 _returnvalue_4) (`KismetSystemLibrary.SphereTraceMulti` :`Start` _returnvalue :`End` _returnvalue :`Radius` 50.0 :`TraceChannel` "TraceTypeQuery3" :`DrawTime` 0.1))
                (if _returnvalue_4
                  (for _array_element_3 _outhits_2
                    (if (`KismetArrayLibrary.Array_Contains` (`TempestCollisionManagerComponent.ActiveTraceObjects` (`Actor.GetComponentByClass` (`self.TraceOwner`) "/Script/TempestCombatFramework.TempestCollisionManagerComponent")) self)
                      (`self.OnTraceHit` _array_element_3))))))))))))