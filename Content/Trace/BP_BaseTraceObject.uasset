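; Base trace object for melee-style hit detection, registered with the owner's TempestCollisionManagerComponent while toggled on.
; Each tick while active, it sphere-traces at sockets on the trace primitive component, ignoring the owner.
; New hits with matching gameplay tags or a Breakable tag are recorded once per activation until the trace is toggled off.
; Hits pass the AttackProperty to attacker and victim combat components, then apply damage.
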(event `self.ConstructTrace`)

(event `self.OnTraceHit`
  (params (HitResult :type "HitResult Structure"))
  (bind (_bblockinghit _binitialoverlap _time _distance _location _impactpoint _normal _impactnormal _physmat _hitactor) (`GameplayStatics.BreakHitResult` HitResult))
  (bind _attackproperty (`self.AttackProperty`))
  (bind _returnvalue (`Actor.GetComponentByClass` (`self.TraceOwner`) "/Script/TempestCombatFramework.TempestCombatComponent"))
  (if (`self.Can Actor Be Hit` _hitactor)
    (`KismetArrayLibrary.Array_AddUnique` (`self.Hit Actors`) _hitactor)
    (`/Engine/EditorBlueprintResources/StandardMacros.IsValid` _attackproperty
      (:`Is Valid`
        (`TempestAttackPropertiesObject.SetHitResult` _attackproperty HitResult))
      (:`Is Not Valid`
        _))
    (`/Engine/EditorBlueprintResources/StandardMacros.IsValid` _returnvalue
      (:`Is Valid`
        (`TempestCombatComponent.SetAttackProperty` _returnvalue (`self.AttackProperty`)))
      (:`Is Not Valid`
        _))
    (`self.Apply Damage To Hit Actor` _hitactor)))

(event `self.TickTrace`
  (params (DeltaSeconds :type "Float (single-precision)"))
  ;[1 1 1] This Only Runs if the Collision Trace is Active. It only Gets Activated When the "ANS_Trace" is Used
  (`self.DoCollisionTrace`))

(event `self.ToggleTrace`
  (params (bToggle :type Boolean))
  (bind _returnvalue (`Actor.GetComponentByClass` (`self.TraceOwner`) "/Script/TempestCombatFramework.TempestCollisionManagerComponent"))
  (if bToggle
    (`TempestCollisionManagerComponent.AddTraceToActiveTraces` _returnvalue self)
    (else
      (`TempestCollisionManagerComponent.RemoveTraceFromActiveTraces` _returnvalue self)
      (`KismetArrayLibrary.Array_Clear` (`self.Hit Actors`)))))

(event `self.DoCollisionTrace`
  (bind _traceprimitivecomponent (`self.TracePrimitiveComponent`))
  (`/Engine/EditorBlueprintResources/StandardMacros.IsValid` (`self.TraceOwner`)
    (:`Is Valid`
      (`/Engine/EditorBlueprintResources/StandardMacros.IsValid` (`self.TracePrimitiveComponent`)
        (:`Is Valid`
          (for _array_element (`self.TracePrimitiveComponentSocketNames`)
            (if (`SceneComponent.DoesSocketExist` _traceprimitivecomponent _array_element)
              (bind _returnvalue (`SceneComponent.GetSocketLocation` _traceprimitivecomponent _array_element))
              (bind (_outhits _returnvalue_2) (`KismetSystemLibrary.SphereTraceMulti` _returnvalue _returnvalue 70.0 "TraceTypeQuery3" false (`|MakeArray` (`self.TraceOwner`)) "None" true (struct :`R` 1.0 :`A` 1.0) (struct :`G` 1.0 :`A` 1.0) 0.1))
              (if _returnvalue_2
                (for _array_element_2 _outhits
                  (if (`KismetArrayLibrary.Array_Contains` (`TempestCollisionManagerComponent.ActiveTraceObjects` (`Actor.GetComponentByClass` (`self.TraceOwner`) "/Script/TempestCombatFramework.TempestCollisionManagerComponent")) self)
                    (`self.OnTraceHit` _array_element_2)))))))))))

(fn `Apply Damage To Hit Actor`
  (params (DamagedActor :type "Actor Object Reference"))
  (bind _returnvalue (`Actor.GetComponentByClass` DamagedActor "/Script/TempestCombatFramework.TempestCombatComponent"))
  (`/Engine/EditorBlueprintResources/StandardMacros.IsValid` _returnvalue
    (:`Is Valid`
      (`TempestCombatComponent.SetReceivedAttackProperty` _returnvalue (`self.AttackProperty`))
      (`GameplayStatics.ApplyDamage` DamagedActor 1.0 null (`self.TraceOwner`)))
    (:`Is Not Valid`
      (`GameplayStatics.ApplyDamage` DamagedActor 1.0 null (`self.TraceOwner`)))))

(fn `Can Actor Be Hit`
  (params (Actor :type "Actor Object Reference"))
  (returns (`Return Value` :type Boolean))
  (if (not (`KismetArrayLibrary.Array_Contains` (`self.Hit Actors`) Actor))
    (bind _tagcontainer (message `GameplayTagAssetInterface.GetOwnedGameplayTags` Actor))
    (return (or (`BlueprintGameplayTagLibrary.HasAnyTags` _tagcontainer (`self.Hit Actor Tags`)) (`Actor.ActorHasTag` Actor "Breakable")))
    (else
      (return false))))