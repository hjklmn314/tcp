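; Grab trace object that detects hit actors around sockets on its owner's trace primitive component.
; DoCollisionTrace runs a stationary multi-sphere trace at each existing socket, forwarding hits while this object is active in the owner's TempestCollisionManagerComponent.
; On an eligible hit, it records the actor, passes the hit-updated AttackProperty to TempestCombatComponent, applies damage and switches the trace off.
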(event `self.OnTraceHit`
  (params (HitResult :type "HitResult Structure"))
  (bind (_bblockinghit _binitialoverlap _time _distance _location _impactpoint _normal _impactnormal _physmat _hitactor) (`GameplayStatics.BreakHitResult` HitResult))
  (bind _returnvalue (`Actor.GetComponentByClass` (`self.TraceOwner`) "/Script/TempestCombatFramework.TempestCombatComponent"))
  (if (`self.Can Actor Be Hit` _hitactor)
    (`KismetArrayLibrary.Array_AddUnique` (`self.Hit Actors`) _hitactor)
    (`TempestAttackPropertiesObject.SetHitResult` (`self.AttackProperty`) HitResult)
    (`/Engine/EditorBlueprintResources/StandardMacros.IsValid` _returnvalue
      (:`Is Valid`
        (`TempestCombatComponent.SetAttackProperty` _returnvalue (`self.AttackProperty`)))
      (:`Is Not Valid`
        _))
    (`self.Apply Damage To Hit Actor` _hitactor)
    (`self.ToggleTrace` false)))

(event `self.DoCollisionTrace`
  (bind _traceprimitivecomponent (`self.TracePrimitiveComponent`))
  (`/Engine/EditorBlueprintResources/StandardMacros.IsValid` (`self.TraceOwner`)
    (:`Is Valid`
      (`/Engine/EditorBlueprintResources/StandardMacros.IsValid` (`self.TracePrimitiveComponent`)
        (:`Is Valid`
          (for _array_element (`self.TracePrimitiveComponentSocketNames`)
            (if (`SceneComponent.DoesSocketExist` _traceprimitivecomponent _array_element)
              (bind _returnvalue (`SceneComponent.GetSocketLocation` _traceprimitivecomponent _array_element))
              (bind (_outhits _returnvalue_2) (`KismetSystemLibrary.SphereTraceMulti` _returnvalue _returnvalue 70.0 "TraceTypeQuery3" false (`|MakeArray` (`self.TraceOwner`)) "None" true (struct :`R` 1.0 :`A` 1.0) (struct :`G` 1.0 :`A` 1.0) 0.1))
              (if _returnvalue_2
                (for _array_element_2 _outhits
                  (if (`KismetArrayLibrary.Array_Contains` (`TempestCollisionManagerComponent.ActiveTraceObjects` (`Actor.GetComponentByClass` (`self.TraceOwner`) "/Script/TempestCombatFramework.TempestCollisionManagerComponent")) self)
                    (`self.OnTraceHit` _array_element_2)))))))))))