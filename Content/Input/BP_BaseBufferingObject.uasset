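; Base input-buffering object that captures allowed Input Actions and replays one through its assigned player state object.
; The buffering mode either fires input instantly or holds the latest or highest-priority action, ranked by AllowedInputActions order, until buffering ends.
; Firing requires still being registered with that state, then deregisters the object.
; On end, held-input modes deregister only when an input fires; other modes simply deregister.
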(event `Try Save As Input Buffer`
  (params (`Input Action` :type "InputAction Object Reference"))
  (bind _buffered_input (`self.Buffered Input`))
  (bind _effected_player_state (`self.Effected Player State`))
  (bind _allowed_input_actions (`self.Allowed Input Actions`))
  (if (`KismetArrayLibrary.Array_Contains` (`self.Allowed Input Actions`) `Input Action`)
    (switch `EInputBufferType` (`self.Buffering State`)
      (:`LastRegisteredInput`
        (set `self.Buffered Input` `Input Action`))
      (:`InstantInputFire`
        (set `self.Buffered Input` `Input Action`)
        (if (`KismetArrayLibrary.Array_Contains` (`/TempestCombatFramework/States/Player/BP_BasePlayerState.Get Buffering Objects` (`self.Effected Player State`)) self)
          (`/TempestCombatFramework/States/Player/BP_BasePlayerState.Set Buffered Input` _effected_player_state (`self.Buffered Input`))
          (`/TempestCombatFramework/States/Player/BP_BasePlayerState.Fire Buffered Input` _effected_player_state)
          (`/TempestCombatFramework/States/Player/BP_BasePlayerState.Remove Buffering Object` _effected_player_state self)))
      (:`HighestPriorityInput`
        (`/Engine/EditorBlueprintResources/StandardMacros.IsValid` _buffered_input
          (:`Is Valid`
            (if (< (`KismetArrayLibrary.Array_Find` _allowed_input_actions `Input Action`) (`KismetArrayLibrary.Array_Find` _allowed_input_actions _buffered_input))
              (set `self.Buffered Input` `Input Action` :!label _label)))
          (:`Is Not Valid`
            (goto _label)))))))

(event `End Buffering Object`
  (bind _effected_player_state (`self.Effected Player State`))
  (bind _buffered_input (`self.Buffered Input`))
  (switch `EInputBufferType` (`self.Buffering State`)
    (:`NoBuffer`
      (`/TempestCombatFramework/States/Player/BP_BasePlayerState.Remove Buffering Object` (`self.Effected Player State`) self :!label _label_2))
    (:`LastRegisteredInput`
      (`/Engine/EditorBlueprintResources/StandardMacros.IsValid` _buffered_input :!label _label_3
        (:`Is Valid`
          (if (`KismetArrayLibrary.Array_Contains` (`/TempestCombatFramework/States/Player/BP_BasePlayerState.Get Buffering Objects` (`self.Effected Player State`)) self)
            (`/TempestCombatFramework/States/Player/BP_BasePlayerState.Set Buffered Input` _effected_player_state _buffered_input)
            (`/TempestCombatFramework/States/Player/BP_BasePlayerState.Fire Buffered Input` _effected_player_state)
            (`/TempestCombatFramework/States/Player/BP_BasePlayerState.Remove Buffering Object` _effected_player_state self)))))
    (:`InstantInputFire`
      (goto _label_2))
    (:`HighestPriorityInput`
      (goto _label_3))))

(fn `Set Base State To Effect`
  (params (`Player State` :type "/TempestCombatFramework/States/Player/BP_BasePlayerState Object Reference"))
  (set `self.Effected Player State` `Player State`))

(fn `Set Buffering State`
  (params (`Buffering State` :type "EInputBufferType Enum" :default "NoBuffer"))
  (set `self.Buffering State` `Buffering State`))